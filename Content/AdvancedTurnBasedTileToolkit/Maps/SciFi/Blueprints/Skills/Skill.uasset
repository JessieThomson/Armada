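; Base skill actor for the SciFi turn-based tile example, with placeholder effect, scoring and hover hooks for specific skills to override.
; Activation makes it the unit's active skill; for players, Tick moves a decal or mesh marker and shows cover around the hovered tile.
; AI helpers score reachable targets, choose a cover-aware firing tile and start movement.
; It also handles action points, charges, cooldown and waking nearby units.
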(event Custom|Activate%20Skill
  (params (Unit :type Unit%20Object%20Reference))
  ;[0 1 0.1621] Activate Skill
  (bind _output_get (Variables|Default|SetOwning%20Unit Unit))
  (bind _asunit_skill (Utilities|Casting|CastToUnit_Skill _output_get))
  (if (Utilities|IsValid (Variables|/Game/AdvancedTurnBasedTileToolkit/Maps/SciFi/Blueprints/Pawns/Unit_Skill.Unit_Skill_C|GetActive%20Skill _asunit_skill))
    (if (!= (Variables|/Game/AdvancedTurnBasedTileToolkit/Maps/SciFi/Blueprints/Pawns/Unit_Skill.Unit_Skill_C|GetActive%20Skill _asunit_skill) self)
      (CallFunction|DeactivateSkill (Variables|/Game/AdvancedTurnBasedTileToolkit/Maps/SciFi/Blueprints/Pawns/Unit_Skill.Unit_Skill_C|GetActive%20Skill _asunit_skill))
      (Variables|/Game/AdvancedTurnBasedTileToolkit/Maps/SciFi/Blueprints/Pawns/Unit_Skill.Unit_Skill_C|SetActive%20Skill _asunit_skill self :!label _label))
    (else
      (goto _label)))
  (Actor|Tick|SetActorTickEnabled true)
  (Variables|Default|SetOnly%20Ckeck%20Value false)
  (if (not (Variables|/Game/AdvancedTurnBasedTileToolkit/Blueprints/Pawns/Unit.Unit_C|GetAI%20Controlled (Variables|Default|GetOwning%20Unit)))
    (if (Variables|/Game/AdvancedTurnBasedTileToolkit/Blueprints/Gameplay/BP_Grid_Manager.BP_Grid_Manager_C|GetUse%20Decals (Variables|Default|GetGrid_Manager_Ref))
      (Rendering|SetVisibility (Variables|Default|GetSkill%20Decal) true false)
      (else
        (Rendering|SetVisibility (Variables|Default|GetSkill%20Marker) true false)))))

(event Custom|AI%20Check%20Value
  (params (Unit :type Unit%20Object%20Reference))
  ;[0.4088 0 1] AI Check Value
  (bind _output_get (Variables|Default|SetOwning%20Unit Unit))
  (bind _asunit_skill (Utilities|Casting|CastToUnit_Skill _output_get))
  (Variables|/Game/AdvancedTurnBasedTileToolkit/Maps/SciFi/Blueprints/Pawns/Unit_Skill.Unit_Skill_C|SetActive%20Skill _asunit_skill self)
  (Variables|Default|SetOnly%20Ckeck%20Value true)
  (Variables|Default|SetAI%20Estimated%20Value -999999.0))

(event Custom|Move%20Hover%20Marker
  (bind _currenttilehover (Variables|Default|GetCurrentTileHover))
  (bind _grid_manager_ref (Variables|Default|GetGrid_Manager_Ref))
  (bind _returnvalue (Transformation|GetActorLocation _grid_manager_ref))
  (bind _vectorfieldarray (Variables|/Game/AdvancedTurnBasedTileToolkit/Blueprints/Gameplay/BP_Grid_Manager.BP_Grid_Manager_C|GetVectorFieldArray _grid_manager_ref))
  (bind _splineheight (Variables|/Game/AdvancedTurnBasedTileToolkit/Blueprints/Gameplay/BP_Grid_Manager.BP_Grid_Manager_C|GetSplineHeight _grid_manager_ref))
  (bind _item (Utilities|Array|Get(acopy) _vectorfieldarray _currenttilehover))
  (bind _returnvalue_2 (Math|Vector|MakeVector 0.0 0.0 _splineheight))
  (bind _returnvalue_3 (+ _returnvalue_2 _returnvalue _item))
  ;[1 0.9295 0] Event Tick
  ;;[0 0 0] Move Hover Index
  (if (Variables|/Game/AdvancedTurnBasedTileToolkit/Blueprints/Gameplay/BP_Grid_Manager.BP_Grid_Manager_C|GetUse%20Decals (Variables|Default|GetGrid_Manager_Ref))
    (Rendering|SetVisibility (Variables|Default|GetSkill%20Decal) true false)
    (else
      (Rendering|SetVisibility (Variables|Default|GetSkill%20Marker) true false)))
  (if (Default|IsTileImpassable? (Variables|Default|GetGrid_Manager_Ref) (Variables|Default|GetCurrentTileHover)) ; Never show path if tile is impassable
    (CallFunction|MouseNotOverValidTile)
    (elif (Variables|/Game/AdvancedTurnBasedTileToolkit/Blueprints/Gameplay/BP_Grid_Manager.BP_Grid_Manager_C|GetUse%20Decals (Variables|Default|GetGrid_Manager_Ref))
      (Transformation|SetWorldLocation (Variables|Default|GetSkill%20Decal) _returnvalue_3 false false)
      (else
        (Transformation|SetWorldLocation (Variables|Default|GetSkill%20Marker) _returnvalue_3 false false)))))

(event Custom|Tile%20Clicked
  (params (Index :type Integer))
  ;[0 1 0.4941] Tile Clicked
  (if (Variables|/Game/AdvancedTurnBasedTileToolkit/Blueprints/Gameplay/BP_Grid_Camera.BP_Grid_Camera_C|GetMoving (Variables|Default|GetGrid%20Camera%20Ref))
    (Variables|Default|SetClicked%20Tile -1)
    (else
      (Variables|Default|SetClicked%20Tile Index))))

(event Custom|Update%20Hover%20Index
  (bind _grid_manager_ref (Variables|Default|GetGrid_Manager_Ref))
  ;[1 0.9295 0] Event Tick
  ;;[0 0 0] Update Hover Index
  (if (or (Variables|/Game/AdvancedTurnBasedTileToolkit/Blueprints/Gameplay/BP_Grid_Camera.BP_Grid_Camera_C|GetMoving (Variables|Default|GetGrid%20Camera%20Ref)) (Variables|/Game/AdvancedTurnBasedTileToolkit/Maps/SciFi/Blueprints/ATBTT_PlayerController_SciFi.ATBTT_PlayerController_SciFi_C|GetMouse%20over%20UI (.AsATBTT%20Player%20Controller%20Sci%20Fi (Utilities|Casting|CastToATBTT_PlayerController_SciFi (Game|GetPlayerController 0)))))
    (CallFunction|MouseNotOverValidTile :!label _label)
    (else
      (bind (_index _location _tracehit) (Default|GetHitTileLocationandIndex (Variables|Default|GetGrid_Manager_Ref)))
      (if _tracehit ; Is the mouse over something blocking PathTrace? (normally a tile)
        (if (!= (Variables|Default|GetCurrentTileHover) _index) ; If the currently hovered tile is the same as the last do not\nbother updating anything and keep results from last time.
          (if (Math|Vector|Equal(Vector) _location (+ (Transformation|GetActorLocation _grid_manager_ref) (Utilities|Array|Get(acopy) (Variables|/Game/AdvancedTurnBasedTileToolkit/Blueprints/Gameplay/BP_Grid_Manager.BP_Grid_Manager_C|GetVectorFieldArray _grid_manager_ref) _index)) (|(sqrt(((square(kat1))+(square(kat2))))) (Variables|/Game/AdvancedTurnBasedTileToolkit/Blueprints/Gameplay/BP_Grid_Manager.BP_Grid_Manager_C|GetTileBoundsX _grid_manager_ref) (Variables|/Game/AdvancedTurnBasedTileToolkit/Blueprints/Gameplay/BP_Grid_Manager.BP_Grid_Manager_C|GetTileBoundsY _grid_manager_ref))) ; Do not show path if hit location and hit index location are very different (might happen if hovering on edges)
            (Variables|Default|SetCurrentTileHover _index)
            (if (Variables|/Game/AdvancedTurnBasedTileToolkit/Maps/SciFi/Blueprints/ATBTT_PlayerController_SciFi.ATBTT_PlayerController_SciFi_C|GetMouse%20over%20UI (Variables|Default|GetPC_Ref))
              (Variables|Default|SetCurrentTileHover -1)
              (else
                (CallFunction|MoveHoverMarker)
                (CallFunction|CustomHoverEvent)))
            (else
              (CallFunction|MouseNotOverValidTile))))
        (else
          (goto _label))))))

(event Custom|Custom%20Hover%20Event
  ;[1 0.9295 0] Event Tick
  ;;[0 0 0] Update Hover Index
)

(event Custom|Mouse%20not%20over%20valid%20tile
  ;[1 0.9295 0] Event Tick
  ;;[0 0 0] Mouse Not Over Valid Tile
  (Variables|Default|SetCurrentTileHover -1)
  (if (Variables|/Game/AdvancedTurnBasedTileToolkit/Blueprints/Gameplay/BP_Grid_Manager.BP_Grid_Manager_C|GetUse%20Decals (Variables|Default|GetGrid_Manager_Ref))
    (Rendering|SetVisibility (Variables|Default|GetSkill%20Decal) false false)
    (else
      (Rendering|SetVisibility (Variables|Default|GetSkill%20Marker) false false))))

(event Custom|Deactivate%20Skill
  (bind _grid_manager_ref (Variables|Default|GetGrid_Manager_Ref))
  ;[1 0.9295 0] Event Tick
  ;;[0 0 0] Mouse Not Over Valid Tile
  (Actor|Tick|SetActorTickEnabled false)
  (if (not (Variables|/Game/AdvancedTurnBasedTileToolkit/Blueprints/Pawns/Unit.Unit_C|GetAI%20Controlled (Variables|Default|GetOwning%20Unit)))
    (Utilities|Array|Clear (Variables|/Game/AdvancedTurnBasedTileToolkit/Blueprints/Gameplay/BP_Grid_Manager.BP_Grid_Manager_C|GetCanMoveToArray _grid_manager_ref))
    (Utilities|Array|Clear (Variables|/Game/AdvancedTurnBasedTileToolkit/Blueprints/Gameplay/BP_Grid_Manager.BP_Grid_Manager_C|GetIndex%20CanMoveToArray _grid_manager_ref))
    (if (Variables|/Game/AdvancedTurnBasedTileToolkit/Blueprints/Gameplay/BP_Grid_Manager.BP_Grid_Manager_C|GetUse%20Decals (Variables|Default|GetGrid_Manager_Ref))
      (Rendering|SetVisibility (Variables|Default|GetSkill%20Decal) false false)
      (else
        (Rendering|SetVisibility (Variables|Default|GetSkill%20Marker) false false)))))

(event EventBeginPlay
  ;[1 0.4592 0] Event Begin Play
  (bind _outactors (Actor|GetAllActorsOfClass "/Game/AdvancedTurnBasedTileToolkit/Blueprints/Gameplay/BP_Grid_Manager.BP_Grid_Manager_C"))
  (Variables|Default|SetGrid_Manager_Ref (Utilities|Array|Get(acopy) _outactors))
  (bind _asatbtt_game_mode (Utilities|Casting|CastToATBTT_GameMode (Game|GetGameMode)))
  (Variables|Default|SetGame%20Mode%20Ref _asatbtt_game_mode)
  (bind _asatbtt_player_controller_sci_fi (Utilities|Casting|CastToATBTT_PlayerController_SciFi (Game|GetPlayerController 0)))
  (Variables|Default|SetPC_Ref _asatbtt_player_controller_sci_fi)
  (if (Variables|/Game/AdvancedTurnBasedTileToolkit/Blueprints/Gameplay/BP_Grid_Manager.BP_Grid_Manager_C|GetUse%20Decals (Variables|Default|GetGrid_Manager_Ref))
    (bind _returnvalue (AddComponent|AddDecalComponent false (Math|Transform|MakeTransform "0, 0, 0" "90.000000, 0,0.000000" "200.000000,85.000000,85.000000")))
    (bind _output_get (Variables|Default|SetSkill%20Decal _returnvalue))
    (Rendering|Components|Decal|SetDecalMaterial _output_get (Variables|Default|GetSkill%20Decal%20Material))
    (Default|ScaleDecalRelativetoDefaultTile (Variables|Default|GetGrid_Manager_Ref) (Variables|Default|GetSkill%20Decal))
    (Class|SceneComponent|Attachto (Variables|Default|GetSkill%20Decal) (Variables|/Game/AdvancedTurnBasedTileToolkit/Blueprints/Gameplay/BP_Grid_Manager.BP_Grid_Manager_C|GetScene1 (Variables|Default|GetGrid_Manager_Ref)) "None" "KeepRelativeOffset" true)
    (else
      (bind _returnvalue_2 (AddComponent|AddStaticMeshComponent false))
      (bind _output_get_2 (Variables|Default|SetSkill%20Marker _returnvalue_2))
      (Components|StaticMesh|SetStaticMesh _output_get_2 (Variables|Default|GetSkill%20Marker%20Mesh))
      (Default|ScaleRelativetoDefaultTile (Variables|Default|GetGrid_Manager_Ref) (Variables|Default|GetSkill%20Marker))
      (Class|SceneComponent|Attachto (Variables|Default|GetSkill%20Marker) (Variables|/Game/AdvancedTurnBasedTileToolkit/Blueprints/Gameplay/BP_Grid_Manager.BP_Grid_Manager_C|GetScene1 (Variables|Default|GetGrid_Manager_Ref)) "None" "KeepRelativeOffset" true)))
  (bind _outactors_2 (Actor|GetAllActorsOfClass "/Game/AdvancedTurnBasedTileToolkit/Blueprints/Gameplay/BP_Grid_Camera.BP_Grid_Camera_C"))
  (Variables|Default|SetGrid%20Camera%20Ref (Utilities|Array|Get(acopy) _outactors_2))
  (Utilities|FlowControl|Delay 0.0)
  (Variables|Default|SetAI%20Controller%20Ref (Variables|/Game/AdvancedTurnBasedTileToolkit/Blueprints/Gameplay/ATBTT_GameMode.ATBTT_GameMode_C|GetAIController_Ref (Variables|Default|GetGame%20Mode%20Ref))))

(event EventTick
  (params (DeltaSeconds :type Float%20%28single-precision%29))
  (bind _currenttilehover (Variables|Default|GetCurrentTileHover))
  ;[1 0.9295 0] Event Tick
  (if (not (Variables|/Game/AdvancedTurnBasedTileToolkit/Blueprints/Pawns/Unit.Unit_C|GetAI%20Controlled (Variables|Default|GetOwning%20Unit)))
    (CallFunction|UpdateHoverIndex)
    (if (!= _currenttilehover -1)
      (bind _asbp_grid_manager_sci_fi (Utilities|Casting|CastToBP_Grid_Manager_SciFi (Variables|Default|GetGrid_Manager_Ref)))
      (Default|ShowCoverMeshesAroundIndex _asbp_grid_manager_sci_fi _currenttilehover))))

(fn ConstructionScript
  (Variables|Default|SetCurrent%20Charges (Variables|Default|GetStarting%20Charges)))

(fn SetHUDText
  (params (NewParam :type String))
  (bind _asbp_grid_manager_sci_fi (Utilities|Casting|CastToBP_Grid_Manager_SciFi (Variables|Default|GetGrid_Manager_Ref)))
  (Variables|/Game/AdvancedTurnBasedTileToolkit/Maps/SciFi/Blueprints/BP_Grid_Manager_SciFi.BP_Grid_Manager_SciFi_C|SetHUD%20Text _asbp_grid_manager_sci_fi (Utilities|Text|ToText(String) NewParam)))

(fn PayActionPointCost
  (bind _asunit_skill (Utilities|Casting|CastToUnit_Skill (Variables|Default|GetOwning%20Unit)))
  (Variables|/Game/AdvancedTurnBasedTileToolkit/Maps/SciFi/Blueprints/Pawns/Unit_Skill.Unit_Skill_C|SetCurrent%20Action%20Points _asunit_skill (Math|Integer|Max(Integer) (- (Variables|/Game/AdvancedTurnBasedTileToolkit/Maps/SciFi/Blueprints/Pawns/Unit_Skill.Unit_Skill_C|GetCurrent%20Action%20Points _asunit_skill) (Variables|Default|GetAction%20Point%20Cost))))
  (Variables|Default|SetCurrent%20Charges (Math|Integer|Min(Integer) (Math|Integer|Max(Integer) (- (Variables|Default|GetCurrent%20Charges) 1)) (Variables|Default|GetStarting%20Charges)))
  (Variables|Default|SetCurrent%20Cooldown (Variables|Default|GetDefault%20Cooldown))
  (if (Variables|/Game/AdvancedTurnBasedTileToolkit/Blueprints/Pawns/Unit.Unit_C|GetAI%20Controlled (Variables|Default|GetOwning%20Unit))
    _
    (else
      (bind _asbp_grid_manager_sci_fi (Utilities|Casting|CastToBP_Grid_Manager_SciFi (Variables|Default|GetGrid_Manager_Ref))
        (:then
          (Default|UpdateHUDInfo (Variables|/Game/AdvancedTurnBasedTileToolkit/Maps/SciFi/Blueprints/HUD_SciFi.HUD_SciFi_C|GetHUD_Info_176 (Variables|/Game/AdvancedTurnBasedTileToolkit/Maps/SciFi/Blueprints/BP_Grid_Manager_SciFi.BP_Grid_Manager_SciFi_C|GetHUD_SciFi _asbp_grid_manager_sci_fi))))
        (:CastFailed
          _))))
  (return))

(fn AIPriorityModifier
  (params (Current%20Index :type Integer) (Target%20Index :type Integer))
  (return (+ 0.0 1.0)))

(fn GetHoverText
  (return "[Hover Text]"))

(fn FindTargetCandidates
  (params (Find%20Friendly%20Units :type Boolean))
  (bind _owning_unit (Variables|Default|GetOwning%20Unit))
  (bind _asunit_skill (Utilities|Casting|CastToUnit_Skill _owning_unit))
  (Utilities|Array|Clear (Variables|Default|GetTarget%20Candidates))
  (bind _tiles_in_sight_array (Default|FindUnitsinRange (Variables|Default|GetGrid_Manager_Ref) (Variables|/Game/AdvancedTurnBasedTileToolkit/Blueprints/Pawns/Unit.Unit_C|GetIndex _asunit_skill) (+ (Variables|Default|GetRange) (Math|Integer|SelectInt (Variables|/Game/AdvancedTurnBasedTileToolkit/Blueprints/Pawns/Unit.Unit_C|GetCurrent%20Move _asunit_skill) 0 (> (Variables|/Game/AdvancedTurnBasedTileToolkit/Maps/SciFi/Blueprints/Pawns/Unit_Skill.Unit_Skill_C|GetCurrent%20Action%20Points _asunit_skill) 1))) false))
  (bind _output_get (Variables|Default|SetTarget%20Candidates _tiles_in_sight_array))
  (Utilities|Array|RemoveIndex _output_get (Utilities|Array|FindItem _output_get (Variables|/Game/AdvancedTurnBasedTileToolkit/Blueprints/Pawns/Unit.Unit_C|GetIndex (Variables|Default|GetOwning%20Unit))))
  ;[0 0.2954 1] Only consider enemy targets
  (bind (_arrayindex _arrayelement) (Utilities|Array|ReverseforEachLoop (Variables|Default|GetTarget%20Candidates))
    (:LoopBody
      (if (not (select Find%20Friendly%20Units (!= (Utilities|Array|FindItem (Variables|/Game/AdvancedTurnBasedTileToolkit/Blueprints/Pawns/Unit.Unit_C|GetAllied%20Factions (Variables|Default|GetOwning%20Unit)) (Variables|/Game/AdvancedTurnBasedTileToolkit/Blueprints/Pawns/Unit.Unit_C|GetFaction (Utilities|Array|Get(acopy) (Variables|/Game/AdvancedTurnBasedTileToolkit/Blueprints/Gameplay/BP_Grid_Manager.BP_Grid_Manager_C|GetPawn%20Array (Variables|Default|GetGrid_Manager_Ref)) _arrayelement))) -1) (== (Utilities|Array|FindItem (Variables|/Game/AdvancedTurnBasedTileToolkit/Blueprints/Pawns/Unit.Unit_C|GetAllied%20Factions (Variables|Default|GetOwning%20Unit)) (Variables|/Game/AdvancedTurnBasedTileToolkit/Blueprints/Pawns/Unit.Unit_C|GetFaction (Utilities|Array|Get(acopy) (Variables|/Game/AdvancedTurnBasedTileToolkit/Blueprints/Gameplay/BP_Grid_Manager.BP_Grid_Manager_C|GetPawn%20Array (Variables|Default|GetGrid_Manager_Ref)) _arrayelement))) -1)))
        (Utilities|Array|RemoveIndex (Variables|Default|GetTarget%20Candidates) _arrayindex)))))

(fn FindPotentialTargets
  (params (Index :type Integer) (Range :type Integer) (Find%20Allies :type Boolean) (Exclude%20Current%20Unit :type Boolean) (Diamond%20Shaped%20Visibility :type Boolean))
  ;[1 0.5687 0] Find Potential Targets
  (bind _tiles_in_sight_array (Default|FindUnitsinRange (Variables|Default|GetGrid_Manager_Ref) Index Range Diamond%20Shaped%20Visibility))
  (bind _output_get (Variables|Default|SetTarget%20Candidates _tiles_in_sight_array))
  (bind _indexes_out (Default|KeepIndexeswithRelevantUnits (Variables|Default|GetGrid_Manager_Ref) _output_get (Variables|/Game/AdvancedTurnBasedTileToolkit/Blueprints/Pawns/Unit.Unit_C|GetAllied%20Factions (Variables|Default|GetOwning%20Unit)) Find%20Allies Exclude%20Current%20Unit))
  (bind _output_get_2 (Variables|Default|SetTarget%20Candidates _indexes_out))
  (return _output_get_2))

(fn FindBestReachableTarget
  (params (Target%20Candidates :type Array%20of%20Integers) (Choice%20Array :type Array%20of%20Floats%20%28single-precision%29))
  (bind (_indexofmaxvalue _maxvalue) (Math|Float|MaxOfFloatArray Choice%20Array))
  (bind _owning_unit (Variables|Default|GetOwning%20Unit))
  ;[1 0 0.8177] Find Best Reachable Target
  (bind _target_found (Default|FindAllPossibleTargets (Variables|Default|GetGrid_Manager_Ref) (Variables|/Game/AdvancedTurnBasedTileToolkit/Blueprints/Pawns/Unit.Unit_C|GetIndex _owning_unit) (Variables|Default|GetRange) (Variables|/Game/AdvancedTurnBasedTileToolkit/Blueprints/Pawns/Unit.Unit_C|GetCurrent%20Move _owning_unit) (Utilities|Array|Get(acopy) Target%20Candidates _indexofmaxvalue) :!label _label))
  (if _target_found
    (LocalVariables|SetLocal%20Target%20Found true)
    (Variables|Default|SetTarget%20Index (Utilities|Array|Get(acopy) Target%20Candidates _indexofmaxvalue)) ; For AI: Simulate clicking target for attack logic
    (bind _output_get (Variables|Default|SetAI%20Estimated%20Value _maxvalue))
    (else
      (Utilities|Array|RemoveIndex (Variables|Default|GetChoice%20Array) _indexofmaxvalue)
      (Utilities|Array|RemoveIndex Target%20Candidates _indexofmaxvalue)
      (if (> (Utilities|Array|Length Target%20Candidates) 0)
        (goto _label)
        (else
          _))))
  (return (LocalVariables|GetLocal%20Target%20Found) (Variables|Default|GetTarget%20Index) _output_get))

(fn FindPathandInitializeMovement
  (params (Move%20Index :type Integer))
  (bind _game_mode_ref (Variables|Default|GetGame%20Mode%20Ref))
  (bind _currentpawn (Variables|/Game/AdvancedTurnBasedTileToolkit/Blueprints/Gameplay/ATBTT_GameMode.ATBTT_GameMode_C|GetCurrentPawn _game_mode_ref))
  ;[0 1 0.3279] Find Path and Initialize Movement. Rest of skill runs at end of movement.
  (Default|FindPathWithinPathfindingArray (Variables|Default|GetGrid_Manager_Ref) Move%20Index true false false)
  (Variables|/Game/AdvancedTurnBasedTileToolkit/Blueprints/Pawns/Unit.Unit_C|SetHasActedThisTurn (Variables|/Game/AdvancedTurnBasedTileToolkit/Blueprints/Gameplay/ATBTT_GameMode.ATBTT_GameMode_C|GetCurrentPawn (Variables|Default|GetGame%20Mode%20Ref)) true)
  (bind _asunit_skill (Utilities|Casting|CastToUnit_Skill (Variables|Default|GetOwning%20Unit))
    (:then
      (Variables|/Game/AdvancedTurnBasedTileToolkit/Maps/SciFi/Blueprints/Pawns/Unit_Skill.Unit_Skill_C|SetCurrent%20Action%20Points _asunit_skill (Math|Integer|Max(Integer) (- (Variables|/Game/AdvancedTurnBasedTileToolkit/Maps/SciFi/Blueprints/Pawns/Unit_Skill.Unit_Skill_C|GetCurrent%20Action%20Points _asunit_skill) 1))))
    (:CastFailed
      _))
  (Default|BeginMovement (Variables|Default|GetOwning%20Unit) 0 true) ; Signals to the unit to start movement. Continued in Unit_Parent
  (Variables|/Game/AdvancedTurnBasedTileToolkit/Blueprints/Pawns/Unit.Unit_C|SetCurrent%20Move _currentpawn (- (Variables|/Game/AdvancedTurnBasedTileToolkit/Blueprints/Pawns/Unit.Unit_C|GetCurrent%20Move _currentpawn) (.cost (Utilities|Array|Get(acopy) (Variables|/Game/AdvancedTurnBasedTileToolkit/Blueprints/Gameplay/BP_Grid_Manager.BP_Grid_Manager_C|GetCanMoveToArray (Variables|Default|GetGrid_Manager_Ref)) (Variables|Default|GetTarget%20Index))))))

(fn FindBestTarget
  (params (Potential%20Targets :type Array%20of%20Integers))
  (bind _choice_array (Variables|Default|GetChoice%20Array))
  (bind (_indexofmaxvalue _maxvalue) (Math|Float|MaxOfFloatArray _choice_array))
  (Utilities|Array|Clear (Variables|Default|GetChoice%20Array))
  (for _array_element Potential%20Targets
    (bind _value (CallFunction|FindTargetValue _array_element))
    (Utilities|Array|Add (Variables|Default|GetChoice%20Array) _value))
  (bind _output_get (Variables|Default|SetTarget%20Index (Utilities|Array|Get(acopy) (Variables|Default|GetTarget%20Candidates) _indexofmaxvalue)))
  (bind _output_get_2 (Variables|Default|SetAI%20Estimated%20Value _maxvalue))
  (return _output_get _output_get_2))

(fn FindTargetValue
  (params (Target%20Index :type Integer))
  (return (* Target%20Index 0.01)))

(fn AIPrepareandExecuteSkill
  (Development|PrintString "ERROR: No skill effect found"))

(fn EvaluateSkill
  (params (Find%20Allies :type Boolean))
  (bind _owning_unit (Variables|Default|GetOwning%20Unit))
  (bind _asunit_skill (Utilities|Casting|CastToUnit_Skill _owning_unit))
  (bind _square_visibility (Variables|/Game/AdvancedTurnBasedTileToolkit/Blueprints/Pawns/Unit.Unit_C|GetSquare%20Visibility _owning_unit))
  (bind _returnvalue (not _square_visibility))
  (bind _target_candidates (CallFunction|FindPotentialTargets (Variables|/Game/AdvancedTurnBasedTileToolkit/Blueprints/Pawns/Unit.Unit_C|GetIndex _asunit_skill) (+ (Variables|Default|GetRange) (* (- (Variables|/Game/AdvancedTurnBasedTileToolkit/Maps/SciFi/Blueprints/Pawns/Unit_Skill.Unit_Skill_C|GetCurrent%20Action%20Points _asunit_skill) 1) (Variables|/Game/AdvancedTurnBasedTileToolkit/Blueprints/Pawns/Unit.Unit_C|GetCurrent%20Move _owning_unit))) Find%20Allies true _returnvalue))
  (bind _found_units_ (Default|FindUnitsinSightfromMoveArray (Variables|Default|GetGrid_Manager_Ref) _target_candidates (Variables|Default|GetRange) _returnvalue false))
  (bind _output_get (Variables|Default|SetTarget%20Candidates _found_units_))
  (bind (_target_index _ai_estimated_value) (CallFunction|FindBestTarget _output_get))
  (return _target_index _ai_estimated_value))

(fn FindBestTilefromWhichtoUseSkill
  (bind _owning_unit (Variables|Default|GetOwning%20Unit))
  ;[1 0.9398 0] Find best tile from which to use skill on target
  (bind (_target_index_ _target_value) (Default|FindBestMoveIndexBasedonCoverandActiveSkill (.AsBP%20Grid%20Manager%20Sci%20Fi (Utilities|Casting|CastToBP_Grid_Manager_SciFi (Variables|Default|GetGrid_Manager_Ref))) self (Variables|/Game/AdvancedTurnBasedTileToolkit/Blueprints/Pawns/Unit.Unit_C|GetIndex _owning_unit) (Variables|Default|GetTarget%20Index) (Variables|Default|GetRange) true true (not (Variables|/Game/AdvancedTurnBasedTileToolkit/Blueprints/Pawns/Unit.Unit_C|GetSquare%20Visibility _owning_unit))))
  (bind _output_get (Variables|Default|SetMove%20Target%20Index _target_index_))
  (bind _output_get_2 (Variables|Default|SetAI%20Estimated%20Value (* _target_value (Variables|Default|GetAI%20Estimated%20Value) (Variables|Default|GetBase%20AI%20Value))))
  (return _output_get _output_get_2))

(fn WakeUnitsinRange
  (params (Source%20Index :type Integer) (Sight%20Range :type Integer) (Hearing%20Range :type Integer))
  (bind _tiles_in_sight_array (Default|FindUnitsinRange (Variables|Default|GetGrid_Manager_Ref) Source%20Index (Math|Integer|Max(Integer) Sight%20Range Hearing%20Range) false))
  (for _array_element _tiles_in_sight_array
    (bind _asatbtt_game_mode_sci_fi (Utilities|Casting|CastToATBTT_GameMode_SciFi (Variables|Default|GetGame%20Mode%20Ref)))
    (Default|CheckifUnitShouldWake _asatbtt_game_mode_sci_fi (Utilities|Array|Get(acopy) (Variables|/Game/AdvancedTurnBasedTileToolkit/Blueprints/Gameplay/BP_Grid_Manager.BP_Grid_Manager_C|GetPawn%20Array (Variables|Default|GetGrid_Manager_Ref)) _array_element) Source%20Index Sight%20Range Hearing%20Range 1.8e+02)))