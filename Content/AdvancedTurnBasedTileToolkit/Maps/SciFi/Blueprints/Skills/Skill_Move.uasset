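; Movement skill for the SciFi tactics map, letting a unit walk or sprint across tiles using action points.
; Players get a pathfound range, with hover previewing paths and potential-target crosshairs.
; Clicking a tile starts movement, costing two points beyond normal move, while clicking a same-faction unit with points left swaps to it.
; AI units rate it near zero, and activation pays points to extend their pathfinding beyond move range.
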(event EventCustomHoverEvent
  (bind _grid_manager_ref (Variables|Default|GetGrid_Manager_Ref))
  (bind _currenttilehover (Variables|Default|GetCurrentTileHover))
  (bind _currenttilehover_2 (Variables|Default|GetCurrentTileHover))
  (bind _grid_manager_ref_2 (Variables|Default|GetGrid_Manager_Ref))
  (bind _pawn_array (Variables|/Game/AdvancedTurnBasedTileToolkit/Blueprints/Gameplay/BP_Grid_Manager.BP_Grid_Manager_C|GetPawn%20Array _grid_manager_ref_2))
  (bind _item (Utilities|Array|Get(acopy) _pawn_array _currenttilehover_2))
  ;[1 0.888 0] Custom Hover Event
  (if (!= _currenttilehover -1)
    (if (not (Default|IsTileImpassable? (Variables|Default|GetGrid_Manager_Ref) _currenttilehover)) ; Never show path if tile is impassable
      (if (and (== (Utilities|Array|Get(acopy) (Variables|/Game/AdvancedTurnBasedTileToolkit/Blueprints/Gameplay/BP_Grid_Manager.BP_Grid_Manager_C|GetPawn%20Array (Variables|Default|GetGrid_Manager_Ref)) (Variables|Default|GetCurrentTileHover)) 0) (> (.cost (Utilities|Array|Get(acopy) (Variables|/Game/AdvancedTurnBasedTileToolkit/Blueprints/Gameplay/BP_Grid_Manager.BP_Grid_Manager_C|GetCanMoveToArray (Variables|Default|GetGrid_Manager_Ref)) (Variables|Default|GetCurrentTileHover))) 0))
        (Default|FindPathWithinPathfindingArray (Variables|Default|GetGrid_Manager_Ref) (Variables|Default|GetCurrentTileHover) true true (Variables|/Game/AdvancedTurnBasedTileToolkit/Blueprints/Gameplay/BP_Grid_Manager.BP_Grid_Manager_C|GetDisplayPathAsSpline (Variables|Default|GetGrid_Manager_Ref))) ; Find and show a path from the path hovered to the tile the pathfinding array was generated from (generally the current pawn)
        (if (Variables|/Game/AdvancedTurnBasedTileToolkit/Blueprints/Gameplay/BP_Grid_Manager.BP_Grid_Manager_C|GetShow%20Crosshairs (Variables|Default|GetGrid_Manager_Ref))
          (Default|RemoveCrosshairs (Variables|Default|GetGrid_Manager_Ref))
          (Default|ShowCrosshaironAllPotentialTargetUnitsinRange (Variables|Default|GetGrid_Manager_Ref) (Variables|Default|GetCurrentTileHover) 16 (not (Variables|/Game/AdvancedTurnBasedTileToolkit/Blueprints/Pawns/Unit.Unit_C|GetSquare%20Visibility (Variables|Default|GetOwning%20Unit))) (* 16 (/ (+ (Variables|/Game/AdvancedTurnBasedTileToolkit/Blueprints/Gameplay/BP_Grid_Manager.BP_Grid_Manager_C|GetTileBoundsX _grid_manager_ref) (Variables|/Game/AdvancedTurnBasedTileToolkit/Blueprints/Gameplay/BP_Grid_Manager.BP_Grid_Manager_C|GetTileBoundsY _grid_manager_ref)) 2.0)) 1 (Variables|/Game/AdvancedTurnBasedTileToolkit/Blueprints/Pawns/Unit.Unit_C|GetAllied%20Factions (Variables|Default|GetOwning%20Unit))))
        (elif (Utilities|IsValid _item)
          (if (Utilities|Enum|Equal(Enum) (Variables|/Game/AdvancedTurnBasedTileToolkit/Blueprints/Pawns/Unit.Unit_C|GetFaction _item) (Variables|/Game/AdvancedTurnBasedTileToolkit/Blueprints/Pawns/Unit.Unit_C|GetFaction (Variables|Default|GetOwning%20Unit)))
            (if (Variables|/Game/AdvancedTurnBasedTileToolkit/Blueprints/Gameplay/BP_Grid_Manager.BP_Grid_Manager_C|GetDisplayPathAsSpline (Variables|Default|GetGrid_Manager_Ref)) ; If not reachable, delete previous path
              (Default|DestroyandClearSplinePath (Variables|Default|GetGrid_Manager_Ref))
              (else
                (Components|InstancedStaticMesh|ClearInstances (Variables|/Game/AdvancedTurnBasedTileToolkit/Blueprints/Gameplay/BP_Grid_Manager.BP_Grid_Manager_C|GetPath (Variables|Default|GetGrid_Manager_Ref))) ; Delete the old path markers (do nothing if path is displayed as path)
              ))
            (else
              (CallFunction|MouseNotOverValidTile :!label _label)))
          (else
            (goto _label)))))))

(event EventActivateSkill
  (params (Unit :type Unit%20Object%20Reference))
  (bind _owning_unit (Variables|Default|GetOwning%20Unit))
  (bind _owning_unit_2 (Variables|Default|GetOwning%20Unit))
  ;[0 1 0.07048] Activate Skill
  (|CallParentFunction Unit)
  (if (Variables|/Game/AdvancedTurnBasedTileToolkit/Blueprints/Pawns/Unit.Unit_C|GetAI%20Controlled Unit)
    ;[0 0 0] AI
    (if (not (Variables|Default|GetOnly%20Ckeck%20Value))
      (if (== (Variables|/Game/AdvancedTurnBasedTileToolkit/Maps/SciFi/Blueprints/Pawns/Unit_Skill.Unit_Skill_C|GetCurrent%20Action%20Points (.AsUnit%20Skill (Utilities|Casting|CastToUnit_Skill (Variables|Default|GetOwning%20Unit)))) 0)
        (Default|ActivateUnit (Variables|Default|GetOwning%20Unit))
        (else
          (Variables|/Game/AdvancedTurnBasedTileToolkit/Blueprints/Pawns/Unit.Unit_C|SetCurrent%20Move _owning_unit (+ (Variables|/Game/AdvancedTurnBasedTileToolkit/Blueprints/Pawns/Unit.Unit_C|GetCurrent%20Move _owning_unit) (Variables|/Game/AdvancedTurnBasedTileToolkit/Blueprints/Pawns/Unit.Unit_C|GetMax%20Move _owning_unit)))
          (CallFunction|PayActionPointCost)
          (Default|ContinuePathfindingBeyondMoveRange (Variables|Default|GetAI%20Controller%20Ref))
          (CallFunction|DeactivateSkill))))
    (else
      (bind _asunit_skill (Utilities|Casting|CastToUnit_Skill _owning_unit_2))
      (Default|Pathfinding (Variables|Default|GetGrid_Manager_Ref) (Variables|/Game/AdvancedTurnBasedTileToolkit/Blueprints/Pawns/Unit.Unit_C|GetIndex _owning_unit_2) (* (Variables|/Game/AdvancedTurnBasedTileToolkit/Maps/SciFi/Blueprints/Pawns/Unit_Skill.Unit_Skill_C|GetCurrent%20Action%20Points _asunit_skill) (Variables|/Game/AdvancedTurnBasedTileToolkit/Blueprints/Pawns/Unit.Unit_C|GetCurrent%20Move _owning_unit_2)) false (* (Variables|/Game/AdvancedTurnBasedTileToolkit/Maps/SciFi/Blueprints/Pawns/Unit_Skill.Unit_Skill_C|GetCurrent%20Action%20Points _asunit_skill) (Variables|/Game/AdvancedTurnBasedTileToolkit/Blueprints/Pawns/Unit.Unit_C|GetCurrent%20Move _owning_unit_2)) true (Variables|/Game/AdvancedTurnBasedTileToolkit/Blueprints/Pawns/Unit.Unit_C|GetPathfinding%20Type _owning_unit_2)) ; Find all possible tiles a unit can move to constrained by its move attribute
    )))

(event EventMouseNotOverValidTile
  ;[1 0.888 0] Custom Hover Event
  ;;[0 0 0] Mouse Not over Valid Tile
  (|CallParentFunction)
  (if (Variables|/Game/AdvancedTurnBasedTileToolkit/Blueprints/Gameplay/BP_Grid_Manager.BP_Grid_Manager_C|GetDisplayPathAsSpline (Variables|Default|GetGrid_Manager_Ref)) ; If not reachable, delete previous path
    (Default|DestroyandClearSplinePath (Variables|Default|GetGrid_Manager_Ref))
    (else
      (Components|InstancedStaticMesh|ClearInstances (Variables|/Game/AdvancedTurnBasedTileToolkit/Blueprints/Gameplay/BP_Grid_Manager.BP_Grid_Manager_C|GetPath (Variables|Default|GetGrid_Manager_Ref))) ; Delete the old path markers (do nothing if path is displayed as path)
    ))
  (Default|RemoveCrosshairs (Variables|Default|GetGrid_Manager_Ref)))

(event EventAICheckValue
  (params (Unit :type Unit%20Object%20Reference))
  ;[0 0 0] AI
  (|CallParentFunction Unit)
  (Variables|Default|SetAI%20Estimated%20Value 1e-06))

(event EventDeactivateSkill
  ;[0 0 0] Deactivate Skill
  (|CallParentFunction)
  (CallFunction|MouseNotOverValidTile)
  (Default|ClearAllinRangeMeshMarkers (Variables|Default|GetGrid_Manager_Ref)))

(event EventTileClicked
  (params (Index :type Integer))
  (bind _grid_manager_ref (Variables|Default|GetGrid_Manager_Ref))
  (bind _grid_manager_ref_2 (Variables|Default|GetGrid_Manager_Ref))
  (bind _clicked_tile (Variables|Default|GetClicked%20Tile))
  (bind _grid_manager_ref_3 (Variables|Default|GetGrid_Manager_Ref))
  (bind _targetmarker (Variables|/Game/AdvancedTurnBasedTileToolkit/Blueprints/Gameplay/BP_Grid_Manager.BP_Grid_Manager_C|GetTargetMarker _grid_manager_ref_2))
  (bind _target_marker_decal (Variables|/Game/AdvancedTurnBasedTileToolkit/Blueprints/Gameplay/BP_Grid_Manager.BP_Grid_Manager_C|GetTarget%20Marker%20Decal _grid_manager_ref_2))
  (bind _pawn_array (Variables|/Game/AdvancedTurnBasedTileToolkit/Blueprints/Gameplay/BP_Grid_Manager.BP_Grid_Manager_C|GetPawn%20Array _grid_manager_ref_3))
  (bind _item (Utilities|Array|Get(acopy) _pawn_array _clicked_tile))
  ;[0 0.1642 1] Decide Action for Clicked Tile
  (|CallParentFunction Index)
  (if (== _item 0)
    (if (> (.cost (Utilities|Array|Get(acopy) (Variables|/Game/AdvancedTurnBasedTileToolkit/Blueprints/Gameplay/BP_Grid_Manager.BP_Grid_Manager_C|GetCanMoveToArray (Variables|Default|GetGrid_Manager_Ref)) (Variables|Default|GetClicked%20Tile))) 0) ; Only move to tile if within move distance (has a cost)
      (Default|SetMarkerLocation (Variables|Default|GetGrid_Manager_Ref) "0, 0, 0" true (Variables|Default|GetClicked%20Tile) _target_marker_decal _targetmarker) ; Set target marker to the target tile
      (Default|SetMarkerVisibility (Variables|Default|GetGrid_Manager_Ref) true _target_marker_decal _targetmarker)
      (Default|FindPathWithinPathfindingArray (Variables|Default|GetGrid_Manager_Ref) (Variables|Default|GetClicked%20Tile) true false false)
      (Default|ClearAllinRangeMeshMarkers _grid_manager_ref)
      (Default|DestroyandClearSplinePath _grid_manager_ref)
      (Utilities|Array|SetArrayElem (Variables|/Game/AdvancedTurnBasedTileToolkit/Blueprints/Gameplay/BP_Grid_Manager.BP_Grid_Manager_C|GetPawn%20Array (Variables|Default|GetGrid_Manager_Ref)) (Variables|/Game/AdvancedTurnBasedTileToolkit/Blueprints/Pawns/Unit.Unit_C|GetIndex (Variables|/Game/AdvancedTurnBasedTileToolkit/Blueprints/Gameplay/ATBTT_GameMode.ATBTT_GameMode_C|GetCurrentPawn (Variables|Default|GetGame%20Mode%20Ref))) 0)
      (bind _asunit_skill (Utilities|Casting|CastToUnit_Skill (Variables|Default|GetOwning%20Unit)))
      (Variables|/Game/AdvancedTurnBasedTileToolkit/Maps/SciFi/Blueprints/Pawns/Unit_Skill.Unit_Skill_C|SetCurrent%20Action%20Points _asunit_skill (Math|Integer|Max(Integer) (- (Variables|/Game/AdvancedTurnBasedTileToolkit/Maps/SciFi/Blueprints/Pawns/Unit_Skill.Unit_Skill_C|GetCurrent%20Action%20Points _asunit_skill) (Math|Integer|SelectInt 2 1 (> (.cost (Utilities|Array|Get(acopy) (Variables|/Game/AdvancedTurnBasedTileToolkit/Blueprints/Gameplay/BP_Grid_Manager.BP_Grid_Manager_C|GetCanMoveToArray (Variables|Default|GetGrid_Manager_Ref)) (Variables|Default|GetClicked%20Tile))) (Variables|/Game/AdvancedTurnBasedTileToolkit/Blueprints/Pawns/Unit.Unit_C|GetCurrent%20Move (Variables|Default|GetOwning%20Unit)))))))
      (bind _asatbtt_player_controller (Utilities|Casting|CastToATBTT_PlayerController (Game|GetPlayerController 0)))
      (Variables|/Game/AdvancedTurnBasedTileToolkit/Blueprints/Gameplay/ATBTT_PlayerController.ATBTT_PlayerController_C|SetDisable%20Player%20Controller%20Input _asatbtt_player_controller true)
      (Default|BeginMovement (Variables|/Game/AdvancedTurnBasedTileToolkit/Blueprints/Gameplay/ATBTT_GameMode.ATBTT_GameMode_C|GetCurrentPawn (Variables|Default|GetGame%20Mode%20Ref)) 0 false) ; Begin pawn movement (continued in event graph Unit_Parent)
      (CallFunction|DeactivateSkill))
    (else
      (bind _asunit_skill_2 (Utilities|Casting|CastToUnit_Skill _item))
      (if (and (> (Variables|/Game/AdvancedTurnBasedTileToolkit/Maps/SciFi/Blueprints/Pawns/Unit_Skill.Unit_Skill_C|GetCurrent%20Action%20Points _asunit_skill_2) 0) (Utilities|Enum|Equal(Enum) (Variables|/Game/AdvancedTurnBasedTileToolkit/Blueprints/Pawns/Unit.Unit_C|GetFaction _asunit_skill_2) (Variables|/Game/AdvancedTurnBasedTileToolkit/Blueprints/Pawns/Unit.Unit_C|GetFaction (Variables|Default|GetOwning%20Unit))))
        (CallFunction|DeactivateSkill)
        (Default|SwaptoUnit (.AsATBTT%20Game%20Mode (Utilities|Casting|CastToATBTT_GameMode (Game|GetGameMode))) _asunit_skill_2)))))

(fn ConstructionScript
  (|CallParentFunction))

(fn GetHoverText
  (return (Utilities|Text|ToText(String) (Utilities|String|Append (Utilities|String|ToString(Text) (Utilities|Text|MakeLiteralText "Sprint: 
")) (Utilities|String|ToString(Text) (Utilities|Text|MakeLiteralText "Move to a tile within move range. Sprinting to 
")) (Utilities|String|ToString(Text) (Utilities|Text|MakeLiteralText "a tile marked in yellow ends your turn."))))))