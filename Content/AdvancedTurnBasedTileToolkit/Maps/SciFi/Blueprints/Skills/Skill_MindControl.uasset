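; Sci-fi turn-based skill that lets a unit mind control a non-allied unit in range so it fights for the caster's faction.
; Players pick from highlighted visible targets, while the AI scores targets by proximity to other potential targets, skips already controlled ones and paths to a casting tile.
; Casting spawns an SE_MindControlled status effect on the victim, moving woken units to the end of the initiative order.
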(event Custom|Mind%20Control%20Unit
  (params (Target%20Unit :type Unit%20Skill%20Object%20Reference))
  (bind _game_mode_ref (Variables|Default|GetGame%20Mode%20Ref))
  (bind _game_mode_ref_2 (Variables|Default|GetGame%20Mode%20Ref))
  (bind _asatbtt_game_mode_sci_fi (Utilities|Casting|CastToATBTT_GameMode_SciFi _game_mode_ref))
  (bind _initiativeorder (Variables|/Game/AdvancedTurnBasedTileToolkit/Blueprints/Gameplay/ATBTT_GameMode.ATBTT_GameMode_C|GetInitiativeOrder _game_mode_ref_2))
  (bind _returnvalue (Utilities|Array|FindItem _initiativeorder Target%20Unit))
  (bind _woke_units (Variables|/Game/AdvancedTurnBasedTileToolkit/Maps/SciFi/Blueprints/ATBTT_GameMode_SciFi.ATBTT_GameMode_SciFi_C|GetWoke%20Units _asatbtt_game_mode_sci_fi))
  ;[1 0 0.969] Mind Control Unit
  (bind _returnvalue_2 (Game|SpawnActorfromClass "/Game/AdvancedTurnBasedTileToolkit/Maps/SciFi/Blueprints/Skills/SE_MindControlled.SE_MindControlled_C" (Math|Conversions|ToTransform(Vector) (Transformation|GetActorLocation Target%20Unit)) "Undefined" 0 0))
  (bind _asunit_skill (Utilities|Casting|CastToUnit_Skill (Variables|Default|GetOwning%20Unit)))
  (Variables|/Game/AdvancedTurnBasedTileToolkit/Maps/SciFi/Blueprints/Skills/SE_MindControlled.SE_MindControlled_C|SetControlling%20Unit _returnvalue_2 _asunit_skill)
  (Default|ActivateSE _returnvalue_2 Target%20Unit)
  (if (!= (Utilities|Array|FindItem _woke_units Target%20Unit) -1)
    (Utilities|Array|RemoveItem _woke_units Target%20Unit)
    (if (== _returnvalue -1)
      _
      (else
        (Utilities|Array|RemoveIndex _initiativeorder _returnvalue)))
    (Utilities|Array|Add _initiativeorder Target%20Unit)))

(event EventCustomHoverEvent
  (bind _grid_manager_ref (Variables|Default|GetGrid_Manager_Ref))
  (bind _range (Variables|Default|GetRange))
  ;[0 0 0] Player
  ;;[0 0.09568 1] Custom Hover Event
  (|CallParentFunction)
  (if (Variables|/Game/AdvancedTurnBasedTileToolkit/Blueprints/Gameplay/BP_Grid_Manager.BP_Grid_Manager_C|GetShow%20Crosshairs (Variables|Default|GetGrid_Manager_Ref))
    (Default|RemoveCrosshairs (Variables|Default|GetGrid_Manager_Ref))
    (Default|ShowCrosshaironAllPotentialTargetUnitsinRange (Variables|Default|GetGrid_Manager_Ref) (Variables|Default|GetCurrentTileHover) _range (not (Variables|/Game/AdvancedTurnBasedTileToolkit/Blueprints/Pawns/Unit.Unit_C|GetSquare%20Visibility (Variables|Default|GetOwning%20Unit))) (* _range (/ (+ (Variables|/Game/AdvancedTurnBasedTileToolkit/Blueprints/Gameplay/BP_Grid_Manager.BP_Grid_Manager_C|GetTileBoundsX _grid_manager_ref) (Variables|/Game/AdvancedTurnBasedTileToolkit/Blueprints/Gameplay/BP_Grid_Manager.BP_Grid_Manager_C|GetTileBoundsY _grid_manager_ref)) 2.0)) 1 (Variables|/Game/AdvancedTurnBasedTileToolkit/Blueprints/Pawns/Unit.Unit_C|GetAllied%20Factions (Variables|Default|GetOwning%20Unit)))))

(event EventAICheckValue
  (params (Unit :type Unit%20Object%20Reference))
  ;[0 0 0] AI
  ;;[0 1 0.2041] Check Value
  (|CallParentFunction Unit)
  (CallFunction|EvaluateSkill false)
  (Utilities|FlowControl|Delay 0.0)
  (bind _move_target_index (CallFunction|FindBestTilefromWhichtoUseSkill))
  (if (not (Variables|Default|GetOnly%20Ckeck%20Value))
    (CallFunction|FindPathandInitializeMovement _move_target_index)))

(event EventActivateSkill
  (params (Unit :type Unit%20Object%20Reference))
  (bind _owning_unit (Variables|Default|GetOwning%20Unit))
  (bind _grid_manager_ref (Variables|Default|GetGrid_Manager_Ref))
  ;[0 1 0.02679] Activate Skill
  (|CallParentFunction Unit)
  (if (Variables|/Game/AdvancedTurnBasedTileToolkit/Blueprints/Pawns/Unit.Unit_C|GetAI%20Controlled Unit)
    ;[0 0 0] AI
    (if (== (Variables|/Game/AdvancedTurnBasedTileToolkit/Maps/SciFi/Blueprints/Pawns/Unit_Skill.Unit_Skill_C|GetCurrent%20Action%20Points (.AsUnit%20Skill (Utilities|Casting|CastToUnit_Skill (Variables|Default|GetOwning%20Unit)))) 1)
      (CallFunction|AIPrepareandExecuteSkill)
      (else
        (CallFunction|EvaluateSkill false)
        (Utilities|FlowControl|Delay 0.0)
        (bind _move_target_index (CallFunction|FindBestTilefromWhichtoUseSkill))
        (if (not (Variables|Default|GetOnly%20Ckeck%20Value))
          (CallFunction|FindPathandInitializeMovement _move_target_index))))
    (else
      (Default|ClearAllinRangeMeshMarkers (Variables|Default|GetGrid_Manager_Ref))
      (Default|Pathfinding (Variables|Default|GetGrid_Manager_Ref) (Variables|/Game/AdvancedTurnBasedTileToolkit/Blueprints/Pawns/Unit.Unit_C|GetIndex (Variables|Default|GetOwning%20Unit)) 0 false 0 false "NewEnumerator0")
      (bind _units_in_sight (Default|FindVisibleUnitsinRange (Variables|Default|GetGrid_Manager_Ref) (Variables|/Game/AdvancedTurnBasedTileToolkit/Blueprints/Pawns/Unit.Unit_C|GetIndex _owning_unit) (Variables|Default|GetRange) (not (Variables|/Game/AdvancedTurnBasedTileToolkit/Blueprints/Pawns/Unit.Unit_C|GetSquare%20Visibility _owning_unit)) (* (Variables|/Game/AdvancedTurnBasedTileToolkit/Blueprints/Pawns/Unit.Unit_C|GetRange _owning_unit) (/ (+ (Variables|/Game/AdvancedTurnBasedTileToolkit/Blueprints/Gameplay/BP_Grid_Manager.BP_Grid_Manager_C|GetTileBoundsX _grid_manager_ref) (Variables|/Game/AdvancedTurnBasedTileToolkit/Blueprints/Gameplay/BP_Grid_Manager.BP_Grid_Manager_C|GetTileBoundsY _grid_manager_ref)) 2.0)) (Variables|/Game/AdvancedTurnBasedTileToolkit/Blueprints/Pawns/Unit.Unit_C|GetMinimum%20Range _owning_unit)))
      (bind _indexes_out (Default|KeepIndexeswithRelevantUnits (Variables|Default|GetGrid_Manager_Ref) _units_in_sight (Variables|/Game/AdvancedTurnBasedTileToolkit/Blueprints/Pawns/Unit.Unit_C|GetAllied%20Factions (Variables|Default|GetOwning%20Unit)) false true))
      (Variables|/Game/AdvancedTurnBasedTileToolkit/Blueprints/Gameplay/BP_Grid_Manager.BP_Grid_Manager_C|SetTiles%20In%20Sight%20Array (Variables|Default|GetGrid_Manager_Ref) _indexes_out)
      (Default|SpawnTilesinSightRange (Variables|Default|GetGrid_Manager_Ref) "NewEnumerator1"))))

(event EventTileClicked
  (params (Index :type Integer))
  (bind _owning_unit (Variables|Default|GetOwning%20Unit))
  (bind _clicked_tile (Variables|Default|GetClicked%20Tile))
  (bind _grid_manager_ref (Variables|Default|GetGrid_Manager_Ref))
  (bind _pawn_array (Variables|/Game/AdvancedTurnBasedTileToolkit/Blueprints/Gameplay/BP_Grid_Manager.BP_Grid_Manager_C|GetPawn%20Array _grid_manager_ref))
  (bind _item (Utilities|Array|Get(acopy) _pawn_array _clicked_tile))
  (bind _faction (Variables|/Game/AdvancedTurnBasedTileToolkit/Blueprints/Pawns/Unit.Unit_C|GetFaction _item))
  ;[0 0 0] Player
  ;;[1 0.5484 0] Decide Action for Clicked Tile
  (|CallParentFunction Index)
  (if (Utilities|IsValid _item) ; Does the clicked tile contain a unit?
    (if (!= _faction (Variables|/Game/AdvancedTurnBasedTileToolkit/Blueprints/Pawns/Unit.Unit_C|GetFaction _owning_unit)) ; Is the unit of a different faction than the one owning the skill?
      (if (== (Utilities|Array|FindItem (Variables|/Game/AdvancedTurnBasedTileToolkit/Blueprints/Pawns/Unit.Unit_C|GetAllied%20Factions _owning_unit) _faction) -1) ; Is the clicked unit not an ally?
        (bind _asunit_skill (Utilities|Casting|CastToUnit_Skill _item))
        (CallFunction|MindControlUnit _asunit_skill)
        (CallFunction|PayActionPointCost)
        (Audio|PlaySoundatLocation "/Game/AdvancedTurnBasedTileToolkit/Maps/SciFi/Audio/MindControl4.MindControl4" (Math|Vector|MakeVector (.x (Transformation|GetActorLocation _asunit_skill)) (.y (Transformation|GetActorLocation _asunit_skill)) (+ (.z (Transformation|GetActorLocation _asunit_skill)) 1.5e+02)))
        (Effects|SpawnEmitteratLocation "/Game/AdvancedTurnBasedTileToolkit/Maps/SciFi/Particles/P_Posseser_Attach.P_Posseser_Attach" (Math|Vector|MakeVector (.x (Transformation|GetActorLocation _asunit_skill)) (.y (Transformation|GetActorLocation _asunit_skill)) (+ (.z (Transformation|GetActorLocation _asunit_skill)) 1.5e+02)))
        (Utilities|FlowControl|Delay 1.0)
        (CallFunction|DeactivateSkill)
        (Default|ActivateUnit (Variables|Default|GetOwning%20Unit))))))

(event EventAIPrepareandExecuteSkill
  (bind _grid_manager_ref (Variables|Default|GetGrid_Manager_Ref))
  (bind _grid_manager_ref_2 (Variables|Default|GetGrid_Manager_Ref))
  (bind _target_index (Variables|Default|GetTarget%20Index))
  (bind _pawn_array (Variables|/Game/AdvancedTurnBasedTileToolkit/Blueprints/Gameplay/BP_Grid_Manager.BP_Grid_Manager_C|GetPawn%20Array _grid_manager_ref_2))
  (bind _target_marker_decal (Variables|/Game/AdvancedTurnBasedTileToolkit/Blueprints/Gameplay/BP_Grid_Manager.BP_Grid_Manager_C|GetTarget%20Marker%20Decal _grid_manager_ref_2))
  (bind _targetmarker (Variables|/Game/AdvancedTurnBasedTileToolkit/Blueprints/Gameplay/BP_Grid_Manager.BP_Grid_Manager_C|GetTargetMarker _grid_manager_ref_2))
  (bind _item (Utilities|Array|Get(acopy) _pawn_array _target_index))
  ;[0 0 0] AI
  ;;[0.9957 0 1] Prepare Mind Control
  (if (not (Variables|Default|GetOnly%20Ckeck%20Value)) ; Temporary. Full version should check value no matter the amount of action points
    (CallFunction|PayActionPointCost)
    (Default|SetMarkerLocation (Variables|Default|GetGrid_Manager_Ref) "0.000000,0.000000,0.000000" true (Variables|Default|GetTarget%20Index) _target_marker_decal _targetmarker)
    (Default|SetMarkerVisibility (Variables|Default|GetGrid_Manager_Ref) true _target_marker_decal _targetmarker)
    (Transformation|SetActorRotation (Variables|Default|GetOwning%20Unit) (Math|Rotator|MakeRotator 0.0 0.0 (.yaw (Math|Rotator|FindLookatRotation (Transformation|GetActorLocation (Variables|Default|GetOwning%20Unit)) (Transformation|GetActorLocation _item)))))
    (bind _asunit_skill (Utilities|Casting|CastToUnit_Skill (Variables|Default|GetOwning%20Unit)))
    (bind _aspawn_anim_bp_parent (Utilities|Casting|CastToPawn_Anim_BP_Parent (Components|SkeletalMesh|GetAnimInstance (Variables|/Game/AdvancedTurnBasedTileToolkit/Maps/SciFi/Blueprints/Pawns/Unit_Skill.Unit_Skill_C|GetSkeletalMesh _asunit_skill))))
    (Default|AttackAnimation _aspawn_anim_bp_parent)
    (bind _asunit_skill_2 (Utilities|Casting|CastToUnit_Skill _item))
    (bind _asatbtt_game_mode (Utilities|Casting|CastToATBTT_GameMode (Game|GetGameMode)))
    (Variables|/Game/AdvancedTurnBasedTileToolkit/Blueprints/Gameplay/BP_Grid_Camera.BP_Grid_Camera_C|SetCustomTarget (Variables|/Game/AdvancedTurnBasedTileToolkit/Blueprints/Gameplay/ATBTT_GameMode.ATBTT_GameMode_C|GetBP_Grid_Camera_Ref _asatbtt_game_mode) (/ (+ (Transformation|GetActorLocation (Variables|Default|GetOwning%20Unit)) (Transformation|GetActorLocation _asunit_skill_2)) 2))
    (Variables|/Game/AdvancedTurnBasedTileToolkit/Blueprints/Gameplay/BP_Grid_Camera.BP_Grid_Camera_C|SetFollow%20Custom%20Target (Variables|/Game/AdvancedTurnBasedTileToolkit/Blueprints/Gameplay/ATBTT_GameMode.ATBTT_GameMode_C|GetBP_Grid_Camera_Ref _asatbtt_game_mode) true)
    (Utilities|FlowControl|Delay 0.5)
    (Audio|PlaySoundatLocation "/Game/AdvancedTurnBasedTileToolkit/Maps/SciFi/Audio/MindControl4.MindControl4" (Math|Vector|MakeVector (.X (Math|Vector|BreakVector (Transformation|GetActorLocation _asunit_skill_2))) (.Y (Math|Vector|BreakVector (Transformation|GetActorLocation _asunit_skill_2))) (+ (.Z (Math|Vector|BreakVector (Transformation|GetActorLocation _asunit_skill_2))) 1.5e+02)))
    (Effects|SpawnEmitteratLocation "/Game/AdvancedTurnBasedTileToolkit/Maps/SciFi/Particles/P_Posseser_Attach.P_Posseser_Attach" (Math|Vector|MakeVector (.X (Math|Vector|BreakVector (Transformation|GetActorLocation _asunit_skill_2))) (.Y (Math|Vector|BreakVector (Transformation|GetActorLocation _asunit_skill_2))) (+ (.Z (Math|Vector|BreakVector (Transformation|GetActorLocation _asunit_skill_2))) 1.5e+02)))
    (Utilities|FlowControl|Delay 0.5)
    (CallFunction|MindControlUnit _asunit_skill_2)
    (CallFunction|DeactivateSkill)
    (Default|ActivateUnit (Variables|Default|GetOwning%20Unit))
    (Default|SetMarkerVisibility _grid_manager_ref false (Variables|/Game/AdvancedTurnBasedTileToolkit/Blueprints/Gameplay/BP_Grid_Manager.BP_Grid_Manager_C|GetTarget%20Marker%20Decal _grid_manager_ref) (Variables|/Game/AdvancedTurnBasedTileToolkit/Blueprints/Gameplay/BP_Grid_Manager.BP_Grid_Manager_C|GetTargetMarker _grid_manager_ref))))

(fn ConstructionScript
  (|CallParentFunction))

(fn FindEnemyUnitinRangeClosesttoAnAlly
  (bind _target_candidates (Variables|Default|GetTarget%20Candidates))
  (bind _local_min_distance_array (LocalVariables|GetLocal%20Min%20Distance%20Array))
  (bind (_indexofminvalue _minvalue) (Math|Integer|MinOfIntArray _local_min_distance_array))
  (bind (_array_element _array_index) (Utilities|ReverseforEachLoop (Variables|Default|GetTarget%20Candidates))
    (:Loop%20Body
      (bind _tiles_in_sight_array (Default|FindUnitsinRange (Variables|Default|GetGrid_Manager_Ref) _array_element 14 false))
      (Utilities|Array|Clear (LocalVariables|GetLocal%20Distance%20Array))
      (for _array_element_2 _tiles_in_sight_array
        (if (!= _array_element _array_element_2)
          (bind _asunit_skill (Utilities|Casting|CastToUnit_Skill (Utilities|Array|Get(acopy) (Variables|/Game/AdvancedTurnBasedTileToolkit/Blueprints/Gameplay/BP_Grid_Manager.BP_Grid_Manager_C|GetPawn%20Array (Variables|Default|GetGrid_Manager_Ref)) _array_element_2)))
          (if (== (Utilities|Array|FindItem (Variables|/Game/AdvancedTurnBasedTileToolkit/Blueprints/Pawns/Unit.Unit_C|GetAllied%20Factions (Variables|Default|GetOwning%20Unit)) (Variables|/Game/AdvancedTurnBasedTileToolkit/Blueprints/Pawns/Unit.Unit_C|GetFaction _asunit_skill)) -1)
            (Utilities|Array|Add (LocalVariables|GetLocal%20Distance%20Array) (Default|FindDistance(inTiles)BetweenIndexes (Variables|Default|GetGrid_Manager_Ref) _array_element _array_element_2 false)))))
      (if (> (Utilities|Array|Length (LocalVariables|GetLocal%20Distance%20Array)) 0)
        (Utilities|Array|Add (LocalVariables|GetLocal%20Min%20Distance%20Array) (.MinValue (Math|Integer|MinOfIntArray (LocalVariables|GetLocal%20Distance%20Array))))
        (else
          (Utilities|Array|RemoveIndex (Variables|Default|GetTarget%20Candidates) _array_index))))
    (:Completed
      (return (> (Utilities|Array|Length _target_candidates) 0) (Utilities|Array|Get(acopy) _target_candidates (- (Utilities|Array|LastIndex _target_candidates) _indexofminvalue)) _minvalue))))

(fn GetHoverText
  (return (Utilities|Text|ToText(String) (Utilities|String|Append (Utilities|String|ToString(Text) (Utilities|Text|MakeLiteralText "Mind Control: 
")) (Utilities|String|ToString(Text) (Utilities|Text|MakeLiteralText "Target unit fights for your faction next turn. 
Range: ")) (Utilities|String|ToString(Integer) (Variables|Default|GetRange)) " 
Cooldown: " (Utilities|String|ToString(Integer) (Variables|Default|GetDefault%20Cooldown))))))

(fn FindTargetValue
  (params (Target%20Index :type Integer))
  (for _array_element (Variables|/Game/AdvancedTurnBasedTileToolkit/Maps/SciFi/Blueprints/Pawns/Unit_Skill.Unit_Skill_C|GetActive%20Effects (.AsUnit%20Skill (Utilities|Casting|CastToUnit_Skill (Utilities|Array|Get(acopy) (Variables|/Game/AdvancedTurnBasedTileToolkit/Blueprints/Gameplay/BP_Grid_Manager.BP_Grid_Manager_C|GetPawn%20Array (Variables|Default|GetGrid_Manager_Ref)) Target%20Index))))
    (if (== (Utilities|GetClass _array_element) "/Game/AdvancedTurnBasedTileToolkit/Maps/SciFi/Blueprints/Skills/SE_MindControlled.SE_MindControlled_C")
      (return 0.0)))
  (bind _target_candidates (CallFunction|FindPotentialTargets Target%20Index 10 false true false))
  (for _array_element_2 _target_candidates
    (Utilities|Array|Add (LocalVariables|GetLocal%20Distance%20Array) (Default|FindDistance(inTiles)BetweenIndexes (Variables|Default|GetGrid_Manager_Ref) Target%20Index _array_element_2 false)))
  (return (* (- 4 (/ (.MinValue (Math|Integer|MinOfIntArray (LocalVariables|GetLocal%20Distance%20Array))) 5)) 0.1)))