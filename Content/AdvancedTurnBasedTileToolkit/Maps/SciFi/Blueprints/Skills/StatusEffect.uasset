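; StatusEffect is an actor for unit status effects in the SciFi turn-based tile toolkit game, apparently a base to build effects on.
; On BeginPlay it caches the grid manager and SciFi game mode.
; ActivateSE attaches it to the target unit and registers it in ActiveEffects; DeactivateSE unregisters and destroys it.
; Turn start and end events only notify the game mode that checks are done, and AcivateEffect is empty.
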(event Custom|On%20Unit%20Turn%20Start
  (Default|StatusEffectStartChecked (Variables|Default|GetGame%20Mode%20Ref)))

(event Custom|Acivate%20Effect
  (params (Target%20Unit :type Unit%20Skill%20Object%20Reference)))

(event Custom|Deactivate%20SE
  (bind _owning_unit (Variables|Default|GetOwning%20Unit))
  (bind _active_effects (Variables|/Game/AdvancedTurnBasedTileToolkit/Maps/SciFi/Blueprints/Pawns/Unit_Skill.Unit_Skill_C|GetActive%20Effects _owning_unit))
  (Utilities|Array|RemoveIndex _active_effects (Utilities|Array|FindItem _active_effects self))
  (Actor|DestroyActor))

(event Custom|Activate%20SE
  (params (Target%20Unit :type Unit%20Skill%20Object%20Reference))
  (Transformation|AttachActorToActor Target%20Unit "None" "SnapToTarget" "KeepRelative" "KeepRelative" true)
  (bind _output_get (Variables|Default|SetOwning%20Unit Target%20Unit))
  (Utilities|Array|Add (Variables|/Game/AdvancedTurnBasedTileToolkit/Maps/SciFi/Blueprints/Pawns/Unit_Skill.Unit_Skill_C|GetActive%20Effects _output_get) self))

(event Custom|On%20Unit%20Turn%20End
  (Default|StatusEffectEndChecked (Variables|Default|GetGame%20Mode%20Ref)))

(event EventBeginPlay
  (bind _outactors (Actor|GetAllActorsOfClass "/Game/AdvancedTurnBasedTileToolkit/Blueprints/Gameplay/BP_Grid_Manager.BP_Grid_Manager_C"))
  (Variables|Default|SetGrid_Manager_Ref (Utilities|Array|Get(acopy) _outactors))
  (bind _asatbtt_game_mode_sci_fi (Utilities|Casting|CastToATBTT_GameMode_SciFi (Game|GetGameMode)))
  (Variables|Default|SetGame%20Mode%20Ref _asatbtt_game_mode_sci_fi))

(event Collision|EventActorBeginOverlap
  (params (OtherActor :type Actor%20Object%20Reference)))

(event EventTick
  (params (DeltaSeconds :type Float%20%28single-precision%29)))

(fn ConstructionScript)