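; Overwatch status effect that lets its owning unit fire a reaction shot at a non-allied unit moving into view.
; It listens to the game mode's tile-entry dispatcher, line-traces from owner to mover, and attacks through the owner's Skill_Laser if unobstructed.
; The target is briefly slowed via speed modifier and time dilation for the shot.
; The effect deactivates afterwards, or at unit turn start, when it also leaves the active effects.
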(event Custom|Check%20Overwatch
  (params (Unit :type Unit%20Object%20Reference) (Index :type Integer) (Location :type Vector))
  (bind _returnvalue (Transformation|GetActorLocation Unit))
  (bind _asunit_skill (Utilities|Casting|CastToUnit_Skill Unit))
  (bind _grid_manager_ref (Variables|Default|GetGrid_Manager_Ref))
  (bind _visibilitytraceheight (Variables|/Game/AdvancedTurnBasedTileToolkit/Blueprints/Gameplay/BP_Grid_Manager.BP_Grid_Manager_C|GetVisibilityTraceHeight _grid_manager_ref))
  ;[1 0.5778 0] Check Overwatch
  (if (== (Utilities|Array|FindItem (Variables|/Game/AdvancedTurnBasedTileToolkit/Blueprints/Pawns/Unit.Unit_C|GetAllied%20Factions (Variables|Default|GetOwning%20Unit)) (Variables|/Game/AdvancedTurnBasedTileToolkit/Blueprints/Pawns/Unit.Unit_C|GetFaction Unit)) -1)
    (bind _returnvalue_2 (Collision|LineTraceByChannel (Math|Vector|MakeVector (.x (Transformation|GetActorLocation (Variables|Default|GetOwning%20Unit))) (.y (Transformation|GetActorLocation (Variables|Default|GetOwning%20Unit))) (+ (.z (Transformation|GetActorLocation (Variables|Default|GetOwning%20Unit))) _visibilitytraceheight)) (Math|Vector|MakeVector (.x _returnvalue) (.y _returnvalue) (+ (.z _returnvalue) _visibilitytraceheight)) "TraceTypeQuery4" false 0 "None"))
    (if (not _returnvalue_2)
      (bind _array_element (Utilities|Array|ForEachLoopwithBreak (Variables|/Game/AdvancedTurnBasedTileToolkit/Maps/SciFi/Blueprints/Pawns/Unit_Skill.Unit_Skill_C|GetSkill%20Child%20Components (Variables|Default|GetOwning%20Unit)) :!label _label)
        (:LoopBody
          (bind _asskill_laser (Utilities|Casting|CastToSkill_Laser (Variables|/Script/Engine.ChildActorComponent|GetChildActor _array_element)))
          (Utilities|FlowControl|Sequence
            (:then_0
              (goto _label Break))
            (:then_1
              (Variables|/Game/AdvancedTurnBasedTileToolkit/Maps/SciFi/Blueprints/Skills/Skill.Skill_C|SetOwning%20Unit _asskill_laser (Variables|Default|GetOwning%20Unit))
              (Variables|/Game/AdvancedTurnBasedTileToolkit/Blueprints/Pawns/Unit.Unit_C|SetSpeed%20Modifier Unit 0.1)
              (Variables|/Script/Engine.Actor|SetCustomTimeDilation _asunit_skill 0.1)
              (Default|AttackUnit _asskill_laser Unit true)
              (Utilities|FlowControl|Delay 1.0)
              (Variables|/Game/AdvancedTurnBasedTileToolkit/Blueprints/Pawns/Unit.Unit_C|SetSpeed%20Modifier Unit 1.0)
              (Variables|/Script/Engine.Actor|SetCustomTimeDilation _asunit_skill 1.0)
              (CallFunction|DeactivateSE))))))))

(event EventBeginPlay
  (|CallParentFunction)
  (EventDispatchers|BindEventtoUnitEntersNewTileDispatcher (Variables|Default|GetGame%20Mode%20Ref) (delegate Custom|Check%20Overwatch)))

(event EventOnUnitTurnStart
  (bind _owning_unit (Variables|Default|GetOwning%20Unit))
  (bind _active_effects (Variables|/Game/AdvancedTurnBasedTileToolkit/Maps/SciFi/Blueprints/Pawns/Unit_Skill.Unit_Skill_C|GetActive%20Effects _owning_unit))
  ;[0.05985 1 0] On Unit Turn Start
  (Utilities|Array|RemoveIndex _active_effects (Utilities|Array|FindItem _active_effects self))
  (|CallParentFunction)
  (CallFunction|DeactivateSE))

(fn ConstructionScript
  (|CallParentFunction))