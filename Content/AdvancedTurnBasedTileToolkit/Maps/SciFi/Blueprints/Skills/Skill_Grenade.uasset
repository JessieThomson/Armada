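; Sci-fi grenade skill for the turn-based tile toolkit that damages every unit, allies included, overlapping an explosion marker around the target tile.
; Players aim with a hover preview, then AttackUnit fires a laser beam, spawns the explosion and spends action points.
; AI moves a search box over potential targets to find clusters, then scores nearby tiles by hits, kills and distance, penalizing friendly fire more heavily.
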(event Custom|Attack%20Unit
  (params (Target%20Index :type Integer))
  (bind _grid_manager_ref (Variables|Default|GetGrid_Manager_Ref))
  (bind _grid_manager_ref_2 (Variables|Default|GetGrid_Manager_Ref))
  (bind _grid_manager_ref_3 (Variables|Default|GetGrid_Manager_Ref))
  ;[0.36 0.009045 0] Attack Unit
  (Variables|Default|SetTarget%20Index Target%20Index)
  (Variables|Default|SetWeapon (Utilities|Array|Get(acopy) (Actor|GetComponentsbyTag (Variables|Default|GetOwning%20Unit) "/Script/Engine.StaticMeshComponent" "Weapon")))
  (Variables|Default|SetLaser (Utilities|Array|Get(acopy) (Actor|GetComponentsbyTag (Variables|Default|GetOwning%20Unit) "/Script/Engine.ParticleSystemComponent" "Laser")))
  (Transformation|SetActorRotation (Variables|Default|GetOwning%20Unit) (Math|Rotator|MakeRotator 0.0 0.0 (.yaw (Math|Rotator|FindLookatRotation (Transformation|GetActorLocation (Variables|Default|GetOwning%20Unit)) (Utilities|Array|Get(acopy) (Variables|/Game/AdvancedTurnBasedTileToolkit/Blueprints/Gameplay/BP_Grid_Manager.BP_Grid_Manager_C|GetVectorFieldArray (Variables|Default|GetGrid_Manager_Ref)) (Variables|Default|GetTarget%20Index))))))
  (bind _aspawn_anim_bp_parent (Utilities|Casting|CastToPawn_Anim_BP_Parent (Components|SkeletalMesh|GetAnimInstance (Utilities|Array|Get(acopy) (Actor|GetComponentsByClass (Variables|Default|GetOwning%20Unit) "/Script/Engine.SkeletalMeshComponent")))))
  (Default|AttackAnimation _aspawn_anim_bp_parent)
  (bind _asatbtt_game_mode (Utilities|Casting|CastToATBTT_GameMode (Game|GetGameMode)))
  (Variables|/Game/AdvancedTurnBasedTileToolkit/Blueprints/Gameplay/BP_Grid_Camera.BP_Grid_Camera_C|SetCustomTarget (Variables|/Game/AdvancedTurnBasedTileToolkit/Blueprints/Gameplay/ATBTT_GameMode.ATBTT_GameMode_C|GetBP_Grid_Camera_Ref _asatbtt_game_mode) (/ (+ (+ (Transformation|GetActorLocation _grid_manager_ref_2) (Utilities|Array|Get(acopy) (Variables|/Game/AdvancedTurnBasedTileToolkit/Blueprints/Gameplay/BP_Grid_Manager.BP_Grid_Manager_C|GetVectorFieldArray _grid_manager_ref_2) (Variables|Default|GetTarget%20Index))) (Transformation|GetActorLocation (Variables|Default|GetOwning%20Unit))) 2))
  (Variables|/Game/AdvancedTurnBasedTileToolkit/Blueprints/Gameplay/BP_Grid_Camera.BP_Grid_Camera_C|SetFollow%20Custom%20Target (Variables|/Game/AdvancedTurnBasedTileToolkit/Blueprints/Gameplay/ATBTT_GameMode.ATBTT_GameMode_C|GetBP_Grid_Camera_Ref _asatbtt_game_mode) true)
  (Utilities|FlowControl|Delay 0.5)
  (Audio|PlaySoundatLocation "/Game/AdvancedTurnBasedTileToolkit/Maps/SciFi/Weapons/laser3.laser3" (Transformation|GetSocketLocation (Variables|Default|GetWeapon) "Muzzle"))
  (Class|ParticleSystemComponent|SetBeamSourcePoint (Variables|Default|GetLaser) 0 (Transformation|GetSocketLocation (Variables|Default|GetWeapon) "Muzzle"))
  (Class|ParticleSystemComponent|SetBeamTargetPoint (Variables|Default|GetLaser) 0 (Math|Vector|MakeVector (.x (+ (Transformation|GetActorLocation _grid_manager_ref) (Utilities|Array|Get(acopy) (Variables|/Game/AdvancedTurnBasedTileToolkit/Blueprints/Gameplay/BP_Grid_Manager.BP_Grid_Manager_C|GetVectorFieldArray _grid_manager_ref) (Variables|Default|GetTarget%20Index)))) (.y (+ (Transformation|GetActorLocation _grid_manager_ref) (Utilities|Array|Get(acopy) (Variables|/Game/AdvancedTurnBasedTileToolkit/Blueprints/Gameplay/BP_Grid_Manager.BP_Grid_Manager_C|GetVectorFieldArray _grid_manager_ref) (Variables|Default|GetTarget%20Index)))) (+ (.z (+ (Transformation|GetActorLocation _grid_manager_ref) (Utilities|Array|Get(acopy) (Variables|/Game/AdvancedTurnBasedTileToolkit/Blueprints/Gameplay/BP_Grid_Manager.BP_Grid_Manager_C|GetVectorFieldArray _grid_manager_ref) (Variables|Default|GetTarget%20Index)))) (* (Variables|/Game/AdvancedTurnBasedTileToolkit/Blueprints/Gameplay/BP_Grid_Manager.BP_Grid_Manager_C|GetVisibilityTraceHeight (Variables|Default|GetGrid_Manager_Ref)) 0.7))))
  (Rendering|SetVisibility (Variables|Default|GetLaser) true false)
  (Utilities|FlowControl|Delay 0.05)
  (Rendering|SetVisibility (Variables|Default|GetLaser) false false)
  (CallFunction|WakeUnitsinRange (Variables|Default|GetTarget%20Index) 0 16)
  (Transformation|SetWorldLocation (Variables|Default|GetExplosionMarker) (+ (Transformation|GetActorLocation _grid_manager_ref_3) (Utilities|Array|Get(acopy) (Variables|/Game/AdvancedTurnBasedTileToolkit/Blueprints/Gameplay/BP_Grid_Manager.BP_Grid_Manager_C|GetVectorFieldArray _grid_manager_ref_3) (Variables|Default|GetTarget%20Index))) false false)
  (bind _returnvalue (Effects|SpawnEmitteratLocation "/Game/AdvancedTurnBasedTileToolkit/Maps/SciFi/Particles/P_Explosion.P_Explosion" (+ (Transformation|GetActorLocation _grid_manager_ref_3) (Utilities|Array|Get(acopy) (Variables|/Game/AdvancedTurnBasedTileToolkit/Blueprints/Gameplay/BP_Grid_Manager.BP_Grid_Manager_C|GetVectorFieldArray _grid_manager_ref_3) (Variables|Default|GetTarget%20Index)))))
  (Transformation|SetWorldScale3D _returnvalue "4.000000,4.000000,4.000000")
  (Audio|PlaySoundatLocation "/Game/AdvancedTurnBasedTileToolkit/Maps/2D_Game_Example/Sound/Fireblast.Fireblast" (+ (Transformation|GetActorLocation _grid_manager_ref_3) (Utilities|Array|Get(acopy) (Variables|/Game/AdvancedTurnBasedTileToolkit/Blueprints/Gameplay/BP_Grid_Manager.BP_Grid_Manager_C|GetVectorFieldArray _grid_manager_ref_3) (Variables|Default|GetTarget%20Index))))
  (CallFunction|PayActionPointCost)
  (for _array_element (Collision|GetOverlappingActors (Variables|Default|GetExplosionMarker) "/Game/AdvancedTurnBasedTileToolkit/Blueprints/Pawns/Unit.Unit_C" :!class /Script/Engine.PrimitiveComponent)
    (bind _asunit (Utilities|Casting|CastToUnit _array_element))
    (Default|ReceiveDamage _asunit (Variables|Default|GetDamage) 0.0))
  (CallFunction|DeactivateSkill)
  (Default|ActivateUnit (Variables|Default|GetOwning%20Unit)))

(event EventAICheckValue
  (params (Unit :type Unit%20Object%20Reference))
  ;[0 0 0] AI
  ;;[0 1 0.2041] Check Value
  (|CallParentFunction Unit)
  (CallFunction|EvaluateSkill false)
  (Utilities|FlowControl|Delay 0.0)
  (bind _move_target_index (CallFunction|FindBestTilefromWhichtoUseSkill))
  (if (not (Variables|Default|GetOnly%20Ckeck%20Value))
    (CallFunction|FindPathandInitializeMovement _move_target_index)))

(event EventAIPrepareandExecuteSkill
  (bind _grid_manager_ref (Variables|Default|GetGrid_Manager_Ref))
  (bind _grid_manager_ref_2 (Variables|Default|GetGrid_Manager_Ref))
  (bind _target_marker_decal (Variables|/Game/AdvancedTurnBasedTileToolkit/Blueprints/Gameplay/BP_Grid_Manager.BP_Grid_Manager_C|GetTarget%20Marker%20Decal _grid_manager_ref))
  (bind _targetmarker (Variables|/Game/AdvancedTurnBasedTileToolkit/Blueprints/Gameplay/BP_Grid_Manager.BP_Grid_Manager_C|GetTargetMarker _grid_manager_ref))
  ;[1 0 0.03273] Prepare Attack
  (Default|SetMarkerLocation (Variables|Default|GetGrid_Manager_Ref) "0.000000,0.000000,0.000000" true (Variables|Default|GetTarget%20Index) _target_marker_decal _targetmarker)
  (Default|SetMarkerVisibility (Variables|Default|GetGrid_Manager_Ref) true _target_marker_decal _targetmarker)
  (Transformation|SetWorldLocation (Variables|Default|GetExplosionMarker) (+ (Transformation|GetActorLocation _grid_manager_ref_2) (Utilities|Array|Get(acopy) (Variables|/Game/AdvancedTurnBasedTileToolkit/Blueprints/Gameplay/BP_Grid_Manager.BP_Grid_Manager_C|GetVectorFieldArray _grid_manager_ref_2) (Variables|Default|GetTarget%20Index))) false false)
  (CallFunction|AttackUnit (Variables|Default|GetTarget%20Index)))

(event EventTileClicked
  (params (Index :type Integer))
  (bind _grid_manager_ref (Variables|Default|GetGrid_Manager_Ref))
  ;[0 0 0] Player
  ;;[1 0.004872 0] Tile Clicked
  (|CallParentFunction Index)
  (bind (_index _location _tracehit) (Default|GetHitTileLocationandIndex (Variables|Default|GetGrid_Manager_Ref)))
  (if _tracehit
    (if (Math|Vector|Equal(Vector) _location (+ (Transformation|GetActorLocation _grid_manager_ref) (Utilities|Array|Get(acopy) (Variables|/Game/AdvancedTurnBasedTileToolkit/Blueprints/Gameplay/BP_Grid_Manager.BP_Grid_Manager_C|GetVectorFieldArray _grid_manager_ref) _index)) (|(sqrt(((square(kat1))+(square(kat2))))) (Variables|/Game/AdvancedTurnBasedTileToolkit/Blueprints/Gameplay/BP_Grid_Manager.BP_Grid_Manager_C|GetTileBoundsX _grid_manager_ref) (Variables|/Game/AdvancedTurnBasedTileToolkit/Blueprints/Gameplay/BP_Grid_Manager.BP_Grid_Manager_C|GetTileBoundsY _grid_manager_ref)))
      (bind _output_get (Variables|Default|SetClicked%20Tile _index))
      (if (> (Utilities|Array|Get(acopy) (Variables|/Game/AdvancedTurnBasedTileToolkit/Blueprints/Gameplay/BP_Grid_Manager.BP_Grid_Manager_C|GetRangeArray (Variables|Default|GetGrid_Manager_Ref)) _output_get) 0)
        (Rendering|SetVisibility (Variables|Default|GetExplosionMarker) false false)
        (Default|SetMarkerVisibility (Variables|Default|GetGrid_Manager_Ref) false (Variables|Default|GetSkill%20Decal) (Variables|Default|GetSkill%20Marker))
        (CallFunction|AttackUnit (Variables|Default|GetClicked%20Tile))
        (bind _asatbtt_player_controller (Utilities|Casting|CastToATBTT_PlayerController (Game|GetPlayerController 0)))
        (Variables|/Game/AdvancedTurnBasedTileToolkit/Blueprints/Gameplay/ATBTT_PlayerController.ATBTT_PlayerController_C|SetDisable%20Player%20Controller%20Input _asatbtt_player_controller true)))))

(event EventActivateSkill
  (params (Unit :type Unit%20Object%20Reference))
  (bind _grid_manager_ref (Variables|Default|GetGrid_Manager_Ref))
  (bind _owning_unit (Variables|Default|GetOwning%20Unit))
  (bind _skill_decal (Variables|Default|GetSkill%20Decal))
  (bind _returnvalue (Transformation|GetWorldScale _skill_decal))
  (|CallParentFunction Unit)
  (if (Variables|/Game/AdvancedTurnBasedTileToolkit/Blueprints/Pawns/Unit.Unit_C|GetAI%20Controlled Unit)
    ;[0 0 0] AI
    (if (== (Variables|/Game/AdvancedTurnBasedTileToolkit/Maps/SciFi/Blueprints/Pawns/Unit_Skill.Unit_Skill_C|GetCurrent%20Action%20Points (.AsUnit%20Skill (Utilities|Casting|CastToUnit_Skill (Variables|Default|GetOwning%20Unit)))) 1)
      (CallFunction|AIPrepareandExecuteSkill)
      (else
        (CallFunction|EvaluateSkill false)
        (Utilities|FlowControl|Delay 0.0)
        (bind _move_target_index (CallFunction|FindBestTilefromWhichtoUseSkill))
        (if (not (Variables|Default|GetOnly%20Ckeck%20Value))
          (CallFunction|FindPathandInitializeMovement _move_target_index))))
    (else
      ;[0 0 0] Player
      (Default|FindTilesinRange (Variables|Default|GetGrid_Manager_Ref) (Variables|/Game/AdvancedTurnBasedTileToolkit/Blueprints/Pawns/Unit.Unit_C|GetIndex _owning_unit) (Variables|Default|GetRange) true false false (not (Variables|/Game/AdvancedTurnBasedTileToolkit/Blueprints/Pawns/Unit.Unit_C|GetSquare%20Visibility _owning_unit)) (* 999 (/ (+ (Variables|/Game/AdvancedTurnBasedTileToolkit/Blueprints/Gameplay/BP_Grid_Manager.BP_Grid_Manager_C|GetTileBoundsX _grid_manager_ref) (Variables|/Game/AdvancedTurnBasedTileToolkit/Blueprints/Gameplay/BP_Grid_Manager.BP_Grid_Manager_C|GetTileBoundsY _grid_manager_ref)) 2.0)) 1 false)
      (CallFunction|SetHUDText "Grenade!")
      (Utilities|FlowControl|DoOnce false
        (:Completed
          (Transformation|SetWorldScale3D _skill_decal (Math|Vector|MakeVector (* (.x _returnvalue) 2.0) (* (.y _returnvalue) 4.0) (* (.z _returnvalue) 4.0))))))))

(event EventDeactivateSkill
  ;[0 0 0] Player
  (|CallParentFunction)
  (Rendering|SetVisibility (Variables|Default|GetExplosionMarker) false false))

(event EventCustomHoverEvent
  (bind _grid_manager_ref (Variables|Default|GetGrid_Manager_Ref))
  (bind _grid_manager_ref_2 (Variables|Default|GetGrid_Manager_Ref))
  (bind _range (Variables|Default|GetRange))
  ;[0 0 0] Player
  ;;[0.4499 0 0.455] Mouse Hover
  (Utilities|FlowControl|Sequence
    (:then_0
      (if (> (Utilities|Array|Get(acopy) (Variables|/Game/AdvancedTurnBasedTileToolkit/Blueprints/Gameplay/BP_Grid_Manager.BP_Grid_Manager_C|GetRangeArray (Variables|Default|GetGrid_Manager_Ref)) (Variables|Default|GetCurrentTileHover)) 0)
        (Transformation|SetWorldLocation (Variables|Default|GetExplosionMarker) (+ (Utilities|Array|Get(acopy) (Variables|/Game/AdvancedTurnBasedTileToolkit/Blueprints/Gameplay/BP_Grid_Manager.BP_Grid_Manager_C|GetVectorFieldArray _grid_manager_ref_2) (Variables|Default|GetCurrentTileHover)) (Transformation|GetActorLocation _grid_manager_ref_2)) false false)
        (Rendering|SetVisibility (Variables|Default|GetExplosionMarker) true false)
        (else
          (Rendering|SetVisibility (Variables|Default|GetExplosionMarker) false false))))
    (:then_1
      (bind _asbp_grid_manager_sci_fi (Utilities|Casting|CastToBP_Grid_Manager_SciFi (Variables|Default|GetGrid_Manager_Ref)))
      (Default|ShowCoverMeshesAroundIndex _asbp_grid_manager_sci_fi (Variables|Default|GetCurrentTileHover))
      (if (Variables|/Game/AdvancedTurnBasedTileToolkit/Blueprints/Gameplay/BP_Grid_Manager.BP_Grid_Manager_C|GetShow%20Crosshairs (Variables|Default|GetGrid_Manager_Ref))
        (Default|RemoveCrosshairs (Variables|Default|GetGrid_Manager_Ref))
        (Default|ShowCrosshaironAllPotentialTargetUnitsinRange (Variables|Default|GetGrid_Manager_Ref) (Variables|Default|GetCurrentTileHover) _range (not (Variables|/Game/AdvancedTurnBasedTileToolkit/Blueprints/Pawns/Unit.Unit_C|GetSquare%20Visibility (Variables|Default|GetOwning%20Unit))) (* _range (/ (+ (Variables|/Game/AdvancedTurnBasedTileToolkit/Blueprints/Gameplay/BP_Grid_Manager.BP_Grid_Manager_C|GetTileBoundsX _grid_manager_ref) (Variables|/Game/AdvancedTurnBasedTileToolkit/Blueprints/Gameplay/BP_Grid_Manager.BP_Grid_Manager_C|GetTileBoundsY _grid_manager_ref)) 2.0)) 1 (Variables|/Game/AdvancedTurnBasedTileToolkit/Blueprints/Pawns/Unit.Unit_C|GetAllied%20Factions (Variables|Default|GetOwning%20Unit)))))))

(fn ConstructionScript
  (|CallParentFunction))

(fn CheckEnemyUnitsOverlappingMarker
  (params (Marker :type Primitive%20Component%20Object%20Reference))
  (bind _overlappingactors (Collision|GetOverlappingActors Marker "/Game/AdvancedTurnBasedTileToolkit/Blueprints/Pawns/Unit.Unit_C" :!class /Script/Engine.PrimitiveComponent))
  (if (> (Utilities|Array|Length _overlappingactors) 0)
    (for _array_element _overlappingactors
      (bind _asunit (Utilities|Casting|CastToUnit _array_element))
      (if (== (Utilities|Array|FindItem (Variables|/Game/AdvancedTurnBasedTileToolkit/Blueprints/Pawns/Unit.Unit_C|GetAllied%20Factions (Variables|Default|GetOwning%20Unit)) (Variables|/Game/AdvancedTurnBasedTileToolkit/Blueprints/Pawns/Unit.Unit_C|GetFaction _asunit)) -1)
        (Math|Integer|IncrementInt (LocalVariables|GetEnemy%20Unit%20Count)
          (:%20%20
            (if (<= (- (Variables|/Game/AdvancedTurnBasedTileToolkit/Blueprints/Pawns/Unit.Unit_C|GetCurrentHealth _asunit) (Variables|Default|GetDamage)) 0.0)
              (Math|Integer|IncrementInt (LocalVariables|GetEnemy%20Killed%20Units%20Count)))))
        (else
          (Math|Integer|IncrementInt (LocalVariables|GetFriendly%20Units%20Count)
            (:%20%20
              (if (<= (- (Variables|/Game/AdvancedTurnBasedTileToolkit/Blueprints/Pawns/Unit.Unit_C|GetCurrentHealth _asunit) (Variables|Default|GetDamage)) 0.0)
                (Math|Integer|IncrementInt (LocalVariables|GetFriendly%20Killed%20Units%20Count))))))))
    (return (LocalVariables|GetEnemy%20Unit%20Count) (LocalVariables|GetEnemy%20Killed%20Units%20Count) (LocalVariables|GetFriendly%20Units%20Count) (LocalVariables|GetFriendly%20Killed%20Units%20Count))))

(fn AIPriorityModifier
  (params (Current%20Index :type Integer) (Target%20Index :type Integer))
  (bind _priority (|CallParentFunction Current%20Index Target%20Index))
  (return _priority))

(fn GetHoverText
  (return (Utilities|Text|ToText(String) (Utilities|String|Append (Utilities|String|ToString(Text) (Utilities|Text|MakeLiteralText "Explosive Shot: 
")) (Utilities|String|ToString(Text) (Utilities|Text|MakeLiteralText "Deal ")) (Utilities|String|ToString(Integer) (Math|Float|Truncate (Variables|Default|GetDamage))) (Utilities|String|ToString(Text) (Utilities|Text|MakeLiteralText " damage to all units within 1 tile of target. 
Range: ")) (Utilities|String|ToString(Integer) (Variables|Default|GetRange)) " 
Charges: " (Utilities|String|ToString(Integer) (Variables|Default|GetCurrent%20Charges))))))

(fn FindTargetValue
  (params (Target%20Index :type Integer))
  (bind _grid_manager_ref (Variables|Default|GetGrid_Manager_Ref))
  (Transformation|SetWorldLocation (Variables|Default|GetExplosionMarker) (+ (Transformation|GetActorLocation _grid_manager_ref) (Utilities|Array|Get(acopy) (Variables|/Game/AdvancedTurnBasedTileToolkit/Blueprints/Gameplay/BP_Grid_Manager.BP_Grid_Manager_C|GetVectorFieldArray _grid_manager_ref) Target%20Index)) false false)
  (bind (_enemy_units_hit _enemy_units_killed _friendly_units_hit _friendly_units_killed) (CallFunction|CheckEnemyUnitsOverlappingMarker (Variables|Default|GetExplosionMarker)))
  (return (* (/ 1.0 (Math|Conversions|ToFloat(Integer) (+ (Default|FindDistance(inTiles)BetweenIndexes (Variables|Default|GetGrid_Manager_Ref) (Variables|/Game/AdvancedTurnBasedTileToolkit/Blueprints/Pawns/Unit.Unit_C|GetIndex (Variables|Default|GetOwning%20Unit)) Target%20Index false) 10))) (+ (* _enemy_units_hit 0.3) (* _enemy_units_killed 0.3) (* _friendly_units_hit -0.6) (* _friendly_units_killed -0.6)))))

(fn EvaluateSkill
  (params (Find%20Allies :type Boolean))
  (bind _grid_manager_ref (Variables|Default|GetGrid_Manager_Ref))
  (bind _owning_unit (Variables|Default|GetOwning%20Unit))
  (bind _asunit_skill (Utilities|Casting|CastToUnit_Skill _owning_unit))
  (bind _target_candidates (CallFunction|FindPotentialTargets (Variables|/Game/AdvancedTurnBasedTileToolkit/Blueprints/Pawns/Unit.Unit_C|GetIndex _asunit_skill) (+ (Variables|Default|GetRange) (* (- (Variables|/Game/AdvancedTurnBasedTileToolkit/Maps/SciFi/Blueprints/Pawns/Unit_Skill.Unit_Skill_C|GetCurrent%20Action%20Points _asunit_skill) 1) (Variables|/Game/AdvancedTurnBasedTileToolkit/Blueprints/Pawns/Unit.Unit_C|GetCurrent%20Move _owning_unit))) false true false))
  (for _array_element _target_candidates
    (Transformation|SetWorldLocation (Variables|Default|GetAIExplosionSearchBox) (+ (Transformation|GetActorLocation _grid_manager_ref) (Utilities|Array|Get(acopy) (Variables|/Game/AdvancedTurnBasedTileToolkit/Blueprints/Gameplay/BP_Grid_Manager.BP_Grid_Manager_C|GetVectorFieldArray _grid_manager_ref) _array_element)) false false)
    (if (> (Utilities|Array|Length (Collision|GetOverlappingActors (Variables|Default|GetAIExplosionSearchBox) "/Game/AdvancedTurnBasedTileToolkit/Blueprints/Pawns/Unit.Unit_C" :!class /Script/Engine.PrimitiveComponent)) 1)
      (Default|GetIndexesinRange (Variables|Default|GetGrid_Manager_Ref) _array_element 1 false false)
      (for _array_element_2 (Variables|/Game/AdvancedTurnBasedTileToolkit/Blueprints/Gameplay/BP_Grid_Manager.BP_Grid_Manager_C|GetTilesInRangeArray (Variables|Default|GetGrid_Manager_Ref))
        (if (not (Default|IsTileImpassable? (Variables|Default|GetGrid_Manager_Ref) (.index _array_element_2)))
          (Utilities|Array|Add (LocalVariables|GetLocal%20Target%20Candidates) (.index _array_element_2))))))
  (Utilities|Array|AppendArray (Variables|Default|GetTarget%20Candidates) (LocalVariables|GetLocal%20Target%20Candidates))
  (bind _found_units_ (Default|FindUnitsinSightfromMoveArray (Variables|Default|GetGrid_Manager_Ref) (Variables|Default|GetTarget%20Candidates) (Variables|Default|GetRange) false false))
  (bind _output_get (Variables|Default|SetTarget%20Candidates _found_units_))
  (bind (_target_index _ai_estimated_value) (CallFunction|FindBestTarget _output_get))
  (return _target_index _ai_estimated_value))