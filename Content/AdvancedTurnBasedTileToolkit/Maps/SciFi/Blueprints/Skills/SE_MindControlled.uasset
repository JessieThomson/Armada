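; Mind control status effect for the turn-based SciFi map, which makes the owning unit act under AI control as an ally of the controlling unit for one turn.
; On turn start it saves the unit's allied factions and AI flag, overrides both, and plays a sound and particle effect above the unit.
; On turn end it restores both values, removes itself from the unit's active effects and deactivates.
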(event EventBeginPlay)

(event Collision|EventActorBeginOverlap
  (params (OtherActor :type Actor%20Object%20Reference)))

(event EventOnUnitTurnStart
  (bind _owning_unit (Variables|Default|GetOwning%20Unit))
  (bind _owning_unit_2 (Variables|Default|GetOwning%20Unit))
  (bind _returnvalue (Transformation|GetActorLocation _owning_unit_2))
  (bind _returnvalue_2 (+ (.z _returnvalue) 1.5e+02))
  ;[0 1 0.07301] On Unit Turn Start
  (Variables|Default|SetOld%20Allied%20Factions (Variables|/Game/AdvancedTurnBasedTileToolkit/Blueprints/Pawns/Unit.Unit_C|GetAllied%20Factions _owning_unit))
  (Variables|/Game/AdvancedTurnBasedTileToolkit/Blueprints/Pawns/Unit.Unit_C|SetAllied%20Factions _owning_unit (Variables|/Game/AdvancedTurnBasedTileToolkit/Blueprints/Pawns/Unit.Unit_C|GetAllied%20Factions (Variables|Default|GetControlling%20Unit)))
  (Variables|Default|SetOld%20AI%20Controlled (Variables|/Game/AdvancedTurnBasedTileToolkit/Blueprints/Pawns/Unit.Unit_C|GetAI%20Controlled _owning_unit))
  (Variables|/Game/AdvancedTurnBasedTileToolkit/Blueprints/Pawns/Unit.Unit_C|SetAI%20Controlled _owning_unit true)
  (Audio|PlaySoundatLocation "/Game/AdvancedTurnBasedTileToolkit/Maps/SciFi/Audio/MindControl4.MindControl4" (Math|Vector|MakeVector (.x _returnvalue) (.y _returnvalue) _returnvalue_2))
  (Effects|SpawnEmitteratLocation "/Game/AdvancedTurnBasedTileToolkit/Maps/SciFi/Particles/P_Posseser_Attach.P_Posseser_Attach" (Math|Vector|MakeVector (.x _returnvalue) (.y _returnvalue) _returnvalue_2))
  (|CallParentFunction))

(event EventOnUnitTurnEnd
  (bind _owning_unit (Variables|Default|GetOwning%20Unit))
  (bind _active_effects (Variables|/Game/AdvancedTurnBasedTileToolkit/Maps/SciFi/Blueprints/Pawns/Unit_Skill.Unit_Skill_C|GetActive%20Effects _owning_unit))
  ;[1 0.05001 0] On Turn End
  (Variables|/Game/AdvancedTurnBasedTileToolkit/Blueprints/Pawns/Unit.Unit_C|SetAllied%20Factions _owning_unit (Variables|Default|GetOld%20Allied%20Factions))
  (Variables|/Game/AdvancedTurnBasedTileToolkit/Blueprints/Pawns/Unit.Unit_C|SetAI%20Controlled _owning_unit (Variables|Default|GetOld%20AI%20Controlled))
  (Utilities|Array|RemoveIndex _active_effects (Utilities|Array|FindItem _active_effects self))
  (|CallParentFunction)
  (CallFunction|DeactivateSE))

(event EventTick
  (params (DeltaSeconds :type Float%20%28single-precision%29)))

(fn ConstructionScript
  (|CallParentFunction))