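; Overwatch skill for the SciFi tactics example, described in its hover text as firing at enemies that move to a visible tile in range.
; Activation spawns an SE_Overwatch status effect on the owning unit, pays the action point cost, then deactivates the skill and reactivates the unit.
; AI units first reset their estimated value and skip the effect when out of action points.
; The AI priority modifier is always neutral.
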(event EventBeginPlay
  (|CallParentFunction)
  (Utilities|Casting|CastToATBTT_GameMode_SciFi (Variables|Default|GetGame%20Mode%20Ref)))

(event EventActivateSkill
  (params (Unit :type Unit%20Object%20Reference))
  ;[0.09307 1 0] Activate Skill
  (|CallParentFunction Unit)
  (if (Variables|/Game/AdvancedTurnBasedTileToolkit/Blueprints/Pawns/Unit.Unit_C|GetAI%20Controlled Unit)
    (Variables|Default|SetAI%20Estimated%20Value -9999999.0) ; Reset the estimated value
    (bind _asunit_skill (Utilities|Casting|CastToUnit_Skill (Variables|Default|GetOwning%20Unit)))
    (switch int (Variables|/Game/AdvancedTurnBasedTileToolkit/Maps/SciFi/Blueprints/Pawns/Unit_Skill.Unit_Skill_C|GetCurrent%20Action%20Points _asunit_skill)
      (:Default
        (bind _returnvalue (Game|SpawnActorfromClass "/Game/AdvancedTurnBasedTileToolkit/Maps/SciFi/Blueprints/Skills/SE_Overwatch.SE_Overwatch_C" (Math|Conversions|ToTransform(Vector) (Transformation|GetActorLocation)) "Undefined" 0 0 :!label _label))
        (bind _asunit_skill_2 (Utilities|Casting|CastToUnit_Skill (Variables|Default|GetOwning%20Unit)))
        (Default|ActivateSE _returnvalue _asunit_skill_2)
        (CallFunction|PayActionPointCost)
        (CallFunction|DeactivateSkill)
        (Default|ActivateUnit (Variables|Default|GetOwning%20Unit)))
      (:0
        (CallFunction|DeactivateSkill)
        (Default|ActivateUnit (Variables|Default|GetOwning%20Unit)))
      (:1
        (goto _label)))
    (else
      (goto _label))))

(fn ConstructionScript
  (|CallParentFunction))

(fn AIPriorityModifier
  (params (Current%20Index :type Integer) (Target%20Index :type Integer))
  (return 0.0))

(fn GetHoverText
  (return (Utilities|Text|ToText(String) (Utilities|String|Append (Utilities|String|ToString(Text) (Utilities|Text|MakeLiteralText "Overwatch: 
")) (Utilities|String|ToString(Text) (Utilities|Text|MakeLiteralText "Fire at any anemy target that moves to a visible 
tile in range."))))))