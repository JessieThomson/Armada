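; Medpack skill for the turn-based tile toolkit that heals a same-faction unit, either self or adjacent, by HealAmount.
; Players pick a target from highlighted range-1 tiles, while AI scores targets by missing health and either moves or heals based on action points.
; Both paths pay action points, play the attack animation and call HealTarget, which after a short delay plays effects, clamps health, updates the health bar and reactivates the owner.
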(event Custom|Heal%20Target
  (params (Target%20Unit :type Unit%20Skill%20Object%20Reference))
  (bind _returnvalue (Transformation|GetActorLocation Target%20Unit))
  (bind _grid_manager_ref (Variables|Default|GetGrid_Manager_Ref))
  (bind _grid_manager_ref_2 (Variables|Default|GetGrid_Manager_Ref))
  (bind _targetmarker (Variables|/Game/AdvancedTurnBasedTileToolkit/Blueprints/Gameplay/BP_Grid_Manager.BP_Grid_Manager_C|GetTargetMarker _grid_manager_ref_2))
  (bind _target_marker_decal (Variables|/Game/AdvancedTurnBasedTileToolkit/Blueprints/Gameplay/BP_Grid_Manager.BP_Grid_Manager_C|GetTarget%20Marker%20Decal _grid_manager_ref_2))
  ;[1 0 0] Heal Target
  (Default|SetMarkerLocation (Variables|Default|GetGrid_Manager_Ref) "0, 0, 0" false (Variables|/Game/AdvancedTurnBasedTileToolkit/Blueprints/Pawns/Unit.Unit_C|GetIndex Target%20Unit) _target_marker_decal _targetmarker)
  (Default|SetMarkerVisibility (Variables|Default|GetGrid_Manager_Ref) true _target_marker_decal _targetmarker)
  (Transformation|SetActorRotation (Math|Rotator|MakeRotator 0.0 0.0 (.yaw (Math|Rotator|FindLookatRotation (Transformation|GetActorLocation) (Transformation|GetActorLocation Target%20Unit)))))
  (Utilities|FlowControl|Delay 0.6)
  (bind _returnvalue_2 (Effects|SpawnEmitteratLocation "/Game/AdvancedTurnBasedTileToolkit/Maps/SciFi/Particles/P_Heal_Target.P_Heal_Target" _returnvalue))
  (Transformation|SetWorldScale3D _returnvalue_2 "2.000000,2.000000,2.000000")
  (Audio|PlaySoundatLocation "/Game/AdvancedTurnBasedTileToolkit/Maps/2D_Game_Example/Sound/Potion.Potion" _returnvalue)
  (Variables|/Game/AdvancedTurnBasedTileToolkit/Blueprints/Pawns/Unit.Unit_C|SetCurrentHealth Target%20Unit (Math|Float|Min(Float) (+ (Variables|/Game/AdvancedTurnBasedTileToolkit/Blueprints/Pawns/Unit.Unit_C|GetCurrentHealth Target%20Unit) (Variables|Default|GetHeal%20Amount)) (Variables|/Game/AdvancedTurnBasedTileToolkit/Blueprints/Pawns/Unit.Unit_C|GetMaxHealth Target%20Unit)))
  (Rendering|Material|SetScalarParameterValue (Variables|/Game/AdvancedTurnBasedTileToolkit/Blueprints/Pawns/Unit.Unit_C|GetDynamic%20Health%20Bar%20Material Target%20Unit) "PercentFill" (/ (Variables|/Game/AdvancedTurnBasedTileToolkit/Blueprints/Pawns/Unit.Unit_C|GetCurrentHealth Target%20Unit) (Variables|/Game/AdvancedTurnBasedTileToolkit/Blueprints/Pawns/Unit.Unit_C|GetMaxHealth Target%20Unit)) :!class /Script/Engine.MaterialInstanceDynamic)
  (Default|SetMarkerVisibility _grid_manager_ref false (Variables|/Game/AdvancedTurnBasedTileToolkit/Blueprints/Gameplay/BP_Grid_Manager.BP_Grid_Manager_C|GetTarget%20Marker%20Decal _grid_manager_ref) (Variables|/Game/AdvancedTurnBasedTileToolkit/Blueprints/Gameplay/BP_Grid_Manager.BP_Grid_Manager_C|GetTargetMarker _grid_manager_ref))
  (CallFunction|DeactivateSkill)
  (Default|ActivateUnit (Variables|Default|GetOwning%20Unit)))

(event EventAICheckValue
  (params (Unit :type Unit%20Object%20Reference))
  ;[0 0 0] AI
  ;;[0 1 0.2041] Check Value
  (|CallParentFunction Unit)
  (CallFunction|EvaluateSkill true)
  (Utilities|FlowControl|Delay 0.0)
  (bind _move_target_index (CallFunction|FindBestTilefromWhichtoUseSkill))
  (if (not (Variables|Default|GetOnly%20Ckeck%20Value))
    (CallFunction|FindPathandInitializeMovement _move_target_index)))

(event EventAIPrepareandExecuteSkill
  (bind _target_index (Variables|Default|GetTarget%20Index))
  (bind _grid_manager_ref (Variables|Default|GetGrid_Manager_Ref))
  (bind _target_marker_decal (Variables|/Game/AdvancedTurnBasedTileToolkit/Blueprints/Gameplay/BP_Grid_Manager.BP_Grid_Manager_C|GetTarget%20Marker%20Decal _grid_manager_ref))
  (bind _targetmarker (Variables|/Game/AdvancedTurnBasedTileToolkit/Blueprints/Gameplay/BP_Grid_Manager.BP_Grid_Manager_C|GetTargetMarker _grid_manager_ref))
  (bind _pawn_array (Variables|/Game/AdvancedTurnBasedTileToolkit/Blueprints/Gameplay/BP_Grid_Manager.BP_Grid_Manager_C|GetPawn%20Array _grid_manager_ref))
  (bind _item (Utilities|Array|Get(acopy) _pawn_array _target_index))
  ;[0 0 0] AI
  ;;[1 0 0] Prepare Heal
  (if (not (Variables|Default|GetOnly%20Ckeck%20Value)) ; Temporary. Full version should check value no matter the amount of action points
    (CallFunction|PayActionPointCost)
    (Default|SetMarkerLocation (Variables|Default|GetGrid_Manager_Ref) "0.000000,0.000000,0.000000" true (Variables|Default|GetTarget%20Index) _target_marker_decal _targetmarker)
    (Default|SetMarkerVisibility (Variables|Default|GetGrid_Manager_Ref) true _target_marker_decal _targetmarker)
    (Transformation|SetActorRotation (Variables|Default|GetOwning%20Unit) (Math|Rotator|MakeRotator 0.0 0.0 (.yaw (Math|Rotator|FindLookatRotation (Transformation|GetActorLocation (Variables|Default|GetOwning%20Unit)) (Transformation|GetActorLocation _item)))))
    (bind _asunit_skill (Utilities|Casting|CastToUnit_Skill (Variables|Default|GetOwning%20Unit)))
    (bind _aspawn_anim_bp_parent (Utilities|Casting|CastToPawn_Anim_BP_Parent (Components|SkeletalMesh|GetAnimInstance (Variables|/Game/AdvancedTurnBasedTileToolkit/Maps/SciFi/Blueprints/Pawns/Unit_Skill.Unit_Skill_C|GetSkeletalMesh _asunit_skill))))
    (Default|AttackAnimation _aspawn_anim_bp_parent)
    (bind _asunit_skill_2 (Utilities|Casting|CastToUnit_Skill _item))
    (CallFunction|HealTarget _asunit_skill_2)))

(event EventActivateSkill
  (params (Unit :type Unit%20Object%20Reference))
  (bind _owning_unit (Variables|Default|GetOwning%20Unit))
  (bind _grid_manager_ref (Variables|Default|GetGrid_Manager_Ref))
  ;[0 1 0.0231] Activate Skill
  (|CallParentFunction Unit)
  (if (Variables|/Game/AdvancedTurnBasedTileToolkit/Blueprints/Pawns/Unit.Unit_C|GetAI%20Controlled Unit)
    ;[0 0 0] AI
    (if (== (Variables|/Game/AdvancedTurnBasedTileToolkit/Maps/SciFi/Blueprints/Pawns/Unit_Skill.Unit_Skill_C|GetCurrent%20Action%20Points (.AsUnit%20Skill (Utilities|Casting|CastToUnit_Skill (Variables|Default|GetOwning%20Unit)))) 1)
      (CallFunction|AIPrepareandExecuteSkill)
      (else
        (CallFunction|EvaluateSkill true)
        (Utilities|FlowControl|Delay 0.0)
        (bind _move_target_index (CallFunction|FindBestTilefromWhichtoUseSkill))
        (if (not (Variables|Default|GetOnly%20Ckeck%20Value))
          (CallFunction|FindPathandInitializeMovement _move_target_index))))
    (else
      (Default|ClearAllinRangeMeshMarkers (Variables|Default|GetGrid_Manager_Ref))
      (Default|Pathfinding (Variables|Default|GetGrid_Manager_Ref) (Variables|/Game/AdvancedTurnBasedTileToolkit/Blueprints/Pawns/Unit.Unit_C|GetIndex (Variables|Default|GetOwning%20Unit)) 0 false 0 false "NewEnumerator0")
      (Default|FindTilesinRange (Variables|Default|GetGrid_Manager_Ref) (Variables|/Game/AdvancedTurnBasedTileToolkit/Blueprints/Pawns/Unit.Unit_C|GetIndex _owning_unit) 1 true false true (not (Variables|/Game/AdvancedTurnBasedTileToolkit/Blueprints/Pawns/Unit.Unit_C|GetSquare%20Visibility _owning_unit)) (* 1 (/ (+ (Variables|/Game/AdvancedTurnBasedTileToolkit/Blueprints/Gameplay/BP_Grid_Manager.BP_Grid_Manager_C|GetTileBoundsX _grid_manager_ref) (Variables|/Game/AdvancedTurnBasedTileToolkit/Blueprints/Gameplay/BP_Grid_Manager.BP_Grid_Manager_C|GetTileBoundsY _grid_manager_ref)) 2.0)) (Variables|/Game/AdvancedTurnBasedTileToolkit/Blueprints/Pawns/Unit.Unit_C|GetMinimum%20Range _owning_unit) false))))

(event EventTileClicked
  (params (Index :type Integer))
  (bind _clicked_tile (Variables|Default|GetClicked%20Tile))
  (bind _grid_manager_ref (Variables|Default|GetGrid_Manager_Ref))
  (bind _pawn_array (Variables|/Game/AdvancedTurnBasedTileToolkit/Blueprints/Gameplay/BP_Grid_Manager.BP_Grid_Manager_C|GetPawn%20Array _grid_manager_ref))
  (bind _item (Utilities|Array|Get(acopy) _pawn_array _clicked_tile))
  ;[1 0.9901 0] Event Tile Clicked
  (|CallParentFunction Index)
  (if (Utilities|IsValid _item) ; Does the clicked tile contain a unit?
    (if (== (Variables|/Game/AdvancedTurnBasedTileToolkit/Blueprints/Pawns/Unit.Unit_C|GetFaction _item) (Variables|/Game/AdvancedTurnBasedTileToolkit/Blueprints/Pawns/Unit.Unit_C|GetFaction (Variables|Default|GetOwning%20Unit))) ; Is the unit the same faction than the one owning the skill?
      (bind _asunit_skill (Utilities|Casting|CastToUnit_Skill _item))
      (CallFunction|HealTarget _asunit_skill)
      (CallFunction|PayActionPointCost)
      (Transformation|SetActorRotation (Variables|Default|GetOwning%20Unit) (Math|Rotator|MakeRotator 0.0 0.0 (.yaw (Math|Rotator|FindLookatRotation (Transformation|GetActorLocation (Variables|Default|GetOwning%20Unit)) (Transformation|GetActorLocation _asunit_skill)))))
      (bind _asunit_skill_2 (Utilities|Casting|CastToUnit_Skill (Variables|Default|GetOwning%20Unit)))
      (bind _aspawn_anim_bp_parent (Utilities|Casting|CastToPawn_Anim_BP_Parent (Components|SkeletalMesh|GetAnimInstance (Variables|/Game/AdvancedTurnBasedTileToolkit/Maps/SciFi/Blueprints/Pawns/Unit_Skill.Unit_Skill_C|GetSkeletalMesh _asunit_skill_2))))
      (Default|AttackAnimation _aspawn_anim_bp_parent)
      (bind _asatbtt_player_controller (Utilities|Casting|CastToATBTT_PlayerController (Game|GetPlayerController 0)))
      (Variables|/Game/AdvancedTurnBasedTileToolkit/Blueprints/Gameplay/ATBTT_PlayerController.ATBTT_PlayerController_C|SetDisable%20Player%20Controller%20Input _asatbtt_player_controller true))))

(fn ConstructionScript
  (|CallParentFunction))

(fn GetHoverText
  (return (Utilities|Text|ToText(String) (Utilities|String|Append (Utilities|String|ToString(Text) (Utilities|Text|MakeLiteralText "Medpack: 
")) (Utilities|String|ToString(Text) (Utilities|Text|MakeLiteralText "Heal self or an adjacent target for ")) (Utilities|String|ToString(Integer) (Math|Float|Truncate (Variables|Default|GetHeal%20Amount))) (Utilities|String|ToString(Text) (Utilities|Text|MakeLiteralText " HP.")) " 
Charges: " (Utilities|String|ToString(Integer) (Variables|Default|GetCurrent%20Charges))))))

(fn FindTargetValue
  (params (Target%20Index :type Integer))
  (bind _grid_manager_ref (Variables|Default|GetGrid_Manager_Ref))
  (bind _pawn_array (Variables|/Game/AdvancedTurnBasedTileToolkit/Blueprints/Gameplay/BP_Grid_Manager.BP_Grid_Manager_C|GetPawn%20Array _grid_manager_ref))
  (bind _item (Utilities|Array|Get(acopy) _pawn_array Target%20Index))
  (return (- (Variables|/Game/AdvancedTurnBasedTileToolkit/Blueprints/Pawns/Unit.Unit_C|GetMaxHealth _item) (Variables|/Game/AdvancedTurnBasedTileToolkit/Blueprints/Pawns/Unit.Unit_C|GetCurrentHealth _item))))