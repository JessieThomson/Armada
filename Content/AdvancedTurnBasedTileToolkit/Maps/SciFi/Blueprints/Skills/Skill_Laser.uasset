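; Laser rifle skill for the sci-fi turn-based tile toolkit: a ranged attack whose hit chance falls with distance.
; Players pick from highlighted visible targets with hit odds on hover; AI scores tiles and targets by hit chance, proximity and kill potential, sometimes choosing Overwatch for distant, low-odds shots.
; AttackUnit, which also supports overwatch shots, rolls the hit, fires a particle beam that overshoots on misses, wakes nearby units and applies damage.
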(event Custom|Attack%20Unit
  (params (Target%20Unit :type Unit%20Object%20Reference) (From%20Overwatch :type Boolean))
  (bind _grid_manager_ref (Variables|Default|GetGrid_Manager_Ref))
  (bind _grid_manager_ref_2 (Variables|Default|GetGrid_Manager_Ref))
  (bind _owning_unit (Variables|Default|GetOwning%20Unit))
  (bind _owning_unit_2 (Variables|Default|GetOwning%20Unit))
  (bind _grid_manager_ref_3 (Variables|Default|GetGrid_Manager_Ref))
  (bind _grid_manager_ref_4 (Variables|Default|GetGrid_Manager_Ref))
  (bind _damage_range (Variables|Default|GetDamage%20Range))
  (bind _returnvalue (Transformation|GetActorLocation _owning_unit))
  (bind (_asunit_skill _bsuccess) (Utilities|Casting|CastToUnit_Skill _owning_unit_2))
  (bind _targetmarker (Variables|/Game/AdvancedTurnBasedTileToolkit/Blueprints/Gameplay/BP_Grid_Manager.BP_Grid_Manager_C|GetTargetMarker _grid_manager_ref_2))
  (bind _target_marker_decal (Variables|/Game/AdvancedTurnBasedTileToolkit/Blueprints/Gameplay/BP_Grid_Manager.BP_Grid_Manager_C|GetTarget%20Marker%20Decal _grid_manager_ref_2))
  (bind _visibilitytraceheight (Variables|/Game/AdvancedTurnBasedTileToolkit/Blueprints/Gameplay/BP_Grid_Manager.BP_Grid_Manager_C|GetVisibilityTraceHeight _grid_manager_ref_3))
  (bind _returnvalue_2 (* _visibilitytraceheight 0.7))
  ;[0 0 0] Player
  ;;[0.175 0 0.008787] Attack Unit
  (Variables|Default|SetFrom%20Overwatch From%20Overwatch)
  (Variables|Default|SetTarget Target%20Unit)
  (Variables|Default|SetWeapon (Utilities|Array|Get(acopy) (Actor|GetComponentsbyTag (Variables|Default|GetOwning%20Unit) "/Script/Engine.StaticMeshComponent" "Weapon")))
  (Variables|Default|SetLaser (Utilities|Array|Get(acopy) (Actor|GetComponentsbyTag (Variables|Default|GetOwning%20Unit) "/Script/Engine.ParticleSystemComponent" "Laser")))
  (Utilities|FlowControl|Sequence
    (:then_0
      ;;;[0 0 0] Visualize Preparation
      (Transformation|SetActorRotation (Variables|Default|GetOwning%20Unit) (Math|Rotator|MakeRotator 0.0 0.0 (.yaw (Math|Rotator|FindLookatRotation _returnvalue (Transformation|GetActorLocation (Variables|Default|GetTarget))))))
      (if (not (Variables|Default|GetFrom%20Overwatch))
        (if (> (Default|FindDistance(inTiles)BetweenIndexes _grid_manager_ref (Variables|/Game/AdvancedTurnBasedTileToolkit/Blueprints/Pawns/Unit.Unit_C|GetIndex (Variables|Default|GetOwning%20Unit)) (Variables|/Game/AdvancedTurnBasedTileToolkit/Blueprints/Pawns/Unit.Unit_C|GetIndex (Variables|Default|GetTarget)) (not (Variables|/Game/AdvancedTurnBasedTileToolkit/Blueprints/Gameplay/BP_Grid_Manager.BP_Grid_Manager_C|GetDiagonal%20Movement _grid_manager_ref))) 1)
          (bind _asatbtt_game_mode (Utilities|Casting|CastToATBTT_GameMode (Game|GetGameMode)))
          (Variables|/Game/AdvancedTurnBasedTileToolkit/Blueprints/Gameplay/BP_Grid_Camera.BP_Grid_Camera_C|SetCustomTarget (Variables|/Game/AdvancedTurnBasedTileToolkit/Blueprints/Gameplay/ATBTT_GameMode.ATBTT_GameMode_C|GetBP_Grid_Camera_Ref _asatbtt_game_mode) (/ (+ _returnvalue (Transformation|GetActorLocation (Variables|Default|GetTarget))) 2))
          (Variables|/Game/AdvancedTurnBasedTileToolkit/Blueprints/Gameplay/BP_Grid_Camera.BP_Grid_Camera_C|SetFollow%20Custom%20Target (Variables|/Game/AdvancedTurnBasedTileToolkit/Blueprints/Gameplay/ATBTT_GameMode.ATBTT_GameMode_C|GetBP_Grid_Camera_Ref _asatbtt_game_mode) true))
        (if (not (Variables|/Game/AdvancedTurnBasedTileToolkit/Blueprints/Pawns/Unit.Unit_C|GetAI%20Controlled (Variables|Default|GetOwning%20Unit)))
          (Default|SetMarkerLocation (Variables|Default|GetGrid_Manager_Ref) "0, 0, 0" false (Variables|/Game/AdvancedTurnBasedTileToolkit/Blueprints/Pawns/Unit.Unit_C|GetIndex (Variables|Default|GetTarget)) _target_marker_decal _targetmarker)
          (Default|SetMarkerVisibility (Variables|Default|GetGrid_Manager_Ref) true _target_marker_decal _targetmarker))))
    (:then_1
      ;;;[0 0 0] Check if attack hits
      (Utilities|FlowControl|Delay 0.5)
      (bind _asunit_skill_2 (Utilities|Casting|CastToUnit_Skill (Variables|Default|GetTarget))
        (:then
          (bind _asbp_grid_manager_sci_fi (Utilities|Casting|CastToBP_Grid_Manager_SciFi (Variables|Default|GetGrid_Manager_Ref))
            (:then
              (bind _hit (Default|CalculateHitChance _asbp_grid_manager_sci_fi (+ (Variables|/Game/AdvancedTurnBasedTileToolkit/Maps/SciFi/Blueprints/Pawns/Unit_Skill.Unit_Skill_C|GetDodge _asunit_skill_2) (Math|Float|SelectFloat (Variables|/Game/AdvancedTurnBasedTileToolkit/Maps/SciFi/Blueprints/Pawns/Unit_Skill.Unit_Skill_C|GetAccuracy _asunit_skill) 1.0 _bsuccess)) -0.05 0.0 (Variables|/Game/AdvancedTurnBasedTileToolkit/Blueprints/Pawns/Unit.Unit_C|GetIndex _asunit_skill) (Variables|/Game/AdvancedTurnBasedTileToolkit/Blueprints/Pawns/Unit.Unit_C|GetIndex _asunit_skill_2)))
              (Variables|Default|SetAttack%20Hit _hit))
            (:CastFailed
              _)))
        (:CastFailed
          _))
      ;;;[0 0 0] Fire Laser Beam
      (bind _aspawn_anim_bp_parent (Utilities|Casting|CastToPawn_Anim_BP_Parent (Components|SkeletalMesh|GetAnimInstance (Utilities|Array|Get(acopy) (Actor|GetComponentsByClass (Variables|Default|GetOwning%20Unit) "/Script/Engine.SkeletalMeshComponent")))))
      (Default|AttackAnimation _aspawn_anim_bp_parent)
      (Utilities|FlowControl|Delay 0.05)
      (Audio|PlaySoundatLocation "/Game/AdvancedTurnBasedTileToolkit/Maps/SciFi/Weapons/laser3.laser3" (Transformation|GetSocketLocation (Variables|Default|GetWeapon) "Muzzle"))
      (Class|ParticleSystemComponent|SetBeamSourcePoint (Variables|Default|GetLaser) 0 (Transformation|GetSocketLocation (Variables|Default|GetWeapon) "Muzzle"))
      (Class|ParticleSystemComponent|SetBeamTargetPoint (Variables|Default|GetLaser) 0 (Math|Vector|SelectVector (Math|Vector|MakeVector (.x (Transformation|GetActorLocation (Variables|Default|GetTarget))) (.y (Transformation|GetActorLocation (Variables|Default|GetTarget))) (+ (.z (Transformation|GetActorLocation (Variables|Default|GetTarget))) _returnvalue_2)) (+ (Math|Vector|MakeVector (.x (Transformation|GetActorLocation (Variables|Default|GetTarget))) (.y (Transformation|GetActorLocation (Variables|Default|GetTarget))) (+ _returnvalue_2 (Variables|/Game/AdvancedTurnBasedTileToolkit/Blueprints/Gameplay/BP_Grid_Manager.BP_Grid_Manager_C|GetHeight%20Between%20Levels _grid_manager_ref_3))) (* (- (Math|Vector|MakeVector (.x (Transformation|GetActorLocation (Variables|Default|GetTarget))) (.y (Transformation|GetActorLocation (Variables|Default|GetTarget))) (+ _returnvalue_2 (Variables|/Game/AdvancedTurnBasedTileToolkit/Blueprints/Gameplay/BP_Grid_Manager.BP_Grid_Manager_C|GetHeight%20Between%20Levels _grid_manager_ref_3))) (Transformation|GetSocketLocation (Variables|Default|GetWeapon) "Muzzle")) 1e+02)) (Variables|Default|GetAttack%20Hit)))
      (Rendering|SetVisibility (Variables|Default|GetLaser) true false)
      (CallFunction|WakeUnitsinRange (Variables|/Game/AdvancedTurnBasedTileToolkit/Blueprints/Pawns/Unit.Unit_C|GetIndex (Variables|Default|GetTarget)) 10)
      (CallFunction|WakeUnitsinRange (Variables|/Game/AdvancedTurnBasedTileToolkit/Blueprints/Pawns/Unit.Unit_C|GetIndex (Variables|Default|GetOwning%20Unit)) 0 6)
      (bind _asatbtt_game_mode_sci_fi (Utilities|Casting|CastToATBTT_GameMode_SciFi (Variables|Default|GetGame%20Mode%20Ref)))
      (Default|WakeUnit _asatbtt_game_mode_sci_fi (Variables|Default|GetTarget))
      (Utilities|FlowControl|Sequence
        (:then_0
          ;;;[0 0 0] Deal Damage
          (if (Variables|Default|GetAttack%20Hit)
            (Default|ReceiveDamage (Variables|Default|GetTarget) (Math|Conversions|ToFloat(Integer) (Math|Random|RandomIntegerinRange (.min _damage_range) (.max _damage_range))) 0.0))
          (Utilities|FlowControl|Delay 0.79)
          ;;;[0 0 0] Deactivate Skill
          (Default|SetMarkerVisibility _grid_manager_ref_4 false (Variables|/Game/AdvancedTurnBasedTileToolkit/Blueprints/Gameplay/BP_Grid_Manager.BP_Grid_Manager_C|GetTarget%20Marker%20Decal _grid_manager_ref_4) (Variables|/Game/AdvancedTurnBasedTileToolkit/Blueprints/Gameplay/BP_Grid_Manager.BP_Grid_Manager_C|GetTargetMarker _grid_manager_ref_4))
          (CallFunction|DeactivateSkill)
          (if (not (Variables|Default|GetFrom%20Overwatch))
            (Default|ActivateUnit (Variables|Default|GetOwning%20Unit))))
        (:then_1
          (Utilities|FlowControl|Delay 0.05)
          (Rendering|SetVisibility (Variables|Default|GetLaser) false false))))))

(event EventAICheckValue
  (params (Unit :type Unit%20Object%20Reference))
  ;[0 0 0] AI
  ;;[0 1 0.2041] Check Value
  (|CallParentFunction Unit)
  (CallFunction|EvaluateSkill false)
  (Utilities|FlowControl|Delay 0.0)
  (bind _move_target_index (CallFunction|FindBestTilefromWhichtoUseSkill))
  (if (not (Variables|Default|GetOnly%20Ckeck%20Value))
    (CallFunction|FindPathandInitializeMovement _move_target_index)))

(event EventAIPrepareandExecuteSkill
  (bind _owning_unit (Variables|Default|GetOwning%20Unit))
  (bind _owning_unit_2 (Variables|Default|GetOwning%20Unit))
  (bind _grid_manager_ref (Variables|Default|GetGrid_Manager_Ref))
  (bind _grid_manager_ref_2 (Variables|Default|GetGrid_Manager_Ref))
  (bind (_asunit_skill _bsuccess) (Utilities|Casting|CastToUnit_Skill _owning_unit_2))
  (bind _target_marker_decal (Variables|/Game/AdvancedTurnBasedTileToolkit/Blueprints/Gameplay/BP_Grid_Manager.BP_Grid_Manager_C|GetTarget%20Marker%20Decal _grid_manager_ref))
  (bind _targetmarker (Variables|/Game/AdvancedTurnBasedTileToolkit/Blueprints/Gameplay/BP_Grid_Manager.BP_Grid_Manager_C|GetTargetMarker _grid_manager_ref))
  (bind _index (Variables|/Game/AdvancedTurnBasedTileToolkit/Blueprints/Pawns/Unit.Unit_C|GetIndex _owning_unit))
  ;[0 0 0] AI
  ;;[0.485 0.0302 0.03985] Choose to attack target or enter overwatch
  (Utilities|FlowControl|Sequence
    (:then_0
      (goto _label Open))
    (:then_1
      (for _array_element (Variables|/Game/AdvancedTurnBasedTileToolkit/Maps/SciFi/Blueprints/Pawns/Unit_Skill.Unit_Skill_C|GetSkill%20Child%20Components (.AsUnit%20Skill (Utilities|Casting|CastToUnit_Skill (Variables|Default|GetOwning%20Unit))))
        (if (== (Utilities|GetClass (Variables|/Script/Engine.ChildActorComponent|GetChildActor _array_element)) "/Game/AdvancedTurnBasedTileToolkit/Maps/SciFi/Blueprints/Skills/Skill_Overwatch.Skill_Overwatch_C")
          (Utilities|FlowControl|Sequence
            (:then_0
              (goto _label Close))
            (:then_1
              (bind _asunit_skill_2 (Utilities|Casting|CastToUnit_Skill (Utilities|Array|Get(acopy) (Variables|/Game/AdvancedTurnBasedTileToolkit/Blueprints/Gameplay/BP_Grid_Manager.BP_Grid_Manager_C|GetPawn%20Array (Variables|Default|GetGrid_Manager_Ref)) (Variables|Default|GetTarget%20Index))))
              (bind _hit_chance (Default|CalculateHitChance (.AsBP%20Grid%20Manager%20Sci%20Fi (Utilities|Casting|CastToBP_Grid_Manager_SciFi _grid_manager_ref_2)) (+ (Variables|/Game/AdvancedTurnBasedTileToolkit/Maps/SciFi/Blueprints/Pawns/Unit_Skill.Unit_Skill_C|GetDodge _asunit_skill_2) (Math|Float|SelectFloat (Variables|/Game/AdvancedTurnBasedTileToolkit/Maps/SciFi/Blueprints/Pawns/Unit_Skill.Unit_Skill_C|GetAccuracy _asunit_skill) 1.0 _bsuccess)) -0.05 0.0 _index (Variables|/Game/AdvancedTurnBasedTileToolkit/Blueprints/Pawns/Unit.Unit_C|GetIndex _asunit_skill_2)))
              (if (and (< (+ (Math|Random|RandomFloat) _hit_chance) 0.5) (> (Default|FindDistance(inTiles)BetweenIndexes _grid_manager_ref_2 _index (Variables|/Game/AdvancedTurnBasedTileToolkit/Blueprints/Pawns/Unit.Unit_C|GetIndex _asunit_skill_2) false) 5))
                (Default|ActivateSkill (.AsSkill%20Overwatch (Utilities|Casting|CastToSkill_Overwatch (Variables|/Script/Engine.ChildActorComponent|GetChildActor _array_element))) (Variables|Default|GetOwning%20Unit))
                (else
                  (CallFunction|PayActionPointCost)
                  (Default|SetMarkerLocation (Variables|Default|GetGrid_Manager_Ref) "0.000000,0.000000,0.000000" true (Variables|Default|GetTarget%20Index) _target_marker_decal _targetmarker)
                  (Default|SetMarkerVisibility (Variables|Default|GetGrid_Manager_Ref) true _target_marker_decal _targetmarker)
                  (CallFunction|AttackUnit (Utilities|Array|Get(acopy) (Variables|/Game/AdvancedTurnBasedTileToolkit/Blueprints/Gameplay/BP_Grid_Manager.BP_Grid_Manager_C|GetPawn%20Array (Variables|Default|GetGrid_Manager_Ref)) (Variables|Default|GetTarget%20Index)) false)))))))
      (Utilities|FlowControl|Gate false :!label _label
        (:Exit
          (CallFunction|PayActionPointCost)
          (Default|SetMarkerLocation (Variables|Default|GetGrid_Manager_Ref) "0.000000,0.000000,0.000000" true (Variables|Default|GetTarget%20Index) _target_marker_decal _targetmarker)
          (Default|SetMarkerVisibility (Variables|Default|GetGrid_Manager_Ref) true _target_marker_decal _targetmarker)
          (CallFunction|AttackUnit (Utilities|Array|Get(acopy) (Variables|/Game/AdvancedTurnBasedTileToolkit/Blueprints/Gameplay/BP_Grid_Manager.BP_Grid_Manager_C|GetPawn%20Array (Variables|Default|GetGrid_Manager_Ref)) (Variables|Default|GetTarget%20Index)) false))))))

(event EventActivateSkill
  (params (Unit :type Unit%20Object%20Reference))
  (bind _grid_manager_ref (Variables|Default|GetGrid_Manager_Ref))
  (bind _damage_range (Variables|Default|GetDamage%20Range))
  ;[0 1 0.005877] Activate Skill
  (|CallParentFunction Unit)
  (if (Variables|/Game/AdvancedTurnBasedTileToolkit/Blueprints/Pawns/Unit.Unit_C|GetAI%20Controlled Unit)
    ;[0 0 0] AI
    (if (== (Variables|/Game/AdvancedTurnBasedTileToolkit/Maps/SciFi/Blueprints/Pawns/Unit_Skill.Unit_Skill_C|GetCurrent%20Action%20Points (.AsUnit%20Skill (Utilities|Casting|CastToUnit_Skill (Variables|Default|GetOwning%20Unit)))) 1)
      (CallFunction|AIPrepareandExecuteSkill)
      (else
        (CallFunction|EvaluateSkill false)
        (Utilities|FlowControl|Delay 0.0)
        (bind _move_target_index (CallFunction|FindBestTilefromWhichtoUseSkill))
        (if (not (Variables|Default|GetOnly%20Ckeck%20Value))
          (CallFunction|FindPathandInitializeMovement _move_target_index))))
    (else
      ;[0 0 0] Player
      ;;[0.045 0.09893 1] Display Targets
      (Default|ClearAllinRangeMeshMarkers (Variables|Default|GetGrid_Manager_Ref))
      (Default|Pathfinding (Variables|Default|GetGrid_Manager_Ref) (Variables|/Game/AdvancedTurnBasedTileToolkit/Blueprints/Pawns/Unit.Unit_C|GetIndex (Variables|Default|GetOwning%20Unit)) 0 false 0 false "NewEnumerator0")
      (bind _units_in_sight (Default|FindVisibleUnitsinRange (Variables|Default|GetGrid_Manager_Ref) (Variables|/Game/AdvancedTurnBasedTileToolkit/Blueprints/Pawns/Unit.Unit_C|GetIndex (.AsUnit%20Skill (Utilities|Casting|CastToUnit_Skill (Variables|Default|GetOwning%20Unit)))) (Variables|Default|GetRange) false (* 16 (/ (+ (Variables|/Game/AdvancedTurnBasedTileToolkit/Blueprints/Gameplay/BP_Grid_Manager.BP_Grid_Manager_C|GetTileBoundsX _grid_manager_ref) (Variables|/Game/AdvancedTurnBasedTileToolkit/Blueprints/Gameplay/BP_Grid_Manager.BP_Grid_Manager_C|GetTileBoundsY _grid_manager_ref)) 2.0)) 1))
      (bind _indexes_out (Default|KeepIndexeswithRelevantUnits (Variables|Default|GetGrid_Manager_Ref) _units_in_sight (Variables|/Game/AdvancedTurnBasedTileToolkit/Blueprints/Pawns/Unit.Unit_C|GetAllied%20Factions (Variables|Default|GetOwning%20Unit)) false false))
      (Variables|/Game/AdvancedTurnBasedTileToolkit/Blueprints/Gameplay/BP_Grid_Manager.BP_Grid_Manager_C|SetTiles%20In%20Sight%20Array (Variables|Default|GetGrid_Manager_Ref) _indexes_out)
      (Default|SpawnTilesinSightRange (Variables|Default|GetGrid_Manager_Ref) "NewEnumerator1")
      (CallFunction|SetHUDText (Utilities|String|Append "Hit: " "-" " 
Damage: " (Utilities|String|ToString(Integer) (.min _damage_range)) " - " (Utilities|String|ToString(Integer) (.max _damage_range)))))))

(event EventTileClicked
  (params (Index :type Integer))
  (bind _grid_manager_ref (Variables|Default|GetGrid_Manager_Ref))
  (bind _clicked_tile (Variables|Default|GetClicked%20Tile))
  (bind _pawn_array (Variables|/Game/AdvancedTurnBasedTileToolkit/Blueprints/Gameplay/BP_Grid_Manager.BP_Grid_Manager_C|GetPawn%20Array _grid_manager_ref))
  (bind _item (Utilities|Array|Get(acopy) _pawn_array _clicked_tile))
  ;[0 0 0] Player
  ;;[0 1 0.6707] Tile Clicked
  (|CallParentFunction Index)
  (if (Utilities|IsValid _item) ; Does the clicked tile contain a unit?
    (if (!= (Utilities|Array|FindItem (Variables|/Game/AdvancedTurnBasedTileToolkit/Blueprints/Gameplay/BP_Grid_Manager.BP_Grid_Manager_C|GetTiles%20In%20Sight%20Array (Variables|Default|GetGrid_Manager_Ref)) (Variables|Default|GetClicked%20Tile)) -1)
      (CallFunction|PayActionPointCost)
      (CallFunction|AttackUnit _item false)
      (bind _asatbtt_player_controller (Utilities|Casting|CastToATBTT_PlayerController (Game|GetPlayerController 0)))
      (Variables|/Game/AdvancedTurnBasedTileToolkit/Blueprints/Gameplay/ATBTT_PlayerController.ATBTT_PlayerController_C|SetDisable%20Player%20Controller%20Input _asatbtt_player_controller true))))

(event EventCustomHoverEvent
  (bind _damage_range (Variables|Default|GetDamage%20Range))
  (bind _damage_range_2 (Variables|Default|GetDamage%20Range))
  ;[0 0 0] Player
  ;;[1 0.6677 0] Mouse Hover
  (|CallParentFunction)
  ;;;[0 0 0] Update Skill HUD
  (if (== (Utilities|Array|FindItem (Variables|/Game/AdvancedTurnBasedTileToolkit/Blueprints/Gameplay/BP_Grid_Manager.BP_Grid_Manager_C|GetTiles%20In%20Sight%20Array (Variables|Default|GetGrid_Manager_Ref)) (Variables|Default|GetCurrentTileHover)) -1)
    (CallFunction|SetHUDText (Utilities|String|Append "Hit: " "-" " 
Damage: " (Utilities|String|ToString(Integer) (.min _damage_range)) " - " (Utilities|String|ToString(Integer) (.max _damage_range))) :!label _label)
    (else
      (bind _asunit_skill (Utilities|Casting|CastToUnit_Skill (Utilities|Array|Get(acopy) (Variables|/Game/AdvancedTurnBasedTileToolkit/Blueprints/Gameplay/BP_Grid_Manager.BP_Grid_Manager_C|GetPawn%20Array (Variables|Default|GetGrid_Manager_Ref)) (Variables|Default|GetCurrentTileHover)))
        (:then
          (bind _asunit_skill_2 (Utilities|Casting|CastToUnit_Skill (Variables|/Game/AdvancedTurnBasedTileToolkit/Blueprints/Gameplay/ATBTT_GameMode.ATBTT_GameMode_C|GetCurrentPawn (.AsATBTT%20Game%20Mode (Utilities|Casting|CastToATBTT_GameMode (Game|GetGameMode)))))
            (:then
              (bind _asbp_grid_manager_sci_fi (Utilities|Casting|CastToBP_Grid_Manager_SciFi (Variables|Default|GetGrid_Manager_Ref)))
              (bind _hit_chance (Default|CalculateHitChance _asbp_grid_manager_sci_fi (+ (Variables|/Game/AdvancedTurnBasedTileToolkit/Maps/SciFi/Blueprints/Pawns/Unit_Skill.Unit_Skill_C|GetDodge _asunit_skill) (Variables|/Game/AdvancedTurnBasedTileToolkit/Maps/SciFi/Blueprints/Pawns/Unit_Skill.Unit_Skill_C|GetAccuracy _asunit_skill_2)) -0.05 0.0 (Variables|/Game/AdvancedTurnBasedTileToolkit/Blueprints/Pawns/Unit.Unit_C|GetIndex _asunit_skill_2) (Variables|/Game/AdvancedTurnBasedTileToolkit/Blueprints/Pawns/Unit.Unit_C|GetIndex _asunit_skill)))
              (Variables|/Game/AdvancedTurnBasedTileToolkit/Maps/SciFi/Blueprints/BP_Grid_Manager_SciFi.BP_Grid_Manager_SciFi_C|SetHUD%20Text _asbp_grid_manager_sci_fi (Utilities|Text|ToText(String) (Utilities|String|Append "Hit: " (Utilities|String|ToString(Integer) (Math|Float|Floor (Math|Float|Min(Float) (Math|Float|Max(Float) (* _hit_chance 1e+02) 0.0) 1e+02))) "% 
" "Damage: " (Utilities|String|ToString(Integer) (.min _damage_range_2)) " - " (Utilities|String|ToString(Integer) (.max _damage_range_2))))))
            (:CastFailed
              (goto _label))))
        (:CastFailed
          (goto _label))))))

(fn ConstructionScript
  (|CallParentFunction))

(fn PriorityModifier
  (params (Source%20Index :type Integer) (Target%20Index :type Integer))
  (bind _asbp_grid_manager_sci_fi (Utilities|Casting|CastToBP_Grid_Manager_SciFi (Variables|Default|GetGrid_Manager_Ref))
    (:then
      (bind _hit_chance (Default|CalculateHitChance _asbp_grid_manager_sci_fi 1.0 -0.05 0.0 Source%20Index Target%20Index)))
    (:CastFailed
      _))
  (return (* _hit_chance 2.0)))

(fn AIPriorityModifier
  (params (Current%20Index :type Integer) (Target%20Index :type Integer))
  (bind _asbp_grid_manager_sci_fi (Utilities|Casting|CastToBP_Grid_Manager_SciFi (Variables|Default|GetGrid_Manager_Ref))
    (:then
      (bind _hit_chance (Default|CalculateHitChance _asbp_grid_manager_sci_fi 1.0 -0.05 0.0 Current%20Index Target%20Index)))
    (:CastFailed
      _))
  (return _hit_chance))

(fn GetHoverText
  (bind _damage_range (Variables|Default|GetDamage%20Range))
  (return (Utilities|Text|ToText(String) (Utilities|String|Append (Utilities|String|ToString(Text) (Utilities|Text|MakeLiteralText "Laser Rifle: 
")) (Utilities|String|ToString(Text) (Utilities|Text|MakeLiteralText "Fire a laser beam for ")) "" (Utilities|String|ToString(Integer) (.min _damage_range)) " - " (Utilities|String|ToString(Integer) (.max _damage_range)) (Utilities|String|ToString(Text) (Utilities|Text|MakeLiteralText " points of damage at 
an enemy. Accuracy decreases with distance."))))))

(fn FindTargetValue
  (params (Target%20Index :type Integer))
  (bind _grid_manager_ref (Variables|Default|GetGrid_Manager_Ref))
  (bind _pawn_array (Variables|/Game/AdvancedTurnBasedTileToolkit/Blueprints/Gameplay/BP_Grid_Manager.BP_Grid_Manager_C|GetPawn%20Array _grid_manager_ref))
  (bind _item (Utilities|Array|Get(acopy) _pawn_array Target%20Index))
  (bind _currenthealth (Variables|/Game/AdvancedTurnBasedTileToolkit/Blueprints/Pawns/Unit.Unit_C|GetCurrentHealth _item))
  (return (* (/ 1.0 (Math|Conversions|ToFloat(Integer) (+ (Default|FindDistance(inTiles)BetweenIndexes (Variables|Default|GetGrid_Manager_Ref) Target%20Index (Variables|/Game/AdvancedTurnBasedTileToolkit/Blueprints/Pawns/Unit.Unit_C|GetIndex (Variables|Default|GetOwning%20Unit)) false) 10))) (Utilities|Select :Index (+ (Math|Conversions|ToInteger(Boolean) (<= (- (Math|Float|Truncate _currenthealth) (.min (Variables|Default|GetDamage%20Range))) 0)) (Math|Conversions|ToInteger(Boolean) (<= (- (Math|Float|Truncate _currenthealth) (.max (Variables|Default|GetDamage%20Range))) 0))) :Option%200 0.3 :Option%201 0.5 :Option%202 1.0))))