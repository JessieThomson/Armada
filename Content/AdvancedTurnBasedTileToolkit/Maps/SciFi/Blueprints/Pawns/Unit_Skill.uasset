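; Skill-driven unit pawn for the SciFi map of the turn-based tile toolkit, extending a parent unit.
; Spawns Skills as child actors; activation refills action points and ticks cooldowns once per turn, then hands off to AI or player controller until points run out.
; AI units fire their active skill after moving, waiting out slowed overwatch moments.
; Anim Blueprint calls drive movement, hit, death and randomly timed idle breaks.
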(event Custom|RandomizeBreakTimer
  ;[0.2571 1 0] Event Begin Play
  (Utilities|Time|SetTimerbyFunctionName 0 "BreakTimer" (Math|Random|RandomFloatinRange 1e+01 2e+01)))

(event EventActivateUnit
  ;[0.0452 1 0] Activate Unit
  (Utilities|FlowControl|Sequence
    (:then_0
      (Utilities|FlowControl|DoOnce false :!label _label
        (:Completed
          (Variables|Default|SetCurrent%20Action%20Points (Variables|Default|GetMax%20Action%20Points))
          (for _array_element (Variables|Default|GetSkill%20Child%20Components)
            (bind _asskill (Utilities|Casting|CastToSkill (Variables|/Script/Engine.ChildActorComponent|GetChildActor _array_element)))
            (Variables|/Game/AdvancedTurnBasedTileToolkit/Maps/SciFi/Blueprints/Skills/Skill.Skill_C|SetCurrent%20Cooldown _asskill (Math|Integer|Max(Integer) 0 (- (Variables|/Game/AdvancedTurnBasedTileToolkit/Maps/SciFi/Blueprints/Skills/Skill.Skill_C|GetCurrent%20Cooldown _asskill) 1)))
            (Rendering|SetVisibility (Variables|Default|GetBillboard%20Waiting) false false)))))
    (:then_1
      (if (> (Variables|Default|GetCurrent%20Action%20Points) 0)
        (if (Variables|Default|GetAI%20Controlled)
          (Default|ActivateAIUnit (Variables|/Game/AdvancedTurnBasedTileToolkit/Blueprints/Gameplay/ATBTT_GameMode.ATBTT_GameMode_C|GetAIController_Ref (Variables|Default|GetGameMode_Ref)) 1.0) ; Continued in ATBTT_AI_Controller
          (else
            (bind _asatbtt_player_controller (Utilities|Casting|CastToATBTT_PlayerController (Game|GetPlayerController 0)))
            (Default|ActivatePlayerUnit _asatbtt_player_controller self) ; Continued in ATBTT_PlayerController
          ))
        (else
          (Utilities|FlowControl|Sequence
            (:then_0
              (goto _label Reset))
            (:then_1
              (Default|DeactivateSkill (Variables|Default|GetActive%20Skill))
              (if (== (Utilities|Array|Length (Variables|Default|GetActive%20Effects)) 0)
                (Rendering|SetVisibility (Variables|Default|GetBillboard%20Waiting) (not (Variables|Default|GetAI%20Controlled)) false))
              (bind _asatbtt_player_controller_2 (Utilities|Casting|CastToATBTT_PlayerController (Game|GetPlayerController 0)))
              (Variables|/Game/AdvancedTurnBasedTileToolkit/Blueprints/Gameplay/ATBTT_PlayerController.ATBTT_PlayerController_C|SetDisable%20Player%20Controller%20Input _asatbtt_player_controller_2 true)
              (Default|ChooseNextPawn (Variables|Default|GetGameMode_Ref) 1.0))))))))

(event EventKillUnit
  (params (Anim%20Delay :type Float%20%28single-precision%29))
  ;[0 0 0] Kill Unit
  (Audio|Components|Audio|Stop (Variables|Default|GetMove%20Timeline))
  (Variables|Default|SetCustomTimeDilation 1.0)
  (bind _aspawn_anim_bp_parent (Utilities|Casting|CastToPawn_Anim_BP_Parent (Components|SkeletalMesh|GetAnimInstance (Variables|Default|GetSkeletalMesh))))
  (Default|DeathAnimation _aspawn_anim_bp_parent)
  (bind (_arrayindex _arrayelement) (Utilities|Array|ReverseforEachLoop (Variables|Default|GetActive%20Effects))
    (:LoopBody
      (if (Utilities|IsValid _arrayelement)
        (Actor|DestroyActor _arrayelement)
        (Utilities|Array|RemoveIndex (Variables|Default|GetActive%20Effects) _arrayindex)))
    (:Completed
      (|CallParentFunction Anim%20Delay))))

(event EventMoveTimelineUpdateFunc
  (bind _skeletalmesh (Variables|Default|GetSkeletalMesh))
  (bind _returnvalue (Components|SkeletalMesh|GetAnimInstance _skeletalmesh))
  (bind _aspawn_anim_bp_parent (Utilities|Casting|CastToPawn_Anim_BP_Parent _returnvalue))
  ;[1 0.8839 0] Move Timeline
  (|CallParentFunction)
  (if (Variables|Default|GetIdle)
    (Utilities|FlowControl|DoOnce true :!label _label
      (:Completed
        _))
    (else
      (Utilities|FlowControl|Sequence
        (:then_0
          (goto _label Reset))
        (:then_1
          (Variables|/Game/AdvancedTurnBasedTileToolkit/Animations/Pawn_Anim_BP_Parent.Pawn_Anim_BP_Parent_C|SetBreak _aspawn_anim_bp_parent false)))))
  (Default|MoveAnimation _aspawn_anim_bp_parent))

(event EventDecideActionAfterMove
  ;[0.2096 0 1] Decide Action after Move
  (if (Variables|Default|GetAI%20Controlled)
    (if (!= (Variables|Default|GetSpeed%20Modifier) 0.1) :!label _label ; Small hack to prevent unit from proceeding\nwith its action if it has been killed by a unit\nin overwatch
      (if (not (Variables|Default|GetPending%20Death))
        (Default|ActivateSkill (Variables|Default|GetActive%20Skill) self))
      (else
        (Utilities|FlowControl|Delay 0.0)
        (goto _label)))
    (else
      (|CallParentFunction))))

(event EventBeginPlay
  ;[0.2571 1 0] Event Begin Play
  (|CallParentFunction)
  (for _array_element (Variables|Default|GetSkills)
    (bind _returnvalue (AddComponent|AddChildActorComponent false))
    (ChildActorComponent|SetChildActorClass _returnvalue _array_element)
    (Utilities|Array|Add (Variables|Default|GetSkill%20Child%20Components) _returnvalue))
  (Utilities|Time|SetTimerbyFunctionName 0 "BreakTimer" (Math|Random|RandomFloatinRange 1e+01 2e+01)))

(event EventDamage
  (params (Damage :type Float%20%28single-precision%29) (Anim%20Delay :type Float%20%28single-precision%29))
  ;[1 0 0] Receive damage
  (|CallParentFunction Damage Anim%20Delay)
  (if (> (Variables|Default|GetCurrentHealth) 0.0)
    (Default|WakeUnit (.AsATBTT%20Game%20Mode%20Sci%20Fi (Utilities|Casting|CastToATBTT_GameMode_SciFi (Variables|Default|GetGameMode_Ref))) (.AsUnit%20Skill (Utilities|Casting|CastToUnit_Skill self)))
    (Utilities|FlowControl|Delay Anim%20Delay)
    (if (Variables|Default|GetIdle)
      (bind _aspawn_anim_bp_parent (Utilities|Casting|CastToPawn_Anim_BP_Parent (Components|SkeletalMesh|GetAnimInstance (Variables|Default|GetSkeletalMesh))))
      (Default|HitAnimation _aspawn_anim_bp_parent))))

(fn ConstructionScript
  (|CallParentFunction)
  (Class|SceneComponent|Attachto (Variables|Default|GetWeapon) (Variables|Default|GetSkeletalMesh) "Weapon" "SnapToTargetIncludingScale" true)
  (Rendering|Material|SetVectorParameterValue (Variables|Default|GetDynamic%20Health%20Bar%20Material) "color" (Utilities|Select :Index (Variables|Default|GetFaction) :NewEnumerator3 "" :NewEnumerator0 "(R=0.000000,G=0.500000,B=0.000000,A=1.000000)" :NewEnumerator1 "(R=1.000000,G=0.000000,B=0.000000,A=1.000000)" :NewEnumerator4 "(R=0.000000,G=0.000000,B=1.000000,A=1.000000)") :!class /Script/Engine.MaterialInstanceDynamic))

(fn BreakTimer
  (bind _aspawn_anim_bp_parent (Utilities|Casting|CastToPawn_Anim_BP_Parent (Components|SkeletalMesh|GetAnimInstance (Variables|Default|GetSkeletalMesh))))
  (Default|BreakAnimation _aspawn_anim_bp_parent)
  (CallFunction|RandomizeBreakTimer))