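; Grid manager for the SciFi map of the turn-based tile toolkit, adding cover-based combat and a turn HUD.
; At BeginPlay it line-traces edge tiles at two heights to store half or full cover, shown through instanced meshes.
; Cover toward the attacker and tile distance modify hit chance.
; Move markers distinguish long-range moves, and AI tile choice weighs skill priority against exposure to non-allied units among tiles with line of sight.
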(event EventSpawnTilesinMoveRangeMarkers
  (params (Only%20Edges :type Enum_TileSpawn%20Enum))
  (bind _returnvalue (Transformation|GetActorLocation))
  ;[1 1 1] Spawn Tiles In Move Range
  (bind _asatbtt_game_mode (Utilities|Casting|CastToATBTT_GameMode (Game|GetGameMode))
    (:then
      (bind _asunit_skill (Utilities|Casting|CastToUnit_Skill (Variables|/Game/AdvancedTurnBasedTileToolkit/Blueprints/Gameplay/ATBTT_GameMode.ATBTT_GameMode_C|GetCurrentPawn _asatbtt_game_mode))
        (:then
          (Variables|Default|SetRun%20Threshold (Math|Integer|SelectInt 0 (/ (* (Variables|/Game/AdvancedTurnBasedTileToolkit/Maps/SciFi/Blueprints/Pawns/Unit_Skill.Unit_Skill_C|GetCurrent%20Action%20Points _asunit_skill) (Variables|/Game/AdvancedTurnBasedTileToolkit/Blueprints/Pawns/Unit.Unit_C|GetMax%20Move (Variables|/Game/AdvancedTurnBasedTileToolkit/Blueprints/Gameplay/ATBTT_GameMode.ATBTT_GameMode_C|GetCurrentPawn _asatbtt_game_mode))) 2) (< (Variables|/Game/AdvancedTurnBasedTileToolkit/Maps/SciFi/Blueprints/Pawns/Unit_Skill.Unit_Skill_C|GetCurrent%20Action%20Points _asunit_skill) 2))))
        (:CastFailed
          (Variables|Default|SetRun%20Threshold 999 :!label _label))))
    (:CastFailed
      (goto _label)))
  (switch Utilities|FlowControl|Switch|SwitchonEnum_TileSpawn Only%20Edges
    (:NewEnumerator1
      (if (Variables|Default|GetUse%20Decals)
        (for _array_element (Variables|Default|GetIndex%20CanMoveToArray)
          (bind _returnvalue_2 (Rendering|Decal|SpawnDecalatLocation (select (> (.cost _array_element) (Variables|Default|GetRun%20Threshold)) (Variables|Default|GetTile%20in%20Long%20Move%20Range%20Decal) (Variables|Default|GetTile%20in%20Move%20Range%20Decal)) (Variables|Default|GetDecalSizeSquare) (Math|Vector|MakeVector (+ (.x (Utilities|Array|Get(acopy) (Variables|Default|GetVectorFieldArray) (.index _array_element))) (.x _returnvalue)) (+ (.y (Utilities|Array|Get(acopy) (Variables|Default|GetVectorFieldArray) (.index _array_element))) (.y _returnvalue)) (+ (.z (Utilities|Array|Get(acopy) (Variables|Default|GetVectorFieldArray) (.index _array_element))) (.z _returnvalue))) "90.000000,0.000000,90.000000" 0.0))
          (Utilities|Array|Add (Variables|Default|GetCurrentDecalsArray) _returnvalue_2))
        (else
          (for _array_element_2 (Variables|Default|GetIndex%20CanMoveToArray)
            (Components|InstancedStaticMesh|AddInstance (select (> (.cost _array_element_2) (Variables|Default|GetRun%20Threshold)) (Variables|Default|GetTileInLongMoveRangeMC) (Variables|Default|GetTileInMoveRangeMC)) (Math|Transform|MakeTransform (Math|Vector|MakeVector (/ (.x (Utilities|Array|Get(acopy) (Variables|Default|GetVectorFieldArray) (.index _array_element_2))) (/ (Variables|Default|GetTileBoundsX) 2e+02)) (/ (.y (Utilities|Array|Get(acopy) (Variables|Default|GetVectorFieldArray) (.index _array_element_2))) (/ (Variables|Default|GetNodeGapY) 2e+02)) (+ (.z (Utilities|Array|Get(acopy) (Variables|Default|GetVectorFieldArray) (.index _array_element_2))) (Variables|Default|GetTileInRangeZOffset))) "0, 0, 0" "1.000000,1.000000,1.000000"))))))
    (:NewEnumerator2
      (for _array_element_3 (Variables|Default|GetIndex%20CanMoveToArray)
        (CallFunction|SpawnEdgeMeshes (.index _array_element_3)))
      (for _array_element_4 (Variables|Default|GetReachable_Pawns_Array)
        (CallFunction|SpawnEdgeMeshes _array_element_4)))))

(event EventBeginPlay
  ;[1 1 1] Set up references
  (|CallParentFunction)
  (CallFunction|GenerateCover)
  (bind _returnvalue (AddComponent|AddHierarchicalInstancedStaticMeshComponent false))
  (bind _output_get (Variables|Default|SetCoverHISM _returnvalue))
  (Components|StaticMesh|SetStaticMesh _output_get (Variables|Default|GetCoverMesh))
  (bind _returnvalue_2 (AddComponent|AddHierarchicalInstancedStaticMeshComponent false))
  (bind _output_get_2 (Variables|Default|SetCoverHalfHISM _returnvalue_2))
  (Components|StaticMesh|SetStaticMesh _output_get_2 (Variables|Default|GetCoverHalfMesh))
  (bind _returnvalue_3 (UserInterface|CreateWidget "/Game/AdvancedTurnBasedTileToolkit/Maps/SciFi/Blueprints/HUD_SciFi.HUD_SciFi_C")) ; Add the hud showing Player/Enemy turn
  (bind _output_get_3 (Variables|Default|SetHUD_SciFi _returnvalue_3))
  (UserInterface|Viewport|AddtoViewport _output_get_3 0)
  (Input|SetInputModeGameandUI (Game|GetPlayerController 0) _output_get_3 "DoNotLock" true)
  (Variables|Default|SetDecalSizeSquare (Math|Vector|MakeVector 2e+02 1e+02 1e+02)))

(event EventClearAllinRangeMeshMarkers
  ;[1 1 1] Clear All In Range Mesh Markers
  (|CallParentFunction)
  (Components|InstancedStaticMesh|ClearInstances (Variables|Default|GetCoverHISM)))

(fn ConstructionScript
  (|CallParentFunction))

(fn GenerateCover
  (bind _gridsizex (Variables|Default|GetGridSizeX))
  (Utilities|Array|Resize (Variables|Default|GetCoverArray) (* (Variables|Default|GetGridSizeX) (Variables|Default|GetGridSizeY) (Variables|Default|GetGrid%20Size%20Z)))
  (for (_array_element _array_index) (Variables|Default|GetEdge%20Array)
    (if (> (Utilities|Array|Length (.edge_array_tile _array_element)) 0)
      (Utilities|Array|Clear (LocalVariables|GetLocal%20Cover%20Array))
      (LocalVariables|SetLocal%20Vector%20Array (Utilities|Array|MakeArray "200.000000, 0, 0" "-200.000000, 0, 0" "0.000000,200.000000, 0" "0,-200.000000, 0"))
      (LocalVariables|SetLocal%20Index%20Array (Utilities|Array|MakeArray 1 -1 _gridsizex (* _gridsizex -1)))
      (for (_array_element_2 _array_index_2) (LocalVariables|GetLocal%20Vector%20Array)
        (bind _returnvalue (Collision|LineTraceByChannel (Math|Vector|MakeVector (.x (+ (Transformation|GetActorLocation) (Utilities|Array|Get(acopy) (Variables|Default|GetVectorFieldArray) _array_index))) (.y (+ (Transformation|GetActorLocation) (Utilities|Array|Get(acopy) (Variables|Default|GetVectorFieldArray) _array_index))) (+ (.z (+ (Transformation|GetActorLocation) (Utilities|Array|Get(acopy) (Variables|Default|GetVectorFieldArray) _array_index))) (Variables|Default|GetHalf%20Cover%20Height))) (Math|Vector|MakeVector (+ (.x (+ (Transformation|GetActorLocation) (Utilities|Array|Get(acopy) (Variables|Default|GetVectorFieldArray) _array_index))) (.X (Math|Vector|BreakVector _array_element_2))) (+ (.y (+ (Transformation|GetActorLocation) (Utilities|Array|Get(acopy) (Variables|Default|GetVectorFieldArray) _array_index))) (.Y (Math|Vector|BreakVector _array_element_2))) (+ (.z (+ (Transformation|GetActorLocation) (Utilities|Array|Get(acopy) (Variables|Default|GetVectorFieldArray) _array_index))) (Variables|Default|GetHalf%20Cover%20Height))) "TraceTypeQuery5" false 0 "None"))
        (if _returnvalue
          (bind _returnvalue_2 (Collision|LineTraceByChannel (Math|Vector|MakeVector (.x (+ (Transformation|GetActorLocation) (Utilities|Array|Get(acopy) (Variables|Default|GetVectorFieldArray) _array_index))) (.y (+ (Transformation|GetActorLocation) (Utilities|Array|Get(acopy) (Variables|Default|GetVectorFieldArray) _array_index))) (+ (.z (+ (Transformation|GetActorLocation) (Utilities|Array|Get(acopy) (Variables|Default|GetVectorFieldArray) _array_index))) (Variables|Default|GetFull%20Cover%20Height))) (Math|Vector|MakeVector (+ (.x (+ (Transformation|GetActorLocation) (Utilities|Array|Get(acopy) (Variables|Default|GetVectorFieldArray) _array_index))) (.X (Math|Vector|BreakVector _array_element_2))) (+ (.y (+ (Transformation|GetActorLocation) (Utilities|Array|Get(acopy) (Variables|Default|GetVectorFieldArray) _array_index))) (.Y (Math|Vector|BreakVector _array_element_2))) (+ (.z (+ (Transformation|GetActorLocation) (Utilities|Array|Get(acopy) (Variables|Default|GetVectorFieldArray) _array_index))) (Variables|Default|GetFull%20Cover%20Height))) "TraceTypeQuery5" false 0 "None"))
          (if _returnvalue_2
            (Utilities|Array|Add (LocalVariables|GetLocal%20Cover%20Array) (Utilities|Struct|MakeStruct_Cover (+ _array_index (Utilities|Array|Get(acopy) (LocalVariables|GetLocal%20Index%20Array) _array_index_2)) -0.5))
            (else
              (Utilities|Array|Add (LocalVariables|GetLocal%20Cover%20Array) (Utilities|Struct|MakeStruct_Cover (+ _array_index (Utilities|Array|Get(acopy) (LocalVariables|GetLocal%20Index%20Array) _array_index_2)) -0.25))))))
      (Utilities|Array|SetArrayElem (Variables|Default|GetCoverArray) _array_index (Utilities|Struct|MakeStruct_Cover_Array (LocalVariables|GetLocal%20Cover%20Array))))))

(fn FindTargetCoverRelativetoSource
  (params (Source%20Index :type Integer) (Target%20Index :type Integer))
  (bind _vectorfieldarray (Variables|Default|GetVectorFieldArray))
  (bind _item (Utilities|Array|Get(acopy) _vectorfieldarray Source%20Index))
  (for _array_element (.struct_cover (Utilities|Array|Get(acopy) (Variables|Default|GetCoverArray) Target%20Index))
    (if (< (Math|Vector|VectorLength (- _item (Utilities|Array|Get(acopy) (Variables|Default|GetVectorFieldArray) (.index _array_element)))) (Math|Vector|VectorLength (- _item (Utilities|Array|Get(acopy) (Variables|Default|GetVectorFieldArray) Target%20Index))))
      (LocalVariables|SetLocal%20Cover (Math|Float|Min(Float) (.cover _array_element) (LocalVariables|GetLocal%20Cover) 0.0))))
  (return (LocalVariables|GetLocal%20Cover)))

(fn CalculateHitChance
  (params (Base%20Hit%20Chance :type Float%20%28single-precision%29) (Range%20Modifier :type Float%20%28single-precision%29) (Other%20Modifier :type Float%20%28single-precision%29) (Source%20Index :type Integer) (Target%20Index :type Integer))
  (bind _cover (CallFunction|FindTargetCoverRelativetoSource Source%20Index Target%20Index))
  (return (< (Math|Random|RandomFloat) (+ Base%20Hit%20Chance Other%20Modifier _cover (* (CallFunction|FindDistance(inTiles)BetweenIndexes Source%20Index Target%20Index false) Range%20Modifier))) (+ Base%20Hit%20Chance Other%20Modifier _cover (* (CallFunction|FindDistance(inTiles)BetweenIndexes Source%20Index Target%20Index false) Range%20Modifier))))

(fn ShowCoverMeshesAroundIndex
  (params (StartIndex :type Integer))
  (CallFunction|GetIndexesinRange StartIndex 1 false true)
  (Components|InstancedStaticMesh|ClearInstances (Variables|Default|GetCoverHISM))
  (for _array_element (Variables|Default|GetTilesInRangeArray)
    (for _array_element_2 (.struct_cover (Utilities|Array|Get(acopy) (Variables|Default|GetCoverArray) (.index _array_element)))
      (if (< (Math|Float|Absolute(Float) (- (.Z (Math|Vector|BreakVector (Utilities|Array|Get(acopy) (Variables|Default|GetVectorFieldArray) (.index _array_element)))) (.z (Utilities|Array|Get(acopy) (Variables|Default|GetVectorFieldArray) StartIndex)))) (Variables|Default|GetHeightImpassableCutoff))
        (Components|InstancedStaticMesh|AddInstance (select (< (.cover _array_element_2) -0.25) (Variables|Default|GetCoverHISM) (Variables|Default|GetCoverHalfHISM)) (Math|Transform|MakeTransform (Math|Vector|MakeVector (.x (/ (+ (Utilities|Array|Get(acopy) (Variables|Default|GetVectorFieldArray) (Math|Integer|%(Integer) (.index _array_element_2) (Variables|Default|GetGrid%20Size%20Squared))) (* (Utilities|Array|Get(acopy) (Variables|Default|GetVectorFieldArray) (.index _array_element)) 1.5)) 2.5)) (.y (/ (+ (Utilities|Array|Get(acopy) (Variables|Default|GetVectorFieldArray) (Math|Integer|%(Integer) (.index _array_element_2) (Variables|Default|GetGrid%20Size%20Squared))) (* (Utilities|Array|Get(acopy) (Variables|Default|GetVectorFieldArray) (.index _array_element)) 1.5)) 2.5)) (+ (.Z (Math|Vector|BreakVector (Utilities|Array|Get(acopy) (Variables|Default|GetVectorFieldArray) (.index _array_element)))) 8e+01)) (Math|Rotator|MakeRotator 2.7e+02 0.0 (+ (.yaw (Math|Rotator|FindLookatRotation (Utilities|Array|Get(acopy) (Variables|Default|GetVectorFieldArray) (Math|Integer|%(Integer) (.index _array_element_2) (Variables|Default|GetGrid%20Size%20Squared))) (Utilities|Array|Get(acopy) (Variables|Default|GetVectorFieldArray) (.index _array_element)))) 9e+01)) "1,1,1"))))))

(fn FindBestMoveIndexBasedonCoverandActiveSkill
  (params (Skill :type Skill%20Object%20Reference) (Start%20Index :type Integer) (Target%20Index :type Integer) (Max%20Range :type Integer) (Trace%20Visibility? :type Boolean) (Randomize :type Boolean) (Diamond%20Shaped%20Visibility :type Boolean))
  (bind _movechoicecandidates (Variables|Default|GetMoveChoiceCandidates))
  (bind _movechoicecandidates_2 (Variables|Default|GetMoveChoiceCandidates))
  (bind _item (Utilities|Array|Get(acopy) _movechoicecandidates))
  (LocalVariables|SetLocal%20Skill Skill)
  (CallFunction|GetIndexesinRange Target%20Index Max%20Range Diamond%20Shaped%20Visibility true)
  (Utilities|Array|Clear (Variables|Default|GetIndexesWithLOS))
  (bind _indexes_with_los (CallFunction|FindAllTilesinMoveRangewithSighttoTarget Start%20Index Target%20Index Max%20Range Diamond%20Shaped%20Visibility Trace%20Visibility? (Variables|Default|GetCanMoveToArray) (Variables|Default|GetTilesInRangeArray)))
  (Utilities|Array|Clear _movechoicecandidates_2)
  (Utilities|Array|Add _movechoicecandidates_2 (Utilities|Struct|MakeStruct_Range 0 -9999999))
  (for _array_element _indexes_with_los
    (bind _value (CallFunction|FindPriorityValueOfTile _array_element Target%20Index (LocalVariables|GetLocal%20Skill)))
    (if (> (Math|Float|Truncate (* _value 1e+02)) (.distance _item))
      (Utilities|Array|Clear (Variables|Default|GetMoveChoiceCandidates))
      (Utilities|Array|Add (Variables|Default|GetMoveChoiceCandidates) (Utilities|Struct|MakeStruct_Range _array_element (Math|Float|Truncate (* _value 1e+02))) :!label _label)
      (elif (== (Math|Float|Truncate (* _value 1e+02)) (.distance _item))
        (goto _label))))
  (bind (_target_index _target_value) (CallFunction|DecidetheFinalTargetfromViableOptions Randomize (Variables|Default|GetMoveChoiceCandidates)))
  (return _target_index (Math|Conversions|ToFloat(Integer) _target_value)))

(fn FindPriorityValueOfTile
  (params (Tile%20Index :type Integer) (Target%20Index :type Integer) (Skill :type Skill%20Object%20Reference))
  (LocalVariables|SetLocal%20Faction (Variables|/Game/AdvancedTurnBasedTileToolkit/Blueprints/Pawns/Unit.Unit_C|GetFaction (Variables|/Game/AdvancedTurnBasedTileToolkit/Blueprints/Gameplay/ATBTT_GameMode.ATBTT_GameMode_C|GetCurrentPawn (.AsATBTT%20Game%20Mode (Utilities|Casting|CastToATBTT_GameMode (Game|GetGameMode))))))
  (bind _priority (Default|AIPriorityModifier Skill Tile%20Index Target%20Index))
  (LocalVariables|SetLocal%20AI%20priority _priority)
  (bind _outactors (Actor|GetAllActorsOfClass "/Game/AdvancedTurnBasedTileToolkit/Maps/SciFi/Blueprints/Pawns/Unit_Skill.Unit_Skill_C"))
  (for _array_element _outactors
    (if (== (Utilities|Array|FindItem (Variables|/Game/AdvancedTurnBasedTileToolkit/Blueprints/Pawns/Unit.Unit_C|GetAllied%20Factions _array_element) (LocalVariables|GetLocal%20Faction)) -1)
      (bind _cover (CallFunction|FindTargetCoverRelativetoSource (Variables|/Game/AdvancedTurnBasedTileToolkit/Blueprints/Pawns/Unit.Unit_C|GetIndex _array_element) Tile%20Index))
      (LocalVariables|SetAI%20Priority%20Danger (+ (* (+ 1.0 (* _cover 1.5)) (/ 1.0 (Math|Conversions|ToFloat(Integer) (+ (CallFunction|FindDistance(inTiles)BetweenIndexes Tile%20Index (Variables|/Game/AdvancedTurnBasedTileToolkit/Blueprints/Pawns/Unit.Unit_C|GetIndex _array_element) false) 10)))) (LocalVariables|GetAI%20Priority%20Danger)))))
  (return (* (LocalVariables|GetLocal%20AI%20priority) (- 1.0 (LocalVariables|GetAI%20Priority%20Danger)))))