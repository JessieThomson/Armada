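; Sci-fi turn-based tile game mode that adds per-turn status effects and dormant units that wake on detection.
; Initiative initially holds one faction; movement triggers hearing, facing and line-trace sight checks that insert woken units into the order.
; Before each turn, the camera visits newly woken units with effect and sound.
; Active effects process sequentially via callbacks at turn start and end; completed rounds reset action points.
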(event Custom|Status%20Effect%20End%20Checked
  ;[1 1 1] Choose Next Pawn
  (Math|Integer|IncrementInt (Variables|Default|GetStatus%20Effect%20Counter) :!label _label
    (:%20%20
      (if (< (Variables|Default|GetStatus%20Effect%20Counter) (Utilities|Array|Length (Variables|/Game/AdvancedTurnBasedTileToolkit/Maps/SciFi/Blueprints/Pawns/Unit_Skill.Unit_Skill_C|GetActive%20Effects (stale EventChooseNextPawn _asunit_skill))))
        (if (Utilities|IsValid (Utilities|Array|Get(acopy) (Variables|/Game/AdvancedTurnBasedTileToolkit/Maps/SciFi/Blueprints/Pawns/Unit_Skill.Unit_Skill_C|GetActive%20Effects (stale EventChooseNextPawn _asunit_skill)) (Variables|Default|GetStatus%20Effect%20Counter)))
          (Default|OnUnitTurnEnd (Utilities|Array|Get(acopy) (Variables|/Game/AdvancedTurnBasedTileToolkit/Maps/SciFi/Blueprints/Pawns/Unit_Skill.Unit_Skill_C|GetActive%20Effects (stale EventChooseNextPawn _asunit_skill)) (Variables|Default|GetStatus%20Effect%20Counter)))
          (else
            (goto _label)))
        (else
          (|CallParentFunction (stale EventChooseNextPawn Delay)))))))

(event Custom|Status%20Effect%20Start%20Checked
  ;[1 1 1] Start New Turn
  (Math|Integer|IncrementInt (Variables|Default|GetStatus%20Effect%20Counter) :!label _label
    (:%20%20
      (if (< (Variables|Default|GetStatus%20Effect%20Counter) (Utilities|Array|Length (Variables|/Game/AdvancedTurnBasedTileToolkit/Maps/SciFi/Blueprints/Pawns/Unit_Skill.Unit_Skill_C|GetActive%20Effects (stale EventStartNextTurn _asunit_skill))))
        (if (Utilities|IsValid (Utilities|Array|Get(acopy) (Variables|/Game/AdvancedTurnBasedTileToolkit/Maps/SciFi/Blueprints/Pawns/Unit_Skill.Unit_Skill_C|GetActive%20Effects (stale EventStartNextTurn _asunit_skill)) (Variables|Default|GetStatus%20Effect%20Counter)))
          (Default|OnUnitTurnStart (Utilities|Array|Get(acopy) (Variables|/Game/AdvancedTurnBasedTileToolkit/Maps/SciFi/Blueprints/Pawns/Unit_Skill.Unit_Skill_C|GetActive%20Effects (stale EventStartNextTurn _asunit_skill)) (Variables|Default|GetStatus%20Effect%20Counter)))
          (else
            (goto _label)))
        (else
          (|CallParentFunction))))))

(event EventManageTurnCounter
  ;[1 1 1] Manage Turn Counter
  (if (Variables|/Game/AdvancedTurnBasedTileToolkit/Blueprints/Pawns/Unit.Unit_C|GetHasActedThisTurn (Variables|Default|GetCurrentPawn)) ; If the freshly activated unit is marked as having already acted this turn this means that all unit have acted, meaning we should signal the start of a new turn.
    (for _array_element (Variables|Default|GetInitiativeOrder) ; If all units have acted, reset "\nhas acted this turn"
      (bind _asunit_skill (Utilities|Casting|CastToUnit_Skill _array_element))
      (Variables|/Game/AdvancedTurnBasedTileToolkit/Blueprints/Pawns/Unit.Unit_C|SetHasActedThisTurn _asunit_skill false)
      (Variables|/Game/AdvancedTurnBasedTileToolkit/Maps/SciFi/Blueprints/Pawns/Unit_Skill.Unit_Skill_C|SetCurrent%20Action%20Points _asunit_skill (Variables|/Game/AdvancedTurnBasedTileToolkit/Maps/SciFi/Blueprints/Pawns/Unit_Skill.Unit_Skill_C|GetMax%20Action%20Points _asunit_skill))
      (Rendering|SetVisibility (Variables|/Game/AdvancedTurnBasedTileToolkit/Maps/SciFi/Blueprints/Pawns/Unit_Skill.Unit_Skill_C|GetBillboard%20Waiting _asunit_skill) false false))
    (Math|Integer|IncrementInt (Variables|Default|GetTurnCounter))))

(event EventChooseNextPawn
  (params (Delay :type Float%20%28single-precision%29))
  (bind _currentpawn (Variables|Default|GetCurrentPawn))
  ;[1 1 1] Choose Next Pawn
  (Variables|Default|SetStatus%20Effect%20Counter 0)
  (if (or (Variables|/Game/AdvancedTurnBasedTileToolkit/Blueprints/Pawns/Unit.Unit_C|GetPending%20Death _currentpawn) (not (Utilities|IsValid _currentpawn)))
    (|CallParentFunction Delay :!label _label)
    (else
      (bind _asunit_skill (Utilities|Casting|CastToUnit_Skill (Variables|Default|GetCurrentPawn)))
      (if (< (Variables|Default|GetStatus%20Effect%20Counter) (Utilities|Array|Length (Variables|/Game/AdvancedTurnBasedTileToolkit/Maps/SciFi/Blueprints/Pawns/Unit_Skill.Unit_Skill_C|GetActive%20Effects _asunit_skill))) :!label _label_2
        (if (Utilities|IsValid (Utilities|Array|Get(acopy) (Variables|/Game/AdvancedTurnBasedTileToolkit/Maps/SciFi/Blueprints/Pawns/Unit_Skill.Unit_Skill_C|GetActive%20Effects _asunit_skill) (Variables|Default|GetStatus%20Effect%20Counter)))
          (Default|OnUnitTurnEnd (Utilities|Array|Get(acopy) (Variables|/Game/AdvancedTurnBasedTileToolkit/Maps/SciFi/Blueprints/Pawns/Unit_Skill.Unit_Skill_C|GetActive%20Effects _asunit_skill) (Variables|Default|GetStatus%20Effect%20Counter)))
          (else
            (Math|Integer|IncrementInt (Variables|Default|GetStatus%20Effect%20Counter)
              (:%20%20
                (goto _label_2)))))
        (else
          (goto _label))))))

(event EventUnitEntersNewTile
  (params (Unit :type Unit%20Object%20Reference) (Index :type Integer) (Location :type Vector))
  (bind _currentpawn (Variables|Default|GetCurrentPawn))
  ;[1 1 1] Unit Enters New Tile
  (|CallParentFunction Unit Index Location)
  (bind _outactors (Actor|GetAllActorsOfClass "/Game/AdvancedTurnBasedTileToolkit/Blueprints/Pawns/Unit.Unit_C"))
  (for _array_element _outactors
    (CallFunction|CheckifUnitShouldWake _array_element (Variables|/Game/AdvancedTurnBasedTileToolkit/Blueprints/Pawns/Unit.Unit_C|GetIndex _currentpawn) 10 (select (Utilities|Enum|Equal(Enum) (Variables|/Game/AdvancedTurnBasedTileToolkit/Blueprints/Pawns/Unit.Unit_C|GetFaction _currentpawn) "NewEnumerator0") 2 6) 1.8e+02)))

(event EventStartNextTurn
  ;[1 1 1] Start New Turn
  (Utilities|ShowWokeUnits)
  (Variables|Default|SetStatus%20Effect%20Counter 0)
  (bind _asunit_skill (Utilities|Casting|CastToUnit_Skill (Variables|Default|GetCurrentPawn)))
  (if (< (Variables|Default|GetStatus%20Effect%20Counter) (Utilities|Array|Length (Variables|/Game/AdvancedTurnBasedTileToolkit/Maps/SciFi/Blueprints/Pawns/Unit_Skill.Unit_Skill_C|GetActive%20Effects _asunit_skill))) :!label _label
    (if (Utilities|IsValid (Utilities|Array|Get(acopy) (Variables|/Game/AdvancedTurnBasedTileToolkit/Maps/SciFi/Blueprints/Pawns/Unit_Skill.Unit_Skill_C|GetActive%20Effects _asunit_skill) (Variables|Default|GetStatus%20Effect%20Counter)))
      (Default|OnUnitTurnStart (Utilities|Array|Get(acopy) (Variables|/Game/AdvancedTurnBasedTileToolkit/Maps/SciFi/Blueprints/Pawns/Unit_Skill.Unit_Skill_C|GetActive%20Effects _asunit_skill) (Variables|Default|GetStatus%20Effect%20Counter)))
      (else
        (Math|Integer|IncrementInt (Variables|Default|GetStatus%20Effect%20Counter)
          (:%20%20
            (goto _label)))))
    (else
      (|CallParentFunction))))

(event EventSortPawnsinInitiativeOrder
  ;[1 1 1] Sort Pawns in Initiative Order
  (bind _outactors (Actor|GetAllActorsOfClass "/Game/AdvancedTurnBasedTileToolkit/Blueprints/Pawns/Unit.Unit_C"))
  (for _array_element _outactors
    (if (Utilities|Enum|Equal(Enum) (Variables|/Game/AdvancedTurnBasedTileToolkit/Blueprints/Pawns/Unit.Unit_C|GetFaction _array_element) "NewEnumerator0")
      (bind (_array_element_2 _array_index) (Utilities|Array|ForEachLoopwithBreak (Variables|Default|GetInitiativeOrder) :!label _label)
        (:LoopBody
          (bind _asunit (Utilities|Casting|CastToUnit _array_element_2))
          (if (< (Variables|/Game/AdvancedTurnBasedTileToolkit/Blueprints/Pawns/Unit.Unit_C|GetInitiative _asunit) (Variables|/Game/AdvancedTurnBasedTileToolkit/Blueprints/Pawns/Unit.Unit_C|GetInitiative _array_element))
            (Utilities|Array|Insert (Variables|Default|GetInitiativeOrder) _array_element _array_index)
            (Utilities|FlowControl|Sequence
              (:then_0
                (goto _label_2 Close))
              (:then_1
                (goto _label Break)))))
        (:Completed
          (Utilities|FlowControl|Sequence
            (:then_0
              (Utilities|FlowControl|Gate false :!label _label_2
                (:Exit
                  (Utilities|Array|Add (Variables|Default|GetInitiativeOrder) _array_element))))
            (:then_1
              (goto _label_2 Open))))))))

(fn ConstructionScript
  (|CallParentFunction))

(fn WakeUnit
  (params (Unit :type Unit%20Object%20Reference%20%28by%20ref%29))
  (if (== (Utilities|Array|FindItem (Variables|Default|GetInitiativeOrder) Unit) -1)
    (if (== (Utilities|Array|FindItem (Variables|Default|GetWoke%20Units) Unit) -1)
      (Utilities|Array|Add (Variables|Default|GetWoke%20Units) Unit)
      (if (Utilities|Enum|Equal(Enum) (Variables|/Game/AdvancedTurnBasedTileToolkit/Blueprints/Pawns/Unit.Unit_C|GetFaction (Variables|Default|GetCurrentPawn)) "NewEnumerator1")
        (Utilities|Array|Add (Variables|Default|GetInitiativeOrder) Unit :!label _label)
        (else
          (Utilities|FlowControl|Sequence
            (:then_0
              (goto _label_3 Open))
            (:then_1
              (bind (_array_element _array_index) (Utilities|Array|ForEachLoopwithBreak (Variables|Default|GetInitiativeOrder) :!label _label_2)
                (:LoopBody
                  (bind _asunit (Utilities|Casting|CastToUnit _array_element))
                  (if (Variables|/Game/AdvancedTurnBasedTileToolkit/Blueprints/Pawns/Unit.Unit_C|GetHasActedThisTurn _asunit)
                    (Utilities|Array|Insert (Variables|Default|GetInitiativeOrder) Unit _array_index)
                    (Utilities|FlowControl|Sequence
                      (:then_0
                        (goto _label_3 Close))
                      (:then_1
                        (goto _label_2 Break)))))
                (:Completed
                  (Utilities|FlowControl|Gate false :!label _label_3
                    (:Exit
                      (goto _label))))))))))))

(fn CheckifUnitShouldWake
  (params (Unit :type Unit%20Object%20Reference) (Source%20Index :type Integer) (Sight%20Range :type Integer) (Hearing%20Range :type Integer) (Sight%20Cone :type Float%20%28single-precision%29))
  (bind _returnvalue (Transformation|GetActorRotation Unit))
  (bind _grid_manager_ref (Variables|Default|GetGrid_Manager_Ref))
  (bind _grid_manager_ref_2 (Variables|Default|GetGrid_Manager_Ref))
  (bind _grid_manager_ref_3 (Variables|Default|GetGrid_Manager_Ref))
  (bind _square_visibility (Variables|/Game/AdvancedTurnBasedTileToolkit/Blueprints/Pawns/Unit.Unit_C|GetSquare%20Visibility Unit))
  (bind _index (Variables|/Game/AdvancedTurnBasedTileToolkit/Blueprints/Pawns/Unit.Unit_C|GetIndex Unit))
  (bind _grid_manager_ref_4 (Variables|Default|GetGrid_Manager_Ref))
  (bind _returnvalue_2 (Transformation|GetActorLocation _grid_manager_ref))
  (bind _returnvalue_3 (Transformation|GetActorLocation _grid_manager_ref_2))
  (bind _returnvalue_4 (not _square_visibility))
  (bind _vectorfieldarray (Variables|/Game/AdvancedTurnBasedTileToolkit/Blueprints/Gameplay/BP_Grid_Manager.BP_Grid_Manager_C|GetVectorFieldArray _grid_manager_ref))
  (bind _visibilitytraceheight (Variables|/Game/AdvancedTurnBasedTileToolkit/Blueprints/Gameplay/BP_Grid_Manager.BP_Grid_Manager_C|GetVisibilityTraceHeight _grid_manager_ref))
  (bind _vectorfieldarray_2 (Variables|/Game/AdvancedTurnBasedTileToolkit/Blueprints/Gameplay/BP_Grid_Manager.BP_Grid_Manager_C|GetVectorFieldArray _grid_manager_ref_2))
  (bind _visibilitytraceheight_2 (Variables|/Game/AdvancedTurnBasedTileToolkit/Blueprints/Gameplay/BP_Grid_Manager.BP_Grid_Manager_C|GetVisibilityTraceHeight _grid_manager_ref_2))
  (bind _vectorfieldarray_3 (Variables|/Game/AdvancedTurnBasedTileToolkit/Blueprints/Gameplay/BP_Grid_Manager.BP_Grid_Manager_C|GetVectorFieldArray _grid_manager_ref_4))
  (bind _item (Utilities|Array|Get(acopy) _vectorfieldarray _index))
  (bind _item_2 (Utilities|Array|Get(acopy) _vectorfieldarray Source%20Index))
  (bind _item_3 (Utilities|Array|Get(acopy) _vectorfieldarray_2 _index))
  (bind _item_4 (Utilities|Array|Get(acopy) _vectorfieldarray_2 Source%20Index))
  (bind _item_5 (Utilities|Array|Get(acopy) _vectorfieldarray_3 Source%20Index))
  (bind _item_6 (Utilities|Array|Get(acopy) _vectorfieldarray_3 _index))
  (bind _distance (Default|FindDistance(inTiles)BetweenIndexes _grid_manager_ref_3 Source%20Index _index _returnvalue_4))
  (bind _returnvalue_5 (Math|Rotator|FindLookatRotation _item_6 _item_5))
  (bind _returnvalue_6 (+ _item _returnvalue_2))
  (bind _returnvalue_7 (+ _item_2 _returnvalue_2))
  (bind _returnvalue_8 (+ _item_3 _returnvalue_3))
  (bind _returnvalue_9 (+ _item_4 _returnvalue_3))
  (bind _returnvalue_10 (Math|Rotator|Delta(Rotator) _returnvalue _returnvalue_5))
  (bind _returnvalue_11 (Math|Float|Absolute(Float) (.yaw _returnvalue_10)))
  (if (== (Utilities|Array|FindItem (Variables|Default|GetInitiativeOrder) Unit) -1)
    (if (<= _distance Hearing%20Range)
      (CallFunction|WakeUnit Unit :!label _label)
      (elif (<= _distance Sight%20Range)
        (if (Math|Boolean|NANDBoolean (< _returnvalue_11 269.0) (> _returnvalue_11 91.0))
          (bind _returnvalue_12 (Collision|LineTraceByChannel (Math|Vector|MakeVector (.x _returnvalue_6) (.y _returnvalue_6) (+ (.z _returnvalue_6) _visibilitytraceheight)) (Math|Vector|MakeVector (.x _returnvalue_7) (.y _returnvalue_7) (+ (.z _returnvalue_7) _visibilitytraceheight)) "TraceTypeQuery1" false 0 "None"))
          (if (not _returnvalue_12)
            (bind _returnvalue_13 (Collision|LineTraceByChannel (Math|Vector|MakeVector (.x _returnvalue_8) (.y _returnvalue_8) (+ (.z _returnvalue_8) _visibilitytraceheight_2)) (Math|Vector|MakeVector (.x _returnvalue_9) (.y _returnvalue_9) (+ (.z _returnvalue_9) _visibilitytraceheight_2)) "TraceTypeQuery5" false 0 "None"))
            (if (not _returnvalue_13)
              (goto _label))))))))