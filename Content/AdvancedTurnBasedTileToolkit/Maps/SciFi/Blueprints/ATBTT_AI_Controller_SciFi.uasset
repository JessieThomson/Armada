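; AI controller for the SciFi turn-based tile example that picks and triggers the active unit's skill.
; On activation it hides the HUD, runs pathfinding, has each charged, off-cooldown skill estimate its value, then activates the highest positive one.
; Scoring runs alongside the activation delay, which a wait loop honors before the skill fires.
; Without a worthwhile skill, it either skips the unit or zeroes its action points and activates it.
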(event EventActivateAIUnit
  (params (Delay :type Float%20%28single-precision%29))
  (bind _gamemode_ref (Variables|Default|GetGameMode_Ref))
  (bind _gamemode_ref_2 (Variables|Default|GetGameMode_Ref))
  (bind _skillcompare (Variables|Default|GetSkillCompare))
  (bind _grid_manager_ref (Variables|Default|GetGrid_Manager_Ref))
  (bind _grid_manager_ref_2 (Variables|Default|GetGrid_Manager_Ref))
  (bind _skill_value_array (Variables|Default|GetSkill%20Value%20Array))
  (bind (_indexofmaxvalue _maxvalue) (Math|Float|MaxOfFloatArray _skill_value_array))
  (bind _currentpawn (Variables|/Game/AdvancedTurnBasedTileToolkit/Blueprints/Gameplay/ATBTT_GameMode.ATBTT_GameMode_C|GetCurrentPawn _gamemode_ref))
  (bind _currentpawn_2 (Variables|/Game/AdvancedTurnBasedTileToolkit/Blueprints/Gameplay/ATBTT_GameMode.ATBTT_GameMode_C|GetCurrentPawn _gamemode_ref_2))
  (bind _item (Utilities|Array|Get(acopy) _skillcompare _indexofmaxvalue))
  (bind _asunit_skill (Utilities|Casting|CastToUnit_Skill _currentpawn_2))
  (Utilities|FlowControl|Sequence
    (:then_0
      (Variables|Default|SetDelay%20has%20passed false)
      (Utilities|FlowControl|Delay Delay)
      (Variables|Default|SetDelay%20has%20passed true))
    (:then_1
      (bind _asbp_grid_manager_sci_fi (Utilities|Casting|CastToBP_Grid_Manager_SciFi (Variables|Default|GetGrid_Manager_Ref)))
      (Widget|SetVisibility (Variables|/Game/AdvancedTurnBasedTileToolkit/Maps/SciFi/Blueprints/BP_Grid_Manager_SciFi.BP_Grid_Manager_SciFi_C|GetHUD_SciFi _asbp_grid_manager_sci_fi) "Hidden")
      (Default|Pathfinding (Variables|Default|GetGrid_Manager_Ref) (Variables|/Game/AdvancedTurnBasedTileToolkit/Blueprints/Pawns/Unit.Unit_C|GetIndex _currentpawn) (Variables|/Game/AdvancedTurnBasedTileToolkit/Blueprints/Pawns/Unit.Unit_C|GetCurrent%20Move _currentpawn) false (Variables|/Game/AdvancedTurnBasedTileToolkit/Blueprints/Pawns/Unit.Unit_C|GetAIMaxSearchRange _currentpawn) false (Variables|/Game/AdvancedTurnBasedTileToolkit/Blueprints/Pawns/Unit.Unit_C|GetPathfinding%20Type _currentpawn)) ; Used in most following skill value calculations
      (bind _asunit_skill_2 (Utilities|Casting|CastToUnit_Skill (Variables|/Game/AdvancedTurnBasedTileToolkit/Blueprints/Gameplay/ATBTT_GameMode.ATBTT_GameMode_C|GetCurrentPawn (Variables|Default|GetGameMode_Ref))))
      (if (> (Variables|/Game/AdvancedTurnBasedTileToolkit/Maps/SciFi/Blueprints/Pawns/Unit_Skill.Unit_Skill_C|GetCurrent%20Action%20Points _asunit_skill_2) 0)
        ;[0.9297 1 0] Evaluate skills
        (Variables|Default|SetSkill%20Counter 0)
        (Utilities|Array|Clear (Variables|Default|GetSkillCompare))
        (if (<= (Variables|Default|GetSkill%20Counter) (Utilities|Array|LastIndex (Variables|/Game/AdvancedTurnBasedTileToolkit/Maps/SciFi/Blueprints/Pawns/Unit_Skill.Unit_Skill_C|GetSkill%20Child%20Components _asunit_skill_2))) :!label _label
          (if (and (!= (Variables|/Game/AdvancedTurnBasedTileToolkit/Maps/SciFi/Blueprints/Skills/Skill.Skill_C|GetCurrent%20Charges (.AsSkill (Utilities|Casting|CastToSkill (Variables|/Script/Engine.ChildActorComponent|GetChildActor (Utilities|Array|Get(acopy) (Variables|/Game/AdvancedTurnBasedTileToolkit/Maps/SciFi/Blueprints/Pawns/Unit_Skill.Unit_Skill_C|GetSkill%20Child%20Components _asunit_skill_2) (Variables|Default|GetSkill%20Counter)))))) 0) (== (Variables|/Game/AdvancedTurnBasedTileToolkit/Maps/SciFi/Blueprints/Skills/Skill.Skill_C|GetCurrent%20Cooldown (.AsSkill (Utilities|Casting|CastToSkill (Variables|/Script/Engine.ChildActorComponent|GetChildActor (Utilities|Array|Get(acopy) (Variables|/Game/AdvancedTurnBasedTileToolkit/Maps/SciFi/Blueprints/Pawns/Unit_Skill.Unit_Skill_C|GetSkill%20Child%20Components _asunit_skill_2) (Variables|Default|GetSkill%20Counter)))))) 0))
            (Utilities|Array|Add (Variables|Default|GetSkillCompare) (.AsSkill (Utilities|Casting|CastToSkill (Variables|/Script/Engine.ChildActorComponent|GetChildActor (Utilities|Array|Get(acopy) (Variables|/Game/AdvancedTurnBasedTileToolkit/Maps/SciFi/Blueprints/Pawns/Unit_Skill.Unit_Skill_C|GetSkill%20Child%20Components _asunit_skill_2) (Variables|Default|GetSkill%20Counter))))))
            (Default|AICheckValue (.AsSkill (Utilities|Casting|CastToSkill (Variables|/Script/Engine.ChildActorComponent|GetChildActor (Utilities|Array|Get(acopy) (Variables|/Game/AdvancedTurnBasedTileToolkit/Maps/SciFi/Blueprints/Pawns/Unit_Skill.Unit_Skill_C|GetSkill%20Child%20Components _asunit_skill_2) (Variables|Default|GetSkill%20Counter))))) (Variables|/Game/AdvancedTurnBasedTileToolkit/Blueprints/Gameplay/ATBTT_GameMode.ATBTT_GameMode_C|GetCurrentPawn (Variables|Default|GetGameMode_Ref)))
            (Utilities|FlowControl|Delay 0.1))
          (Math|Integer|IncrementInt (Variables|Default|GetSkill%20Counter)
            (:%20%20
              (goto _label)))
          (else
            (Utilities|FlowControl|Delay 0.0)
            (Utilities|Array|Clear (Variables|Default|GetSkill%20Value%20Array))
            (for _array_element (Variables|Default|GetSkillCompare)
              (Utilities|Array|Add (Variables|Default|GetSkill%20Value%20Array) (Variables|/Game/AdvancedTurnBasedTileToolkit/Maps/SciFi/Blueprints/Skills/Skill.Skill_C|GetAI%20Estimated%20Value _array_element)))
            ;[0.2176 1 0] Choose best skill and activate
            (if (> _maxvalue 0.0)
              (Default|SetMarkerVisibility _grid_manager_ref true (Variables|/Game/AdvancedTurnBasedTileToolkit/Blueprints/Gameplay/BP_Grid_Manager.BP_Grid_Manager_C|GetCurrentMarkerDecal _grid_manager_ref) (Variables|/Game/AdvancedTurnBasedTileToolkit/Blueprints/Gameplay/BP_Grid_Manager.BP_Grid_Manager_C|GetCurrentPawnMarker _grid_manager_ref))
              (Variables|/Game/AdvancedTurnBasedTileToolkit/Blueprints/Gameplay/BP_Grid_Camera.BP_Grid_Camera_C|SetIsPanning (Variables|Default|GetGrid%20Camera%20Ref) false)
              (Utilities|WaitUntilDelayHasPassed
                (:%20%20
                  (Variables|/Game/AdvancedTurnBasedTileToolkit/Maps/SciFi/Blueprints/Skills/Skill.Skill_C|SetOnly%20Ckeck%20Value _item false)
                  (Default|ActivateSkill _item (.AsUnit%20Skill (Utilities|Casting|CastToUnit_Skill (Variables|/Game/AdvancedTurnBasedTileToolkit/Blueprints/Gameplay/ATBTT_GameMode.ATBTT_GameMode_C|GetCurrentPawn (Variables|Default|GetGameMode_Ref)))))))
              (elif (Variables|Default|GetSkip%20Unit%20if%20no%20action%20availible)
                (Default|ChooseNextPawn (Variables|Default|GetGameMode_Ref) 0.0)
                (else
                  (Default|SetMarkerVisibility _grid_manager_ref_2 true (Variables|/Game/AdvancedTurnBasedTileToolkit/Blueprints/Gameplay/BP_Grid_Manager.BP_Grid_Manager_C|GetCurrentMarkerDecal _grid_manager_ref_2) (Variables|/Game/AdvancedTurnBasedTileToolkit/Blueprints/Gameplay/BP_Grid_Manager.BP_Grid_Manager_C|GetCurrentPawnMarker _grid_manager_ref_2))
                  (Variables|/Game/AdvancedTurnBasedTileToolkit/Blueprints/Gameplay/BP_Grid_Camera.BP_Grid_Camera_C|SetIsPanning (Variables|Default|GetGrid%20Camera%20Ref) false)
                  (Variables|/Game/AdvancedTurnBasedTileToolkit/Maps/SciFi/Blueprints/Pawns/Unit_Skill.Unit_Skill_C|SetCurrent%20Action%20Points _asunit_skill 0)
                  (Default|ActivateUnit _asunit_skill))))))
        (else
          (Default|ActivateUnit (Variables|/Game/AdvancedTurnBasedTileToolkit/Blueprints/Gameplay/ATBTT_GameMode.ATBTT_GameMode_C|GetCurrentPawn (Variables|Default|GetGameMode_Ref))))))))

(fn ConstructionScript
  (|CallParentFunction))

(fn FindMaxRangeOfCurrentUnit'sSkills
  (params (Unit :type Unit%20Skill%20Object%20Reference))
  (LocalVariables|SetTemp%20Range 0)
  (for _array_element (Actor|GetAllChildActors Unit true)
    (bind _asskill (Utilities|Casting|CastToSkill _array_element))
    (if (> (Variables|/Game/AdvancedTurnBasedTileToolkit/Maps/SciFi/Blueprints/Skills/Skill.Skill_C|GetRange _asskill) (LocalVariables|GetTemp%20Range))
      (LocalVariables|SetTemp%20Range (Variables|/Game/AdvancedTurnBasedTileToolkit/Maps/SciFi/Blueprints/Skills/Skill.Skill_C|GetRange _asskill))))
  (return (LocalVariables|GetTemp%20Range)))