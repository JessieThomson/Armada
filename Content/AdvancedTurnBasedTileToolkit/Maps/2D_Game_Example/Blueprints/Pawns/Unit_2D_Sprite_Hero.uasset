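; Player hero unit for the 2D dungeon example of the turn-based tile toolkit; its death triggers game over on the DungeonHUD.
; On BeginPlay it reveals tiles within sight range and equips the first dagger found in the level.
; Equipped items set weapon, armor or shield variables and sprites.
; Attacks use weapon damage through projectile or melee timelines before passing the turn, while shield and armor reduce incoming damage.
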(event Custom|Equip%20Item
  (params (Item :type Item%20Parent%20Object%20Reference))
  (switch Utilities|FlowControl|Switch|SwitchonEnum_Item_Type (Variables|/Game/AdvancedTurnBasedTileToolkit/Maps/2D_Game_Example/Blueprints/Items/Item_Parent.Item_Parent_C|GetItem%20Type Item)
    (:NewEnumerator0
      (Development|PrintString "ERROR: Item type cannot be equipped"))
    (:NewEnumerator1
      (bind _asitem_weapon_parent_sword (Utilities|Casting|CastToItem_Weapon_Parent_Sword Item))
      (Variables|Default|SetWeapon _asitem_weapon_parent_sword)
      (Variables|Default|SetRange (Variables|/Game/AdvancedTurnBasedTileToolkit/Maps/2D_Game_Example/Blueprints/Items/Item_Weapon_Parent_Sword.Item_Weapon_Parent_Sword_C|GetRange _asitem_weapon_parent_sword))
      (Rendering|Components|Sprite|SetSprite (Variables|Default|GetWeaponSprite) (Variables|/Game/AdvancedTurnBasedTileToolkit/Maps/2D_Game_Example/Blueprints/Items/Item_Weapon_Parent_Sword.Item_Weapon_Parent_Sword_C|GetEquippedSprite _asitem_weapon_parent_sword))
      (Variables|Default|SetHit%20Sound (Variables|/Game/AdvancedTurnBasedTileToolkit/Maps/2D_Game_Example/Blueprints/Items/Item_Weapon_Parent_Sword.Item_Weapon_Parent_Sword_C|GetHitSound _asitem_weapon_parent_sword)))
    (:NewEnumerator2
      (bind _asitem_armor_parent_plate (Utilities|Casting|CastToItem_Armor_Parent_Plate Item))
      (Variables|Default|SetArmor _asitem_armor_parent_plate)
      (Rendering|Components|Sprite|SetSprite (Variables|Default|GetArmorSprite) (Variables|/Game/AdvancedTurnBasedTileToolkit/Maps/2D_Game_Example/Blueprints/Items/Item_Armor_Parent_Plate.Item_Armor_Parent_Plate_C|GetEquippedSprite _asitem_armor_parent_plate)))
    (:NewEnumerator3
      (bind _asitem_shield_parent_metal (Utilities|Casting|CastToItem_Shield_Parent_Metal Item))
      (Variables|Default|SetShield _asitem_shield_parent_metal)
      (Rendering|Components|Sprite|SetSprite (Variables|Default|GetShieldSprite) (Variables|/Game/AdvancedTurnBasedTileToolkit/Maps/2D_Game_Example/Blueprints/Items/Item_Shield_Parent_Metal.Item_Shield_Parent_Metal_C|GetEquippedSprite _asitem_shield_parent_metal)))))

(event EventKillUnit
  (params (Anim%20Delay :type Float%20%28single-precision%29))
  (Variables|/Game/AdvancedTurnBasedTileToolkit/Blueprints/Gameplay/ATBTT_GameMode.ATBTT_GameMode_C|SetGame%20Over (Variables|Default|GetGameMode_Ref) true)
  (Actor|DestroyActor)
  (bind _foundwidgets (Widget|GetAllWidgetsOfClass "/Game/AdvancedTurnBasedTileToolkit/Maps/2D_Game_Example/Blueprints/DungeonHUD.DungeonHUD_C" true))
  (Default|GameOver (Utilities|Array|Get(acopy) _foundwidgets)))

(event EventDamage
  (params (Damage :type Float%20%28single-precision%29) (Anim%20Delay :type Float%20%28single-precision%29))
  (bind _gridmanager_ref (Variables|Default|GetGridManager_Ref))
  (bind _shield (Variables|Default|GetShield))
  (bind _armor (Variables|Default|GetArmor))
  ;[1 0 0.8273] Recieve Damage - differs in that damage is reduced by the hero's Shield and Armor variables
  (Variables|Default|SetDamage%20Temp Damage)
  (Utilities|FlowControl|Delay Anim%20Delay)
  (if (!= _shield 0)
    (Variables|Default|SetDamage%20Temp (- (Variables|Default|GetDamage%20Temp) (Variables|/Game/AdvancedTurnBasedTileToolkit/Maps/2D_Game_Example/Blueprints/Items/Item_Shield_Parent_Metal.Item_Shield_Parent_Metal_C|GetArmor _shield))))
  (if (!= _armor 0)
    (Variables|Default|SetDamage%20Temp (- (Variables|Default|GetDamage%20Temp) (Variables|/Game/AdvancedTurnBasedTileToolkit/Maps/2D_Game_Example/Blueprints/Items/Item_Armor_Parent_Plate.Item_Armor_Parent_Plate_C|GetArmor _armor))))
  (Variables|Default|SetCurrentHealth (- (Variables|Default|GetCurrentHealth) (Math|Float|SelectFloat (Variables|Default|GetDamage%20Temp) 0.0 (> (Variables|Default|GetDamage%20Temp) 0.0))))
  (Rendering|Material|SetScalarParameterValue (Variables|Default|GetDynamic%20Health%20Bar%20Material) "PercentFill" (/ (Variables|Default|GetCurrentHealth) (Variables|Default|GetMaxHealth)) :!class /Script/Engine.MaterialInstanceDynamic)
  (Default|SetMarkerVisibility _gridmanager_ref false (Variables|/Game/AdvancedTurnBasedTileToolkit/Blueprints/Gameplay/BP_Grid_Manager.BP_Grid_Manager_C|GetTarget%20Marker%20Decal _gridmanager_ref) (Variables|/Game/AdvancedTurnBasedTileToolkit/Blueprints/Gameplay/BP_Grid_Manager.BP_Grid_Manager_C|GetTargetMarker _gridmanager_ref))
  (if (<= (Variables|Default|GetCurrentHealth) 0.0)
    (Rendering|SetVisibility (Variables|Default|GetHealthBillboard) false false)
    (Utilities|Array|RemoveItem (Variables|/Game/AdvancedTurnBasedTileToolkit/Blueprints/Gameplay/ATBTT_GameMode.ATBTT_GameMode_C|GetInitiativeOrder (Variables|Default|GetGameMode_Ref)) self)
    (Utilities|Array|SetArrayElem (Variables|/Game/AdvancedTurnBasedTileToolkit/Blueprints/Gameplay/BP_Grid_Manager.BP_Grid_Manager_C|GetPawn%20Array (Variables|Default|GetGridManager_Ref)) (Variables|Default|GetIndex) 0)
    (CallFunction|KillUnit (Variables|Default|GetDeath%20Anim%20Delay))))

(event EventBeginPlay
  (|CallParentFunction)
  (Utilities|FlowControl|Delay 0.01)
  (bind _index (Class|InterfaceTile|VectortoIndexInterface(Message) (Variables|Default|GetGridManager_Ref) (Transformation|GetActorLocation)))
  (bind _asbp_grid_manager_2d (Utilities|Casting|CastToBP_Grid_Manager_2D (Variables|Default|GetGridManager_Ref)))
  (Default|RevealVisibleTiles _asbp_grid_manager_2d _index (Variables|Default|GetSight%20Range)) ; Reveal all tiles initially visible to the unit
  (bind _outactors (Actor|GetAllActorsOfClass "/Game/AdvancedTurnBasedTileToolkit/Maps/2D_Game_Example/Blueprints/Items/Item_Weapon_Dagger.Item_Weapon_Dagger_C"))
  (CallFunction|EquipItem (Utilities|Array|Get(acopy) _outactors)) ; Equip the dagger placed in the game.\nIf there is no dagger everything will still\nwork, but there will be an error in the log.
)

(event EventAttackVictim
  (params (Victim :type Unit%20Object%20Reference))
  (bind _gridmanager_ref (Variables|Default|GetGridManager_Ref))
  (bind _gamemode_ref (Variables|Default|GetGameMode_Ref))
  (bind _targetmarker (Variables|/Game/AdvancedTurnBasedTileToolkit/Blueprints/Gameplay/BP_Grid_Manager.BP_Grid_Manager_C|GetTargetMarker _gridmanager_ref))
  (bind _target_marker_decal (Variables|/Game/AdvancedTurnBasedTileToolkit/Blueprints/Gameplay/BP_Grid_Manager.BP_Grid_Manager_C|GetTarget%20Marker%20Decal _gridmanager_ref))
  ;[0 0 0] Attack Victim - differs from other 2D units in that damage comes from the hero's Weapon variable
  (Default|SetMarkerLocation (Variables|Default|GetGridManager_Ref) "0, 0, 0" false (Variables|/Game/AdvancedTurnBasedTileToolkit/Blueprints/Pawns/Unit.Unit_C|GetIndex Victim) _target_marker_decal _targetmarker)
  (Default|SetMarkerVisibility (Variables|Default|GetGridManager_Ref) true _target_marker_decal _targetmarker)
  (Variables|Default|SetAttackerLocation (Transformation|GetActorLocation))
  (Variables|Default|SetTargetLocation (Transformation|GetActorLocation Victim))
  (if (Variables|/Game/AdvancedTurnBasedTileToolkit/Maps/2D_Game_Example/Blueprints/Items/Item_Weapon_Parent_Sword.Item_Weapon_Parent_Sword_C|GetProjectile (Variables|Default|GetWeapon))
    (Audio|PlaySound2D (Variables|Default|GetProjectile%20Sound))
    (bind _returnvalue (Game|SpawnActorfromClass (Variables|/Game/AdvancedTurnBasedTileToolkit/Maps/2D_Game_Example/Blueprints/Items/Item_Weapon_Parent_Sword.Item_Weapon_Parent_Sword_C|GetProjectile%20Class (Variables|Default|GetWeapon)) (Math|Conversions|ToTransform(Vector) (Variables|Default|GetAttackerLocation)) "Undefined" 0 0))
    (bind _attack_timeline (Timeline|Timeline_3 PlayFromStart)
      (:Update
        (Transformation|SetActorLocationAndRotation _returnvalue (+ (Variables|Default|GetAttackerLocation) (* (- (Variables|Default|GetTargetLocation) (Variables|Default|GetAttackerLocation)) _attack_timeline)) (Math|Rotator|MakeRotator 0.0 0.0 (+ (.yaw (Math|Rotator|FindLookatRotation (Variables|Default|GetAttackerLocation) (Variables|Default|GetTargetLocation))) 9e+01))))
      (:Finished
        (Actor|DestroyActor _returnvalue)
        (Utilities|FlowControl|Sequence
          (:then_0
            (Audio|PlaySound2D (Variables|Default|GetHit%20Sound) :!label _label)
            (Default|ReceiveDamage Victim (Math|Float|Max(Float) (Variables|/Game/AdvancedTurnBasedTileToolkit/Maps/2D_Game_Example/Blueprints/Items/Item_Weapon_Parent_Sword.Item_Weapon_Parent_Sword_C|GetDamage (Variables|Default|GetWeapon)) 25.0) 0.0))
          (:then_1
            (Default|ChooseNextPawn _gamemode_ref (Variables|/Game/AdvancedTurnBasedTileToolkit/Blueprints/Gameplay/ATBTT_GameMode.ATBTT_GameMode_C|GetAI%20Activation%20Delay _gamemode_ref) :!label _label_2)
            (Transformation|SetActorLocation (+ (* (- (Variables|Default|GetTargetLocation) (Variables|Default|GetAttackerLocation)) (stale _attack_timeline_2)) (Variables|Default|GetAttackerLocation)) false false :!label _label_3)))))
    (else
      (bind _attack_timeline_2 (Timeline|Timeline_3_0 PlayFromStart)
        (:Update
          (goto _label_3))
        (:Finished
          (goto _label_2))
        (:Attack%20Hit
          (goto _label))))))

(fn ConstructionScript
  (|CallParentFunction))